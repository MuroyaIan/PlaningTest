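; BP_TutorialSign is a tutorial sign actor that shows paged Stage 1 control instructions on screen.
; On BeginPlay it enables player input and creates the tutorial widget plus a floating-button widget, which it never displays in these graphs.
; Confirm opens the tutorial with a sound, guarded by visibility and animation checks, and Back plays its hide animation.
; While displayed, left/right buttons or delayed stick input past a threshold change pages.
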(event `self.ReceiveBeginPlay`
  (bind _asbp_player_controller (cast `/Game/Blueprints/Player/BP_PlayerController` (`GameplayStatics.GetPlayerController` 0)))
  (`self.EnableInput` _asbp_player_controller) ; 入力有効化
  (bind _returnvalue (`|CreateWidget` "/Game/Maps/TestMap/Kitayama/UI_Kitayama/Widget_UI/TutorialWidget/UMG_SignStage1_Tutorial.UMG_SignStage1_Tutorial_C")) ; Stage1の操作方法UI
  (set `self.Tutorial` _returnvalue)
  (bind _returnvalue_2 (`|CreateWidget` "/Game/Maps/TestMap/Kitayama/UI_Kitayama/Widget_UI/TutorialWidget/UMG_SingButton.UMG_SingButton_C")) ; ふよふよ浮かぶボタンUI
  (set `self.ButtonUI` _returnvalue_2))

(event `self.ReceiveTick`
  (params (DeltaSeconds :type "Float (single-precision)")))

(event `InputAction|UI_Confirm` :consume false
  (params (Key :type "Key Structure"))
  (:`Pressed`
    (`self.UMGAdd Toview`)))

(event `InputAction|UI_Back` :consume false
  (params (Key :type "Key Structure"))
  (:`Pressed`
    (if (`self.bIsDisp`)
      (bind _isplaying (`/Game/Maps/TestMap/Kitayama/UI_Kitayama/Widget_UI/TutorialWidget/UMG_SignStage1_Tutorial.IsPlayingAnimCheck` (`self.Tutorial`)))
      (if (not _isplaying)
        (`/Game/Maps/TestMap/Kitayama/UI_Kitayama/Widget_UI/TutorialWidget/UMG_SignStage1_Tutorial.PlayUnDisp` (`self.Tutorial`))
        (set `self.bIsDisp` false)
        (`GameplayStatics.PlaySound2D` "/Game/Resource/SO/SE/UI/SO_SE_UI_Back_Cue.SO_SE_UI_Back_Cue" 1.0 1.0 0.0 null null) ; 効果音再生
      ))))

(event `InputAction|UI_Right` :consume false
  (params (Key :type "Key Structure"))
  (:`Pressed`
    (if (`self.bIsDisp`)
      (`/Game/Maps/TestMap/Kitayama/UI_Kitayama/Widget_UI/TutorialWidget/UMG_SignStage1_Tutorial.ChangePage` (`self.Tutorial`) true))))

(event `InputAxis|UI_Stick_X` :consume false
  (params (AxisValue :type "Float (single-precision)"))
  (if (> AxisValue (`self.StickX`))
    (`KismetSystemLibrary.Delay` 0.5)
    (if (`self.bIsDisp`)
      (`/Game/Maps/TestMap/Kitayama/UI_Kitayama/Widget_UI/TutorialWidget/UMG_SignStage1_Tutorial.ChangePage` (`self.Tutorial`) true))
    (elif (< AxisValue (* (`self.StickX`) -1.0))
      (`KismetSystemLibrary.Delay` 0.5)
      (if (`self.bIsDisp`)
        (`/Game/Maps/TestMap/Kitayama/UI_Kitayama/Widget_UI/TutorialWidget/UMG_SignStage1_Tutorial.ChangePage` (`self.Tutorial`) false)))))

(event `InputAction|UI_Left` :consume false
  (params (Key :type "Key Structure"))
  (:`Pressed`
    (if (`self.bIsDisp`)
      (`/Game/Maps/TestMap/Kitayama/UI_Kitayama/Widget_UI/TutorialWidget/UMG_SignStage1_Tutorial.ChangePage` (`self.Tutorial`) false))))

(fn `UMGAdd Toview`
  (if (`self.bIsDisp`)
    _
    (elif (not (`Widget.IsInViewport` (`self.Tutorial`)))
      (bind _isplaying (`/Game/Maps/TestMap/Kitayama/UI_Kitayama/Widget_UI/TutorialWidget/UMG_SignStage1_Tutorial.IsPlayingAnimCheck` (`self.Tutorial`)))
      (if (not _isplaying)
        (`UserWidget.AddToViewport` (`self.Tutorial`) 0)
        (set `self.bIsDisp` true)
        (`GameplayStatics.PlaySound2D` "/Game/Resource/SO/SE/UI/Pause/SO_SE_Pause_Start_Cue.SO_SE_Pause_Start_Cue" 1.0 1.0 0.0 null null) ; 効果音再生
      ))))

(fn `UserConstructionScript`)