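; AI controller for the dragon that sets up BB_Dragon and runs the BT_Dragon behavior tree on BeginPlay.
; Its RotateTo function turns the controlled pawn toward a target position at a constant RotationSpeed, using XY-flattened locations to ignore height.
; Each call takes one frame-delta step and returns false, or returns true if the pawn already faces the target.
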(event `self.ReceiveBeginPlay`
  (`self.UseBlackboard` "/Game/Blueprints/Dragon/AI/BB_Dragon.BB_Dragon")
  (`self.RunBehaviorTree` "/Game/Blueprints/Dragon/AI/BT_Dragon.BT_Dragon"))

(fn `RotateTo`
  (params (TargetPos :type "Vector Structure"))
  (returns (Done :type Boolean))
  (locals (RotationSpeed :type "Float (double-precision)" :default 100.0) (CurrentRot :type "Rotator Structure") (TargetRot :type "Rotator Structure"))
  (bind _returnvalue (`self.K2_GetPawn`))
  (set `local.CurrentRot` (`self.K2_GetActorRotation` _returnvalue))
  (set `local.TargetRot` (`KismetMathLibrary.FindLookAtRotation` (`/Game/Blueprints/BP_FuncLibrary.Vector to 2D(XY)` (`self.K2_GetActorLocation` _returnvalue)) (`/Game/Blueprints/BP_FuncLibrary.Vector to 2D(XY)` TargetPos)))
  (if (!= (`local.CurrentRot`) (`local.TargetRot`) :`ErrorTolerance` 0.001)
    (`self.K2_SetActorRotation` _returnvalue (`KismetMathLibrary.RInterpTo_Constant` (`local.CurrentRot`) (`local.TargetRot`) (`GameplayStatics.GetWorldDeltaSeconds`) (`local.RotationSpeed`)) false)
    (return false)
    (else
      (return true))))

(fn `UserConstructionScript`)