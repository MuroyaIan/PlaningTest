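; BP_Dragon_MeteorCrystal is a crystal hazard, named as part of the Dragon's meteor, that knocks back and damages the player on contact.
; It takes a random yaw on BeginPlay and reacts when BP_Player overlaps its capsule collider.
; The overlap records the hit position on the player and launches them horizontally away, briefly ignoring Pawn collision on their capsule.
; After that short delay it restores blocking, applies damage and destroys itself.
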(event `self.ReceiveBeginPlay`
  (`self.K2_SetActorRotation` (`KismetMathLibrary.MakeRotator` 0.0 0.0 (`KismetMathLibrary.RandomFloatInRange` 0.0 360.0))))

(event `self.CapsuleCollider.OnComponentBeginOverlap`
  (params (OverlappedComponent :type "PrimitiveComponent Object Reference") (OtherActor :type "Actor Object Reference") (OtherComp :type "PrimitiveComponent Object Reference") (OtherBodyIndex :type Integer) (bFromSweep :type Boolean) (SweepResult :type "HitResult Structure (by ref)"))
  (bind _asbp_player (cast `/Game/Blueprints/Player/BP_Player` OtherActor))
  (bind _output_get (set `/Game/Blueprints/Player/BP_Player.DamagePos` (`SceneComponent.K2_GetComponentLocation` OverlappedComponent) _asbp_player))
  (`PrimitiveComponent.SetCollisionResponseToChannel` (`Character.CapsuleComponent` _asbp_player) "ECC_Pawn" "ECR_Ignore")
  (`Character.LaunchCharacter` _asbp_player (* (`/Game/Blueprints/BP_FuncLibrary.Vector to 2D(NormalizeXY)` (`KismetMathLibrary.GetDirectionUnitVector` _output_get (`self.K2_GetActorLocation` _asbp_player))) 1000.0) false false)
  (`KismetSystemLibrary.Delay` 0.1)
  (`PrimitiveComponent.SetCollisionResponseToChannel` (`Character.CapsuleComponent` _asbp_player) "ECC_Pawn" "ECR_Block")
  (`GameplayStatics.ApplyDamage` _asbp_player 2.0)
  (`self.K2_DestroyActor`))

(fn `UserConstructionScript`)