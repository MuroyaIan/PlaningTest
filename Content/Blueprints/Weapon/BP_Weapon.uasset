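; Player slime weapon that sucks up slime into a flask and fires it as spread bullets, with suction taking priority.
; It follows the player's weapon socket and aims bullets via a camera trace.
; Controller input drives a looping fire timer and a spawned detector's scan, with VFX, rumble and pipe/flask material feedback.
; AddSlime and FireBullet adjust flask capacity, but Tick resets it to a fixed value every frame.
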(event `self.ReceiveBeginPlay`
  (bind _playercontroller (`self.GetUserController`))
  (`|ExecutionSequence`
    (:`then_0`
      (add `self.AimOn` (`|CreateDelegate` _playercontroller :!event `AimOn`))
      (add `self.AimOff` (`|CreateDelegate` _playercontroller :!event `AimOff`))
      (add `/Game/Blueprints/Player/BP_PlayerController.SuckOn` _playercontroller (`|CreateDelegate` :!event `StartSuck`))
      (add `/Game/Blueprints/Player/BP_PlayerController.SuckOff` _playercontroller (`|CreateDelegate` :!event `EndSuck`))
      (add `/Game/Blueprints/Player/BP_PlayerController.FireOn` _playercontroller (`|CreateDelegate` :!event `StartFire`))
      (add `/Game/Blueprints/Player/BP_PlayerController.FireOff` _playercontroller (`|CreateDelegate` :!event `EndFire`)))
    (:`then_1`
      (bind _returnvalue (`|SpawnActorFromClass` "/Game/Blueprints/Weapon/BP_Detector.BP_Detector_C" (`self.GetTransform`) "Undefined" "OverrideRootScale" null (`|ConvertAsset` self) null)) ; スキャン機生成
      (add `self.ScanOn` (`|CreateDelegate` _returnvalue :!event `StartScan`))
      (add `self.ScanOff` (`|CreateDelegate` _returnvalue :!event `EndScan`))
      (set `self.Detector` (`|ConvertAsset` _returnvalue)) ; 参照設定
    )
    (:`then_2`
      (`self.SetLocation`)
      (`self.SetRotation`))))

(event `self.ReceiveTick`
  (params (DeltaSeconds :type "Float (single-precision)"))
  (`self.SetLocation`)
  (`self.SetRotation`)
  (set `self.AimMode` (`/Game/Blueprints/Player/BP_PlayerController.AimMode` (`self.GetUserController`))) ; 照準確認
  (`self.UpdateFlask`)
  (`self.UpdateAimPos`)
  (`self.PrintWeaponInfo`)
  (set `self.Flask_Capacity` 0.2))

(event `StartSuck`
  ;[1 0.5365 0.9316] 吸込み＆吐出し切替
  (if (`self.UseFire`)
    (`self.EndFire`) ; 射撃中吸込みへ切替
    (set `self.UseFire` true))
  (set `self.UseSuck` true)
  (`self.AimOn`)
  (`self.ScanOn`) ; 吸込みモード開始
)

(event `EndSuck`
  ;[1 0.5365 0.9316] 吸込み＆吐出し切替
  (set `self.UseSuck` false)
  (`self.AimOff`)
  (`self.ScanOff`) ; 吸込みモード終了
  (if (`self.bSuckSuccess`)
    (set `self.bSuckSuccess` false) ; モーション終了
  )
  (if (`self.UseFire`)
    (`self.StartFire`)
    (else
      (`/Game/Blueprints/Player/BP_Player.UpdatePipeMID` (`/Game/Blueprints/Player/BP_PlayerController.GetPlayerPawn` (`self.GetUserController`)) false false) ; チューブFX終了
    )))

(event `StartFire`
  ;[1 0.5365 0.9316] 吸込み＆吐出し切替
  (set `self.UseFire` true)
  (if (not (`self.UseSuck`))
    (`self.AimOn`)
    (`KismetSystemLibrary.K2_SetTimer` null "FireBullet" (`self.FireSpeed`) true) ; 弾発射（連射）
  ))

(event `EndFire`
  ;[1 0.5365 0.9316] 吸込み＆吐出し切替
  (set `self.UseFire` false)
  (if (not (`self.UseSuck`))
    (`self.AimOff`)
    (`KismetSystemLibrary.K2_ClearTimer` null "FireBullet") ; 弾発射停止
    (if (`self.bFireSuccess`)
      (set `self.bFireSuccess` false) ; モーション終了
      (`self.MakeVibration` false true) ; 振動処理オフ
      (`/Game/Blueprints/Player/BP_Player.UpdatePipeMID` (`/Game/Blueprints/Player/BP_PlayerController.GetPlayerPawn` (`self.GetUserController`)) false false) ; チューブFX終了
    )))

(event `AddSlime`
  ;[0.5 0.9194 1] フラスコ容量制御
  (`NiagaraFunctionLibrary.SpawnSystemAttached` "/Game/Resource/FX/VFX/Granet/FX_VFX_PlayerAbsorption.FX_VFX_PlayerAbsorption" (`self.Box`) "None" (0.0 0.0 30.0) (struct :`Pitch` 90.0) "KeepRelativeOffset" true) ; エフェクト再生
  (if (< (`self.Flask_Capacity`) (`self.Flask_MaxCapacity`))
    (set `self.Flask_Capacity` (+ (`self.Flask_Capacity`) 0.02)) ; フラスコ容量を増やす
    (if (`self.UseSuck`)
      (set `self.bSuckSuccess` true) ; モーション開始
      (`self.MakeVibration` true) ; 振動処理オン（吐出し）
      (`/Game/Blueprints/Player/BP_Player.UpdatePipeMID` (`/Game/Blueprints/Player/BP_PlayerController.GetPlayerPawn` (`self.GetUserController`)) true true) ; チューブFX更新
    )))

(event `UpdateAimPos`
  (bind _cameramanager (`/Game/Blueprints/Player/BP_PlayerController.GetCameraManager` (`self.GetUserController`)))
  (bind _returnvalue (`PlayerCameraManager.GetCameraLocation` _cameramanager))
  (bind _value (`/Game/Blueprints/Player/BP_PlayerCameraManager.GetForwardVector` _cameramanager))
  ;[1 1 1] 照準中心決め
  (bind (_outhit _returnvalue_2) (`KismetSystemLibrary.LineTraceSingle` _returnvalue (+ _returnvalue (* _value 2500.0)) "TraceTypeQuery2")) ; 照準位置検索
  (if _returnvalue_2
    (bind (_bblockinghit _binitialoverlap _time _distance _location) (`GameplayStatics.BreakHitResult` _outhit))
    (if (> (`KismetMathLibrary.Vector_Distance` (`self.K2_GetActorLocation`) _location) 175.0)
      (set `self.AimPos` _location) ; 照準位置設定
      (else
        (set `self.AimPos` (+ _returnvalue (* _value 10000.0)) :!label _label)))
    (else
      (goto _label)))
  (if (not (`self.bSuckBoss`))
    (set `self.AimRotation` (`KismetMathLibrary.FindLookAtRotation` (`self.K2_GetActorLocation`) (`self.AimPos`))) ; 照準回転設定
  ))

(event `UpdateFlask`
  (bind _returnvalue (`KismetMathLibrary.FCeil` (/ (`self.Flask_Capacity`) 0.125)))
  ;[0.5 0.9194 1] フラスコ容量制御
  (if (!= (`self.Flask_Level`) _returnvalue)
    (bind _output_get (set `self.Flask_Level` _returnvalue)) ; フラスコ容量更新
    (`/Game/Blueprints/Player/BP_Player.UpdateFlaskMID` (`/Game/Blueprints/Player/BP_PlayerController.GetPlayerPawn` (`self.GetUserController`)) _output_get) ; マテリアル更新
  ))

(event `MakeVibration`
  (params (UseVibration :type Boolean) (Fire :type Boolean))
  (bind _playercontroller (`self.GetUserController`))
  ;[0.526 1 0.6228] 振動処理
  (if Fire
    (if UseVibration
      (`PlayerController.K2_ClientPlayForceFeedback` _playercontroller "/Game/Blueprints/Weapon/Vibration_Weapon_Fire.Vibration_Weapon_Fire" "None" true false false)
      (else
        (`PlayerController.ClientStopForceFeedback` _playercontroller "/Game/Blueprints/Weapon/Vibration_Weapon_Fire.Vibration_Weapon_Fire" "None")))
    (elif UseVibration
      (`PlayerController.K2_ClientPlayForceFeedback` _playercontroller "/Game/Blueprints/Weapon/Vibration_Weapon_Fire.Vibration_Weapon_Fire" "None" false false false))))

(fn `FireBullet`
  (if (> (`self.Flask_Capacity`) 0.0)
    (bind _returnvalue (`|SpawnActorFromClass` "/Game/Blueprints/Slime/BP_Slime_Small.BP_Slime_Small_C" (`KismetMathLibrary.MakeTransform` (+ (`self.K2_GetActorLocation`) (* (`self.GetActorUpVector`) 60)) (`KismetMathLibrary.ComposeRotators` (`self.AimRotation`) (`KismetMathLibrary.MakeRotator` (`KismetMathLibrary.RandomFloatInRange` -4.0 4.0) (`KismetMathLibrary.RandomFloatInRange` -4.0 4.0) (`KismetMathLibrary.RandomFloatInRange` -4.0 4.0)))) "Undefined" "OverrideRootScale" null null)) ; 弾生成
    (if (`KismetSystemLibrary.IsValid` _returnvalue)
      (`/Game/Blueprints/Slime/BP_Slime_Small.SetToBullet` _returnvalue) ; 弾モードへ移行
      (set `self.Flask_Capacity` (- (`self.Flask_Capacity`) 0.02)) ; フラスコ容量を減らす
      (`NiagaraFunctionLibrary.SpawnSystemAttached` "/Game/Resource/FX/VFX/Granet/FX_VFX_Player_Shot.FX_VFX_Player_Shot" (`self.Box`) "None" (0.0 0.0 20.0) (struct :`Pitch` 90.0) "KeepRelativeOffset" true) ; エフェクト再生
      (if (not (`self.bFireSuccess`))
        (set `self.bFireSuccess` true) ; モーション開始
        (`self.MakeVibration` true true) ; 振動処理オン
        (`/Game/Blueprints/Player/BP_Player.UpdatePipeMID` (`/Game/Blueprints/Player/BP_PlayerController.GetPlayerPawn` (`self.GetUserController`)) true false) ; チューブFX更新
      ))
    (elif (`self.bFireSuccess`)
      (set `self.bFireSuccess` false) ; モーション終了
      (`self.MakeVibration` false true) ; 振動処理オフ
      (`/Game/Blueprints/Player/BP_Player.UpdatePipeMID` (`/Game/Blueprints/Player/BP_PlayerController.GetPlayerPawn` (`self.GetUserController`)) false false) ; チューブFX更新
    )))

(fn `GetDetector`
  (returns (Detector :type "/Game/Blueprints/Weapon/BP_Detector Object Reference"))
  (bind _detector (`self.Detector`))
  (if (`KismetSystemLibrary.IsValidSoftObjectReference` _detector)
    (return (`|ConvertAsset` _detector))))

(fn `GetUserController`
  (returns (PlayerController :type "/Game/Blueprints/Player/BP_PlayerController Object Reference"))
  (bind _asbp_player_controller (cast `/Game/Blueprints/Player/BP_PlayerController` (`GameplayStatics.GetPlayerController` 0)))
  (return _asbp_player_controller))

(fn `PrintWeaponInfo`
  (bind _bdebug (`/Game/Blueprints/BP_FuncLibrary.CheckDebugPrint`))
  (if _bdebug
    (`KismetSystemLibrary.PrintString` (`KismetStringLibrary.Concat_StrStr` "[WeaponInfo] \nSuckMode:" (`KismetStringLibrary.Conv_BoolToString` (`self.UseSuck`)) " \nFireMode:" (`KismetStringLibrary.Conv_BoolToString` (`self.UseFire`)) " \nFlaskLevell:" (`KismetStringLibrary.Conv_IntToString` (`self.Flask_Level`)) " \nFlaskCapacity:" (`KismetStringLibrary.Conv_DoubleToString` (`self.Flask_Capacity`))) true false (struct :`R` 1.0 :`G` 0.078368 :`A` 1.0) 0.0)))

(fn `SetLocation`
  (bind _mesh (`Character.Mesh` (`/Game/Blueprints/Player/BP_PlayerController.GetPlayerPawn` (`self.GetUserController`))))
  (`self.K2_SetActorLocation` (+ (`SceneComponent.GetSocketLocation` _mesh "JNT_weapon3") (* (`KismetMathLibrary.GetForwardVector` (`SceneComponent.GetSocketRotation` _mesh "JNT_weapon3")) 9))))

(fn `SetRotation`
  (bind _returnvalue (`SceneComponent.GetSocketRotation` (`Character.Mesh` (`/Game/Blueprints/Player/BP_PlayerController.GetPlayerPawn` (`self.GetUserController`))) "JNT_weapon3"))
  (`self.K2_SetActorRotation` (`KismetMathLibrary.ComposeRotators` _returnvalue (`KismetMathLibrary.RotatorFromAxisAndAngle` (`.Y` (`KismetMathLibrary.GetAxes` _returnvalue)) 90.0))))

(fn `UserConstructionScript`)

(fn `Vibration01`
  (bind _returnvalue (`KismetMathLibrary.Now`))
  (if (<= (`KismetMathLibrary.GetTotalSeconds` (- _returnvalue (`self.SuctionTime`))) (`self.MinDurationTime`))
    (set `self.VibrationIndex` 0)
    (else
      (set `self.VibrationIndex` 1)))
  (`PlayerController.K2_ClientPlayForceFeedback` (`self.GetUserController`) (`|GetArrayItem` (`self.FFEffectPattern`) (`self.VibrationIndex`)) "None" false false false)
  (set `self.SuctionTime` _returnvalue))

(fn `Vibration02`
  (bind _returnvalue (`KismetMathLibrary.Now`))
  (if (<= (`KismetMathLibrary.GetTotalSeconds` (- _returnvalue (`self.SuctionTime`))) 0.3)
    (set `self.VibrationIndex` 2)
    (else
      (set `self.VibrationIndex` 3)))
  (`PlayerController.K2_ClientPlayForceFeedback` (`self.GetUserController`) (`|GetArrayItem` (`self.FFEffectPattern`) (`self.VibrationIndex`)) "None" false false false)
  (set `self.SuctionTime` _returnvalue))