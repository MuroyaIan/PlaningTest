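; Game mode for the stage select screen that sets up its audio and UI.
; On BeginPlay it spawns a BP_Audio actor, starts the stage-select BGM and background SE with fade-ins, then spawns BP_StageSelectUI.
; Play functions stop any current sound before restarting their BGMPlayer or SEPlayer, and StopAudio fades out both players.
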(event `self.ReceiveBeginPlay`
  (bind _returnvalue (`|SpawnActorFromClass` "/Game/Blueprints/System/BP_Audio.BP_Audio_C" (`KismetMathLibrary.MakeTransform` (0.0 0.0 0.0)) "Undefined" "OverrideRootScale" null null))
  (set `self.Actor_Audio` (`|ConvertAsset` _returnvalue))
  (bind _bgm_player (`self.PlayBGM` "/Game/Resource/SO/BGM/Other/SO_BGM_StageSelect_Cue.SO_BGM_StageSelect_Cue"))
  (`AudioComponent.FadeIn` _bgm_player 2.0 1.0 0.0 "Linear")
  (bind _se_player (`self.PlaySE_BG`))
  (`AudioComponent.FadeIn` _se_player 2.0 1.0 0.0 "Linear")
  (`self.InitStageSelectUI`))

(fn `InitStageSelectUI`
  (bind _returnvalue (`|SpawnActorFromClass` "/Game/Blueprints/System/BP_UI/BP_StageSelectUI.BP_StageSelectUI_C" (`KismetMathLibrary.MakeTransform` (0.0 0.0 0.0)) "Undefined" "OverrideRootScale" null null))
  (set `self.Actor_StageSelectUI` (`|ConvertAsset` _returnvalue)))

(fn `PlayBGM`
  (params (BGM_Cue :type "SoundCue Object Reference"))
  (returns (BGM_Player :type "AudioComponent Object Reference"))
  (bind _bgm_player (`self.BGM_Player`))
  (if (`AudioComponent.IsPlaying` _bgm_player)
    (`AudioComponent.Stop` _bgm_player) ; BGM停止
  )
  (`AudioComponent.SetSound` _bgm_player BGM_Cue) ; BGM変更
  (`AudioComponent.Play` _bgm_player 0.0) ; BGM開始
  (return _bgm_player))

(fn `PlaySE_BG`
  (returns (SE_Player :type "AudioComponent Object Reference"))
  (bind _se_player (`self.SE_Player`))
  (if (`AudioComponent.IsPlaying` _se_player)
    (`AudioComponent.Stop` _se_player) ; BGM停止
  )
  (`AudioComponent.Play` _se_player 0.0) ; BGM開始
  (return _se_player))

(fn `StopAudio`
  (bind _bgm_player (`self.BGM_Player`))
  (bind _se_player (`self.SE_Player`))
  (`|ExecutionSequence`
    (:`then_0`
      (if (`AudioComponent.IsPlaying` _bgm_player)
        (`AudioComponent.FadeOut` _bgm_player 2.0 0.0 "Linear")))
    (:`then_1`
      (if (`AudioComponent.IsPlaying` _se_player)
        (`AudioComponent.FadeOut` _se_player 2.0 0.0 "Linear")))))

(fn `UserConstructionScript`)