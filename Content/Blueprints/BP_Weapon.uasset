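; BP_Weapon is a weapon actor that floats beside and above the player, spins, and responds to aim mode.
; Each tick it repositions from the player's right and up vectors, then resets its rotation to an accumulating yaw that advances faster while aiming.
; The controller's AimMode flag also swaps the Nozzle's laser pointer material and plays or reverses the ReadyToAttack timeline, which adds pitch and player yaw.
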(event `self.ReceiveBeginPlay`
  (`self.SetLocation`)
  (`self.SetRotation`))

(event `self.ReceiveTick`
  (params (DeltaSeconds :type "Float (single-precision)"))
  (`self.SetLocation`)
  (`self.SetRotation`)
  (`self.AimMode`))

(event `AimMode`
  (bind _nozzle (`self.Nozzle`))
  (if (`/Game/Blueprints/System/BP_PlayerController.AimMode` (cast `/Game/Blueprints/System/BP_PlayerController` (`GameplayStatics.GetPlayerController` 0) :!pure true))
    (`PrimitiveComponent.SetMaterial` _nozzle 0 "/Engine/VREditor/LaserPointer/LaserPointerMaterial.LaserPointerMaterial") ; マテリアル切替
    (bind (_direction _weaponrotation_pitch_) (`Timeline|ReadyToAttack` :!label _label)
      (:`Update`
        (`self.K2_AddActorWorldRotation` (`KismetMathLibrary.MakeRotator` 0.0 _weaponrotation_pitch_ (.yaw (`self.K2_GetActorRotation` (`GameplayStatics.GetPlayerPawn` 0))))) ; 照準用回転を追加
      ))
    (else
      (`PrimitiveComponent.SetMaterial` _nozzle 0 "/Engine/VREditor/LaserPointer/LaserPointerMaterial_Inst.LaserPointerMaterial_Inst")
      (goto _label :!via `Reverse`))))

(fn `SetLocation`
  (bind _asbp_player (cast `/Game/Blueprints/BP_Player` (`GameplayStatics.GetPlayerPawn` 0) :!pure true))
  (`self.K2_SetActorLocation` (+ (+ (`self.K2_GetActorLocation` _asbp_player) (* (`/Game/Blueprints/BP_FuncLibrary.Vector to 2D(NormalizeXY)` (`self.GetActorRightVector` _asbp_player)) 40)) (* (`KismetMathLibrary.Normal` (`KismetMathLibrary.MakeVector` 0.0 0.0 (.z (`self.GetActorUpVector` _asbp_player)))) 100))))

(fn `SetRotation`
  (if (`/Game/Blueprints/System/BP_PlayerController.AimMode` (cast `/Game/Blueprints/System/BP_PlayerController` (`GameplayStatics.GetPlayerController` 0) :!pure true))
    (set `self.RotateAngle` (+ (`self.RotateAngle`) 4.0)) ; 武器を自転させる
    (else
      (set `self.RotateAngle` (+ (`self.RotateAngle`) 2.0))))
  (if (== (`self.RotateAngle`) 360.0)
    (set `self.RotateAngle` 0.0) ; 自転角度をリセット
  )
  (`self.K2_SetActorRotation` (`KismetMathLibrary.MakeRotator` 0.0 0.0 (`self.RotateAngle`))))

(fn `UserConstructionScript`)