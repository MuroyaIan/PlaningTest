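; Destructible prop that shatters when an actor tagged "Golem" overlaps its static mesh.
; On overlap it destroys the static mesh and adds a destructible component using the mesh in DestMeshSlot.
; It then applies damage along the golem's forward vector, with DesrPower as both damage and impulse strength.
; The actor destroys itself after a short delay.
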(event `self.ReceiveBeginPlay`)

(event `self.StaticMesh.OnComponentBeginOverlap`
  (params (OverlappedComponent :type "PrimitiveComponent Object Reference") (OtherActor :type "Actor Object Reference") (OtherComp :type "PrimitiveComponent Object Reference") (OtherBodyIndex :type Integer) (bFromSweep :type Boolean) (SweepResult :type "HitResult Structure (by ref)"))
  (bind _desrpower (`self.DesrPower`))
  (if (`self.ActorHasTag` OtherActor "Golem")
    (`ActorComponent.K2_DestroyComponent` (`self.StaticMesh`))
    (bind _returnvalue (`AddComponent|NODE_AddDestructibleComponent-0`)) ; 破壊メッシュ置換
    (`DestructibleComponent.SetDestructibleMesh` _returnvalue (`self.DestMeshSlot`))
    (`DestructibleComponent.ApplyDamage` _returnvalue _desrpower (`SceneComponent.K2_GetComponentLocation` _returnvalue) (`self.GetActorForwardVector` OtherActor) _desrpower) ; ダメージ設定
    (`KismetSystemLibrary.Delay` 5.0) ; 消滅処理
    (`self.K2_DestroyActor`)))

(fn `UserConstructionScript`)