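; Player camera manager that drives an orbiting third-person camera around the view target's chest height, with smoothed rotation, offset and FOV.
; Tick eases rotation, offset and FOV toward their target values with fixed-alpha lerps and prints debug camera info on screen.
; BlueprintUpdateCamera rotates the offset around the chest point and looks back at it.
; Yaw and clamped pitch inputs adjust the target rotation only while control is enabled.
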(event `self.ReceiveBeginPlay`
  (set `self.Rotation` (`self.TargetRotation`)) ; 回転値初期化
  (set `self.Location` (`self.TargetLocation`)) ; 位置修正初期化
  (set `self.FOV` (`self.TargetFOV`)) ; 視野角初期化
)

(event `self.ReceiveTick`
  (params (DeltaSeconds :type "Float (single-precision)"))
  (bind _output_get (set `self.Rotation` (`KismetMathLibrary.RLerp` (`self.Rotation`) (`self.TargetRotation`) 0.25 true))) ; 回転値更新
  (bind _output_get_2 (set `self.Location` (`KismetMathLibrary.VLerp` (`self.Location`) (`self.TargetLocation`) 0.25))) ; 位置修正更新
  (bind _output_get_3 (set `self.FOV` (`KismetMathLibrary.Lerp` (`self.FOV`) (`self.TargetFOV`) 0.25))) ; 視野角更新
  (`KismetSystemLibrary.PrintString` (`KismetStringLibrary.Concat_StrStr` "[CameraInfo] \nPitchAngle:" (`KismetStringLibrary.Conv_IntToString` (`KismetMathLibrary.Round` (.pitch _output_get))) " \nDistance:" (`KismetStringLibrary.Conv_IntToString` (`KismetMathLibrary.Round` (`KismetMathLibrary.VSize` _output_get_2))) " \nFOV:" (`KismetStringLibrary.Conv_IntToString` (`KismetMathLibrary.Round` _output_get_3))) true false (struct :`R` 1.0 :`A` 1.0) 0.0))

(fn `AddPitchInput`
  (params (Value :type "Float (double-precision)"))
  (if (`self.ControlOn`)
    (set `self.TargetRotation` (`KismetMathLibrary.MakeRotator` (.roll (`self.TargetRotation`)) (`KismetMathLibrary.ClampAngle` (+ (.pitch (`self.TargetRotation`)) Value) (`self.ViewPitchMin`) (`self.ViewPitchMax`)) (.yaw (`self.TargetRotation`))))))

(fn `AddYawInput`
  (params (Value :type "Float (double-precision)"))
  (if (`self.ControlOn`)
    (set `self.TargetRotation` (`KismetMathLibrary.MakeRotator` (.roll (`self.TargetRotation`)) (.pitch (`self.TargetRotation`)) (+ (.yaw (`self.TargetRotation`)) Value)))))

(fn `BlueprintUpdateCamera`
  (params (CameraTarget :type "Actor Object Reference"))
  (returns (NewCameraLocation :type "Vector Structure") (NewCameraRotation :type "Rotator Structure") (NewCameraFOV :type "Float (double-precision)") (ReturnValue :type Boolean))
  (bind _returnvalue (`KismetMathLibrary.MakeVector` (.x (`self.K2_GetActorLocation` CameraTarget)) (.y (`self.K2_GetActorLocation` CameraTarget)) (+ (.z (`self.K2_GetActorLocation` CameraTarget)) (`self.ChestOffset`))))
  (bind _returnvalue_2 (+ _returnvalue (`KismetMathLibrary.GreaterGreater_VectorRotator` (`self.Location`) (`self.Rotation`))))
  (return _returnvalue_2 (`KismetMathLibrary.FindLookAtRotation` _returnvalue_2 _returnvalue) (`self.FOV`) true))

(fn `GetForwardVector`
  (returns (Value :type "Vector Structure"))
  (return (`KismetMathLibrary.GetForwardVector` (`self.GetCameraRotation`))))

(fn `GetRightVector`
  (returns (Value :type "Vector Structure"))
  (return (`KismetMathLibrary.GetRightVector` (`self.GetCameraRotation`))))

(fn `UserConstructionScript`)