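; BP_PauseUI is an input-enabled Blueprint that controls a pause menu widget.
; On BeginPlay it enables input from BP_PlayerController, then PauseUI_Disp toggles the widget on and off the viewport via IsDispUI.
; While shown, Up, Down and Confirm inputs forward to the widget's SelectMenu and DecidedMenu, which handle the menu logic.
; The game is not paused here, and the DispWidget helper is unused by these events.
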(event `self.ReceiveBeginPlay`
  (bind _asbp_player_controller (cast `/Game/Blueprints/Player/BP_PlayerController` (`GameplayStatics.GetPlayerController` 0)))
  (`self.EnableInput` _asbp_player_controller) ; 入力有効化
)

(event `InputAction|PauseUI_Disp`
  (params (Key :type "Key Structure"))
  (:`Pressed`
    (set `self.isDispUI` (not (`self.isDispUI`)))
    (if (`self.isDispUI`)
      (set `self.isDispUI` true)
      (`UserWidget.AddToViewport` (`self.GetWidget`) 0)
      (else
        (set `self.isDispUI` false)
        (`Widget.RemoveFromParent` (`self.GetWidget`))))))

(event `InputAction|UI_Confirm` :consume false
  (params (Key :type "Key Structure"))
  (:`Pressed`
    (if (`self.isDispUI`)
      (`/Game/Maps/TestMap/Kitayama/UI_Kitayama/Widget_UI/PauseWidget/UMG_PauseMenu.DecidedMenu` (`self.GetWidget`)))))

(event `InputAction|UI_Up` :consume false
  (params (Key :type "Key Structure"))
  (:`Pressed`
    (if (`self.isDispUI`)
      (`/Game/Maps/TestMap/Kitayama/UI_Kitayama/Widget_UI/PauseWidget/UMG_PauseMenu.SelectMenu` (`self.GetWidget`) false))))

(event `InputAction|UI_Down` :consume false
  (params (Key :type "Key Structure"))
  (:`Pressed`
    (if (`self.isDispUI`)
      (`/Game/Maps/TestMap/Kitayama/UI_Kitayama/Widget_UI/PauseWidget/UMG_PauseMenu.SelectMenu` (`self.GetWidget`) true))))

(fn `DispWidget`
  (params (Widget :type "UserWidget Object Reference") (IsDisp :type Boolean))
  (returns (ReturnIsDisp :type Boolean))
  (if IsDisp
    (`Widget.RemoveFromParent` Widget) ; UIの非表示にする
    (else
      (`UserWidget.AddToViewport` Widget 0) ; UIを表示する
    ))
  (return (not IsDisp)))

(fn `GetWidget`
  (returns (Widget_PauseUI :type "/Game/Maps/TestMap/Kitayama/UI_Kitayama/Widget_UI/PauseWidget/UMG_PauseMenu Object Reference"))
  (return (`|ConvertAsset` (`self.Widget_PauseUI`))))

(fn `UserConstructionScript`)