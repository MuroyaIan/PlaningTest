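; BP_LoseUI is an actor that shows and controls the lose screen menu.
; It creates the UMG_LoseMaster widget at BeginPlay, and Tick adds or removes it according to IsDispUI, playing its display animation when added.
; A Delay of the widget's DispTime feeds a DoOnce that unlocks input.
; Up and Down both call SelectMenu, and Confirm calls DecideMenu on the widget.
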(event `self.ReceiveBeginPlay`
  (bind _asbp_player_controller (cast `/Game/Blueprints/Player/BP_PlayerController` (`GameplayStatics.GetPlayerController` 0)))
  (`self.EnableInput` _asbp_player_controller) ; 入力有効化
  (bind _returnvalue (`|CreateWidget` "/Game/Maps/TestMap/Kitayama/UI_Kitayama/Widget_UI/PauseWidget/UMG_LoseMaster.UMG_LoseMaster_C"))
  (set `self.Widget_LoseUI` _returnvalue))

(event `self.ReceiveTick`
  (params (DeltaSeconds :type "Float (single-precision)"))
  (bind _widget_loseui (`self.Widget_LoseUI`))
  (bind _returnvalue (`Widget.IsInViewport` (`self.Widget_LoseUI`)))
  (if (`self.isDispUI`)
    (if _returnvalue
      (`KismetSystemLibrary.Delay` (`/Game/Maps/TestMap/Kitayama/UI_Kitayama/Widget_UI/PauseWidget/UMG_LoseMaster.DispTime` (`self.Widget_LoseUI`)))
      (`/Engine/EditorBlueprintResources/StandardMacros.DoOnce` false
        (:`Completed`
          (set `self.CanInput` true)))
      (else
        (`UserWidget.AddToViewport` _widget_loseui 2)
        (`/Game/Maps/TestMap/Kitayama/UI_Kitayama/Widget_UI/PauseWidget/UMG_LoseMaster.DispAnim` _widget_loseui)))
    (elif _returnvalue
      (`Widget.RemoveFromParent` (`self.Widget_LoseUI`)))))

(event `ChangeDisp`
  (params (Disp :type Boolean))
  (set `self.isDispUI` Disp))

(event `InputAction|UI_Confirm` :consume false
  (params (Key :type "Key Structure"))
  (:`Pressed`
    (if (and (`self.isDispUI`) (`self.CanInput`))
      (`/Game/Maps/TestMap/Kitayama/UI_Kitayama/Widget_UI/PauseWidget/UMG_LoseMaster.DecideMenu` (`self.Widget_LoseUI`)))))

(event `InputAction|UI_Up` :consume false
  (params (Key :type "Key Structure"))
  (:`Pressed`
    (if (and (`self.isDispUI`) (`self.CanInput`)) :!label _label
      (`/Game/Maps/TestMap/Kitayama/UI_Kitayama/Widget_UI/PauseWidget/UMG_LoseMaster.SelectMenu` (`self.Widget_LoseUI`)))))

(event `InputAction|UI_Down` :consume false
  (params (Key :type "Key Structure"))
  (:`Pressed`
    (goto _label)))

(fn `DispUI`
  (if (not (`Widget.IsInViewport` (`self.Widget_LoseUI`)))
    (`self.ChangeDisp` true)))

(fn `UserConstructionScript`)