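; BP_DragonSpawnPoint is a spawn point Blueprint that maintains a list of slimes and a spawn cooldown, with no spawning logic of its own.
; Every Tick it removes invalid entries from the Slime array while iterating over it.
; It also checks the cooldown flag each Tick and, when set, clears it after a Delay of SpawnCooleTime.
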(event `self.ReceiveTick`
  (params (DeltaSeconds :type "Float (single-precision)"))
  ;[1 0 0] tick
  (`self.Chack_Slime`) ; スライムの状態確認
  (`self.Chack_Cooltime`) ; クールタイム確認
)

(event `Chack_Slime`
  (bind _slime (`self.Slime`))
  ;[0 1 0] スライムの状態確認
  (for _array_element _slime
    (`/Engine/EditorBlueprintResources/StandardMacros.IsValid` _array_element
      (:`Is Not Valid`
        (`KismetArrayLibrary.Array_RemoveItem` _slime _array_element)))))

(event `Chack_Cooltime`
  ;[0 1 0] クールタイムの確認
  (if (`self.Spawn_CooleTime_Flg`)
    (`KismetSystemLibrary.Delay` (`self.Spawn_CooleTime`))
    (set `self.Spawn_CooleTime_Flg` false)))

(fn `UserConstructionScript`)