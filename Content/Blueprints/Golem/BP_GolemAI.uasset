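; BP_GolemAI is the golem's AI controller, which runs its behavior tree and blackboard and drives patrol movement.
; While Patrol is set, Tick advances a distance along the pawn's PatrolRoute spline, steering and facing toward that point, looping at the end, and alternating work with short rests.
; The spline is re-pinned to the start location with zero rotation during movement.
; ChangeDirection offers constant-speed turning toward a target and reports completion.
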(event `self.ReceiveBeginPlay`
  (`self.UseBlackboard` "/Game/Blueprints/Golem/AI/BB_Golem.BB_Golem")
  (`self.RunBehaviorTree` "/Game/Blueprints/Golem/AI/BT_Golem.BT_Golem")
  (`self.InitPatrolRoute`))

(event `self.ReceiveTick`
  (params (DeltaSeconds :type "Float (single-precision)"))
  (set `self.DeltaSec` DeltaSeconds)
  (`self.RunPatrol`))

(fn `Change Direction`
  (params (TargetPos :type "Vector Structure") (CustomRotSpeed :type "Float (double-precision)"))
  (returns (ChangeDone :type Boolean) (CurrentDirection :type "Vector Structure") (TargetDirection :type "Vector Structure"))
  (locals (Local_CurrentRot :type "Rotator Structure") (Local_TgtRot :type "Rotator Structure") (RotSpeed :type "Float (double-precision)" :default 100.0))
  (bind _returnvalue (`self.K2_GetPawn`))
  (bind _returnvalue_2 (`KismetMathLibrary.GetForwardVector` (`local.Local_CurrentRot`)))
  (bind _returnvalue_3 (`KismetMathLibrary.GetForwardVector` (`local.Local_TgtRot`)))
  (if (!= CustomRotSpeed 0.0)
    (set `local.RotSpeed` CustomRotSpeed))
  (set `local.Local_CurrentRot` (`self.K2_GetActorRotation` _returnvalue))
  (set `local.Local_TgtRot` (`KismetMathLibrary.FindLookAtRotation` (`/Game/Blueprints/BP_FuncLibrary.Vector to 2D(XY)` (`self.K2_GetActorLocation` _returnvalue)) (`/Game/Blueprints/BP_FuncLibrary.Vector to 2D(XY)` TargetPos)))
  (if (!= (`local.Local_CurrentRot`) (`local.Local_TgtRot`) :`ErrorTolerance` 0.2)
    (`self.K2_SetActorRotation` _returnvalue (`KismetMathLibrary.RInterpTo_Constant` (`local.Local_CurrentRot`) (`local.Local_TgtRot`) (`self.DeltaSec`) (`local.RotSpeed`)) false) ; 向き調整
    (return false _returnvalue_2 _returnvalue_3)
    (else
      (return true _returnvalue_2 _returnvalue_3))))

(fn `InitPatrolRoute`
  (bind _asbp_golem (cast `/Game/Blueprints/Golem/BP_Golem` (`self.K2_GetPawn`)))
  (set `self.PatrolRoute` (`|ConvertAsset` (`/Game/Blueprints/Golem/BP_Golem.PatrolRoute` _asbp_golem)))
  (set `self.PatrolBasePos` (`self.K2_GetActorLocation` (`self.K2_GetPawn`))))

(fn `RunPatrol`
  (bind _returnvalue (`self.K2_GetPawn`))
  (bind _output (`|ConvertAsset` (`self.PatrolRoute`)))
  (bind _returnvalue_2 (- (`SplineComponent.GetLocationAtDistanceAlongSpline` (`|ConvertAsset` (`self.PatrolRoute`)) (`self.CurrentDistance`) "World") (`self.K2_GetActorLocation` _returnvalue)))
  (if (`self.bPatrol`)
    (if (<= (`self.RestTime`) 0.0)
      (set `self.WorkTime` (- (`self.WorkTime`) (`self.DeltaSec`))) ; 仕事時間計測
      (`SceneComponent.K2_SetWorldLocation` _output (`self.PatrolBasePos`) false false) ; スプライン初期位置固定
      (`SceneComponent.K2_SetWorldRotation` :`self` _output) ; スプライン初期回転固定
      (bind _asbp_golem (cast `/Game/Blueprints/Golem/BP_Golem` _returnvalue))
      (set `self.CurrentDistance` (+ (`self.CurrentDistance`) (* (`/Game/Blueprints/Golem/BP_Golem.MoveSpeed` _asbp_golem) (`self.DeltaSec`)))) ; 距離更新
      (`Pawn.AddMovementInput` _returnvalue _returnvalue_2 1.0 false) ; ルート移動
      (`self.K2_SetActorRotation` _returnvalue (`KismetMathLibrary.Conv_VectorToRotator` _returnvalue_2) false) ; 向き更新
      (`|ExecutionSequence`
        (:`then_0`
          (if (>= (`self.CurrentDistance`) (`SplineComponent.GetSplineLength` (`|ConvertAsset` (`self.PatrolRoute`))))
            (set `self.CurrentDistance` 0.0)))
        (:`then_1`
          (if (<= (`self.WorkTime`) 0.0)
            (set `self.WorkTime` 10.0)
            (set `self.RestTime` 2.0))))
      (else
        (set `self.RestTime` (- (`self.RestTime`) (`self.DeltaSec`))) ; 休憩時間観測
      ))))

(fn `UserConstructionScript`)