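; Game mode that sets up the UI, background music and save/load for the game.
; BeginPlay spawns pause, game, fade and lose UI actors, creates a BP_SaveGame object and asynchronously loads its slot, copying TestVal into the BP_GlobalData game instance.
; SaveGame writes that value back asynchronously and quits the game when finished.
; PlayBGM swaps the track on a shared BGM player, stopping any current playback.
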(event `self.ReceiveBeginPlay`
  (`self.InitPauseUI`)
  (`self.InitGameUI`)
  (`self.InitFadeUI`)
  (`self.InitLoseUI`)
  (bind _returnvalue (`GameplayStatics.CreateSaveGameObject` "/Game/Blueprints/System/BP_SaveGame.BP_SaveGame_C"))
  (set `self.SaveGameObject` (`|ConvertAsset` _returnvalue)) ; データ入出力処理初期化
  (`self.LoadGame`) ; データ読込
)

(event `LoadGame`
  ;[1 1 1] セーブ＆ロード
  (bind (_slotname _userindex) (`/Game/Blueprints/System/BP_SaveGame.GetSaveID` (`|ConvertAsset` (`self.SaveGameObject`))))
  (bind (_savegame _bsuccess) (`AsyncActionHandleSaveGame.AsyncLoadGameFromSlot` _slotname _userindex) ; データ読込
    (:`Completed`
      (if _bsuccess
        (bind _asbp_save_game (cast `/Game/Blueprints/System/BP_SaveGame` _savegame))
        (bind _asbp_global_data (cast `/Game/Blueprints/System/BP_GlobalData` (`GameplayStatics.GetGameInstance`)))
        (set `/Game/Blueprints/System/BP_GlobalData.TestVal` (`/Game/Blueprints/System/BP_SaveGame.TestVal` _asbp_save_game) _asbp_global_data) ; 詳細更新
      ))))

(event `SaveGame`
  (bind _output (`|ConvertAsset` (`self.SaveGameObject`)))
  ;[1 1 1] セーブ＆ロード
  (bind _asbp_global_data (cast `/Game/Blueprints/System/BP_GlobalData` (`GameplayStatics.GetGameInstance`)))
  (set `/Game/Blueprints/System/BP_SaveGame.TestVal` (`/Game/Blueprints/System/BP_GlobalData.TestVal` _asbp_global_data) _output) ; 詳細保存
  (bind (_slotname _userindex) (`/Game/Blueprints/System/BP_SaveGame.GetSaveID` _output)) ; データ保存
  (`AsyncActionHandleSaveGame.AsyncSaveGameToSlot` _output _slotname _userindex
    (:`Completed`
      (`KismetSystemLibrary.QuitGame` null "Quit") ; ゲーム終了
    )))

(fn `InitFadeUI`
  (bind _returnvalue (`|SpawnActorFromClass` "/Game/Blueprints/System/BP_UI/BP_Fade.BP_Fade_C" (`KismetMathLibrary.MakeTransform` (0.0 0.0 0.0)) "Undefined" "OverrideRootScale" null null))
  (set `self.Actor_FadeUI` (`|ConvertAsset` _returnvalue)) ; フェードUI用アクタ初期化
)

(fn `InitGameUI`
  (bind _returnvalue (`|SpawnActorFromClass` "/Game/Blueprints/System/BP_UI/BP_GameUI.BP_GameUI_C" (`KismetMathLibrary.MakeTransform` (0.0 0.0 0.0)) "Undefined" "OverrideRootScale" null null))
  (set `self.Actor_GameUI` (`|ConvertAsset` _returnvalue)) ; ゲームUI用アクタ初期化
)

(fn `InitLoseUI`
  (bind _returnvalue (`|SpawnActorFromClass` "/Game/Blueprints/System/BP_UI/BP_LoseUI.BP_LoseUI_C" (`KismetMathLibrary.MakeTransform` (0.0 0.0 0.0)) "Undefined" "OverrideRootScale" null null))
  (set `self.Actor_LoseUI` (`|ConvertAsset` _returnvalue)) ; 敗北演出UI用アクタ初期化
)

(fn `InitPauseUI`
  (bind _returnvalue (`|SpawnActorFromClass` "/Game/Blueprints/System/BP_UI/BP_PauseUI.BP_PauseUI_C" (`KismetMathLibrary.MakeTransform` (0.0 0.0 0.0)) "Undefined" "OverrideRootScale" null null))
  (set `self.Actor_PauseUI` (`|ConvertAsset` _returnvalue)) ; ポーズUI用アクタ初期化
)

(fn `PlayBGM`
  (params (BGM_Cue :type "SoundCue Object Reference"))
  (returns (BGM_Player :type "AudioComponent Object Reference"))
  (bind _bgm_player (`self.BGM_Player`))
  (if (`AudioComponent.IsPlaying` _bgm_player)
    (`AudioComponent.Stop` _bgm_player) ; BGM停止
  )
  (`AudioComponent.SetSound` _bgm_player BGM_Cue) ; BGM変更
  (`AudioComponent.Play` _bgm_player 0.0) ; BGM開始
  (return _bgm_player))

(fn `UserConstructionScript`)