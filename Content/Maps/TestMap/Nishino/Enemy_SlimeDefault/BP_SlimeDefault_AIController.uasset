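; AI controller for the default slime enemy, deciding whether it chases or flees from the player.
; It runs the slime behavior tree and uses AI perception to set a found flag and state enum on the blackboard.
; While the player is detected, Tick rechecks slime size: larger slimes chase, smaller ones flee and get a test blue material.
; Losing sight sets a lost-player state unless the slime was fleeing.
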(event `self.ReceiveBeginPlay`
  ;[0.5 1 1] ブラックボードの使用とビヘイビアツリーの実行
  (bind _blackboardcomponent (`self.UseBlackboard` "/Game/Maps/TestMap/Nishino/Enemy_SlimeDefault/BB_SlimeDefault.BB_SlimeDefault")) ; ブラックボード呼び出し
  (set `self.Blackboard_Component` _blackboardcomponent) ; ブラックボードの情報保存
  (`self.RunBehaviorTree` "/Game/Maps/TestMap/Nishino/Enemy_SlimeDefault/BT_SlimeDefault.BT_SlimeDefault") ; ビヘイビアツリーの実行
)

(event `self.ReceiveTick`
  (params (DeltaSeconds :type "Float (single-precision)"))
  (`self.CastSlimePawn`)
  (if (`BlackboardComponent.GetValueAsBool` (`self.Blackboard_Component`) "FindFlg")
    (`self.ChackSizeANDState`)))

(event `self.AIPerception.OnPerceptionUpdated`
  (params (UpdatedActors :type "Array of Actor Object Reference (by ref)"))
  ;[1 0.5 0.5] プレイヤーを見つけた＆見逃した時の処理
  (for _array_element UpdatedActors
    (bind _info (`AIPerceptionComponent.GetActorsPerception` (`self.AIPerception`) _array_element)) ; 受けた刺激情報を取得
    (bind (_target _lastsensedstimuli) (break `ActorPerceptionBlueprintInfo` _info))
    (if (== (`GameplayStatics.GetPlayerPawn` 0) _target)
      (`self.StateSet` (`.bSuccessfullySensed` (break `AIStimulus` (`|GetArrayItem` _lastsensedstimuli)))) ; 状態を設定する
    )))

(fn `CastSlimePawn`
  (`/Engine/EditorBlueprintResources/StandardMacros.DoOnce` false :!label _label
    (:`Completed`
      (bind _asbp_slime_default (cast `/Game/Maps/TestMap/Nishino/Enemy_SlimeDefault/BP_SlimeDefault` (`self.K2_GetPawn`))
        (:`then`
          (set `self.SlimePawn` _asbp_slime_default))
        (:`CastFailed`
          (goto _label :!via `Reset`))))))

(fn `ChackSizeANDState`
  (bind _slimepawn (`self.SlimePawn`))
  (if (> (`/Game/Maps/TestMap/Nishino/Enemy_SlimeDefault/BP_SlimeDefault.SlimeSize` _slimepawn) 4)
    (`BlackboardComponent.SetValueAsEnum` (`self.Blackboard_Component`) "SlimeState" (enumliteral `/Game/Maps/TestMap/Nishino/Enemy_SlimeDefault/ENUM_SlimeDefault_SlimeState` "NewEnumerator10")) ; プレイヤーを追いかける！
    (else
      (`PrimitiveComponent.SetMaterial` (`Character.Mesh` _slimepawn) 0 "/AnimationSharing/AnimSharingBlue.AnimSharingBlue") ; ﾃｽﾄ
      (`BlackboardComponent.SetValueAsEnum` (`self.Blackboard_Component`) "SlimeState" (enumliteral `/Game/Maps/TestMap/Nishino/Enemy_SlimeDefault/ENUM_SlimeDefault_SlimeState` "NewEnumerator11")) ; プレイヤーから逃げ出す
    )))

(fn `StateSet`
  (params (Find :type Boolean))
  (bind _blackboard_component (`self.Blackboard_Component`))
  (if Find
    (`KismetSystemLibrary.PrintString` "FIND")
    ;[1 0.5 0.5] プレイヤーを見つけた時
    (`BlackboardComponent.SetValueAsBool` (`self.Blackboard_Component`) "FindFlg" true) ; フラグの設定
    (`self.ChackSizeANDState`) ; 状態の設定
    (else
      (`KismetSystemLibrary.PrintString` "MISS")
      ;[0.5 0.5 1] プレイヤーを見逃した時
      (`BlackboardComponent.SetValueAsBool` _blackboard_component "FindFlg" false) ; フラグの設定
      (if (!= (`BlackboardComponent.GetValueAsEnum` _blackboard_component "SlimeState") (enumliteral `/Game/Maps/TestMap/Nishino/Enemy_SlimeDefault/ENUM_SlimeDefault_SlimeState` "NewEnumerator11"))
        (`BlackboardComponent.SetValueAsEnum` (`self.Blackboard_Component`) "SlimeState" (enumliteral `/Game/Maps/TestMap/Nishino/Enemy_SlimeDefault/ENUM_SlimeDefault_SlimeState` "NewEnumerator9")) ; プレイヤーを見逃した
      ))))

(fn `UserConstructionScript`)