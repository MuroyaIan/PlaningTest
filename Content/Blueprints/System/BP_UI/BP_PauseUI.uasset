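; Pause menu controller Blueprint that opens and closes the pause screen, pauses the game and hosts an options submenu.
; It creates both widgets at BeginPlay, applies saved BGM and SE volumes from BP_GlobalData, and routes input actions to the active menu with sound effects.
; Tick countdowns matching the hide animations delay widget removal, unpausing and returning from options, while a short cooldown blocks immediate reopening.
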(event `self.ReceiveBeginPlay`
  (bind _asbp_player_controller (cast `/Game/Blueprints/Player/BP_PlayerController` (`GameplayStatics.GetPlayerController` 0)))
  (`self.EnableInput` _asbp_player_controller) ; 入力有効化
  (bind _returnvalue (`|CreateWidget` "/Game/Maps/TestMap/Kitayama/UI_Kitayama/Widget_UI/PauseWidget/UMG_PauseMenuMaster.UMG_PauseMenuMaster_C"))
  (set `self.Widget_PauseUI` _returnvalue)
  (bind _returnvalue_2 (`|CreateWidget` "/Game/Maps/TestMap/Kitayama/UI_Kitayama/Widget_UI/PauseWidget/UMG_OptionMaster.UMG_OptionMaster_C"))
  (set `self.Widget_OptionUI` _returnvalue_2)
  (`self.InitSound`)
  (set `self.UnDispTimer` (`WidgetAnimation.GetEndTime` (`/Game/Maps/TestMap/Kitayama/UI_Kitayama/Widget_UI/PauseWidget/UMG_PauseMenuMaster.UnDisp` (`self.Widget_PauseUI`))))
  (set `self.OpUndispTimer` (`WidgetAnimation.GetEndTime` (`/Game/Maps/TestMap/Kitayama/UI_Kitayama/Widget_UI/PauseWidget/UMG_OptionMaster.UnDisp` (`self.Widget_OptionUI`)))))

(event `self.ReceiveTick`
  (params (DeltaSeconds :type "Float (single-precision)"))
  (bind _widget_pauseui (`self.Widget_PauseUI`))
  (`|ExecutionSequence`
    (:`then_0`
      (if (`self.DispOffTrigger`)
        (bind _output_get (set `self.TriggerTimer` (+ DeltaSeconds (`self.TriggerTimer`))))
        (if (> _output_get 0.2)
          (set `self.DispOffTrigger` false)
          (set `self.TriggerTimer` 0.0))))
    (:`then_1`
      (if (`self.UnDispTimerFlg`)
        (bind _output_get_2 (set `self.UnDispTimer` (- (`self.UnDispTimer`) DeltaSeconds)))
        (if (<= _output_get_2 0.0)
          (`Widget.RemoveFromParent` (`self.Widget_PauseUI`))
          (set `self.UnDispTimerFlg` false)
          (set `self.UnDispTimer` (`WidgetAnimation.GetEndTime` (`/Game/Maps/TestMap/Kitayama/UI_Kitayama/Widget_UI/PauseWidget/UMG_PauseMenuMaster.UnDisp` (`self.Widget_PauseUI`))))
          (bind _output_get_3 (set `self.isDispUI` false)) ; 入力制御更新
          (`GameplayStatics.SetGamePaused` _output_get_3) ; ポーズ処理
        )))
    (:`then_2`
      (if (`self.OpUnDispTimerFlg`)
        (bind _output_get_4 (set `self.OpUndispTimer` (- (`self.OpUndispTimer`) DeltaSeconds)))
        (if (<= _output_get_4 0.0)
          (`Widget.RemoveFromParent` (`self.Widget_OptionUI`))
          (`UserWidget.AddToViewport` _widget_pauseui 0)
          (`/Game/Maps/TestMap/Kitayama/UI_Kitayama/Widget_UI/PauseWidget/UMG_PauseMenuMaster.DispAnim` _widget_pauseui)
          (set `self.IsOption` false)
          (set `self.OpUndispTimer` (`WidgetAnimation.GetEndTime` (`/Game/Maps/TestMap/Kitayama/UI_Kitayama/Widget_UI/PauseWidget/UMG_OptionMaster.UnDisp` (`self.Widget_OptionUI`))))
          (set `self.OpUnDispTimerFlg` false))))))

(event `InputAction|PauseUI_Disp` :consume false :paused true
  (params (Key :type "Key Structure"))
  (bind _isdispui (`self.isDispUI`))
  (bind _widget_pauseui (`self.Widget_PauseUI`))
  (:`Pressed`
    (if (not (`self.DispOffTrigger`))
      (bind _isplay (`/Game/Maps/TestMap/Kitayama/UI_Kitayama/Widget_UI/PauseWidget/UMG_PauseMenuMaster.Get Disp AnimTime` (`self.Widget_PauseUI`)))
      (if (or _isplay (`self.UnDispTimerFlg`))
        _
        (elif (not _isdispui)
          (`GameplayStatics.PlaySound2D` "/Game/Resource/SO/SE/UI/Pause/SO_SE_Pause_Start_Cue.SO_SE_Pause_Start_Cue" 1.0 1.0 0.0 null null) ; 効果音再生
          (`UserWidget.AddToViewport` _widget_pauseui 0) ; UIを表示
          (`/Game/Maps/TestMap/Kitayama/UI_Kitayama/Widget_UI/PauseWidget/UMG_PauseMenuMaster.DispAnim` _widget_pauseui)
          (bind _output_get (set `self.isDispUI` (not _isdispui))) ; 入力制御更新
          (`GameplayStatics.SetGamePaused` _output_get) ; ポーズ処理
        )))))

(event `InputAction|UI_Confirm` :consume false :paused true
  (params (Key :type "Key Structure"))
  (bind _widget_optionui (`self.Widget_OptionUI`))
  (:`Pressed`
    (if (`self.isDispUI`)
      (if (!= (`/Game/Maps/TestMap/Kitayama/UI_Kitayama/Widget_UI/PauseWidget/UMG_PauseMenuMaster.SelectNum` (`self.Widget_PauseUI`)) 3)
        (`/Game/Maps/TestMap/Kitayama/UI_Kitayama/Widget_UI/PauseWidget/UMG_PauseMenuMaster.DecideMenu` (`self.Widget_PauseUI`))
        (`GameplayStatics.PlaySound2D` "/Game/Resource/SO/SE/UI/SO_SE_UI_Confirm_Cue.SO_SE_UI_Confirm_Cue" 1.0 1.0 0.0 null null :!label _label) ; 効果音再生
        (elif (not (`self.IsOption`))
          (`Widget.RemoveFromParent` (`self.Widget_PauseUI`))
          (`UserWidget.AddToViewport` _widget_optionui 0)
          (`/Game/Maps/TestMap/Kitayama/UI_Kitayama/Widget_UI/PauseWidget/UMG_OptionMaster.DispAnim` _widget_optionui)
          (set `self.IsOption` true)
          (goto _label))))))

(event `InputAction|UI_Back` :consume false :paused true
  (params (Key :type "Key Structure"))
  (:`Pressed`
    (if (`self.isDispUI`)
      (`GameplayStatics.PlaySound2D` "/Game/Resource/SO/SE/UI/SO_SE_UI_Back_Cue.SO_SE_UI_Back_Cue" 1.0 1.0 0.0 null null) ; 効果音再生
      (if (`self.IsOption`)
        (`/Game/Maps/TestMap/Kitayama/UI_Kitayama/Widget_UI/PauseWidget/UMG_OptionMaster.UnDispAnim` (`self.Widget_OptionUI`))
        (set `self.OpUnDispTimerFlg` true)
        (else
          (bind _isplay (`/Game/Maps/TestMap/Kitayama/UI_Kitayama/Widget_UI/PauseWidget/UMG_PauseMenuMaster.Get Disp AnimTime` (`self.Widget_PauseUI`)))
          (if (not (or _isplay (`self.UnDispTimerFlg`)))
            (`self.DispOff`)
            (set `self.DispOffTrigger` true)))))))

(event `InputAction|UI_Up` :consume false :paused true
  (params (Key :type "Key Structure"))
  (:`Pressed`
    (if (`self.isDispUI`)
      (if (`self.IsOption`)
        (`/Game/Maps/TestMap/Kitayama/UI_Kitayama/Widget_UI/PauseWidget/UMG_OptionMaster.SelectOption` (`self.Widget_OptionUI`) false)
        (else
          (`/Game/Maps/TestMap/Kitayama/UI_Kitayama/Widget_UI/PauseWidget/UMG_PauseMenuMaster.SelectMenu` (`self.Widget_PauseUI`) false))))))

(event `InputAction|UI_Down` :consume false :paused true
  (params (Key :type "Key Structure"))
  (:`Pressed`
    (if (`self.isDispUI`)
      (if (`self.IsOption`)
        (`/Game/Maps/TestMap/Kitayama/UI_Kitayama/Widget_UI/PauseWidget/UMG_OptionMaster.SelectOption` (`self.Widget_OptionUI`) true)
        (else
          (`/Game/Maps/TestMap/Kitayama/UI_Kitayama/Widget_UI/PauseWidget/UMG_PauseMenuMaster.SelectMenu` (`self.Widget_PauseUI`) true))))))

(event `InputAction|UI_Right` :consume false :paused true
  (params (Key :type "Key Structure"))
  (:`Pressed`
    (if (`self.isDispUI`)
      (if (`self.IsOption`)
        (`GameplayStatics.PlaySound2D` "/Game/Resource/SO/SE/UI/SO_SE_UI_Select_Cue.SO_SE_UI_Select_Cue" 1.0 1.0 0.0 null null) ; 効果音再生
        (`/Game/Maps/TestMap/Kitayama/UI_Kitayama/Widget_UI/PauseWidget/UMG_OptionMaster.SetVal` (`self.Widget_OptionUI`) 1)))))

(event `InputAction|UI_Left` :consume false :paused true
  (params (Key :type "Key Structure"))
  (:`Pressed`
    (if (`self.isDispUI`)
      (if (`self.IsOption`)
        (`GameplayStatics.PlaySound2D` "/Game/Resource/SO/SE/UI/SO_SE_UI_Select_Cue.SO_SE_UI_Select_Cue" 1.0 1.0 0.0 null null) ; 効果音再生
        (`/Game/Maps/TestMap/Kitayama/UI_Kitayama/Widget_UI/PauseWidget/UMG_OptionMaster.SetVal` (`self.Widget_OptionUI`) -1)))))

(event `InputAction|UI_Confirm` :consume false :paused true
  (params (Key :type "Key Structure"))
  (bind _widget_optionui (`self.Widget_OptionUI`))
  (:`Pressed`
    (if (`self.isDispUI`)
      (if (`self.IsOption`)
        (if (== (`/Game/Maps/TestMap/Kitayama/UI_Kitayama/Widget_UI/PauseWidget/UMG_OptionMaster.SelectNum` _widget_optionui) 4)
          (`/Game/Maps/TestMap/Kitayama/UI_Kitayama/Widget_UI/PauseWidget/UMG_OptionMaster.SetVib` _widget_optionui)
          (`GameplayStatics.PlaySound2D` "/Game/Resource/SO/SE/UI/SO_SE_UI_Confirm_Cue.SO_SE_UI_Confirm_Cue" 1.0 1.0 0.0 null null) ; 効果音再生
        )))))

(fn `DispOff`
  (`/Game/Maps/TestMap/Kitayama/UI_Kitayama/Widget_UI/PauseWidget/UMG_PauseMenuMaster.UnDispAnim` (`self.Widget_PauseUI`))
  (set `self.UnDispTimerFlg` true))

(fn `InitSound`
  (bind _asbp_global_data (cast `/Game/Blueprints/System/BP_GlobalData` (`GameplayStatics.GetGameInstance`)))
  (`|ExecutionSequence`
    (:`then_0`
      (`GameplayStatics.SetSoundMixClassOverride` "/Game/Blueprints/Sound/SO_SoundMix.SO_SoundMix" "/Game/Blueprints/Sound/SO_BGM.SO_BGM" (/ (`KismetMathLibrary.Conv_IntToDouble` (`/Game/Blueprints/System/BP_GlobalData.Volume_BGM` _asbp_global_data)) 10.0) 1.0 0.0) ; 音量情報の上書き
      (`GameplayStatics.PushSoundMixModifier` "/Game/Blueprints/Sound/SO_SoundMix.SO_SoundMix") ; 音量情報の更新
    )
    (:`then_1`
      (`GameplayStatics.SetSoundMixClassOverride` "/Game/Blueprints/Sound/SO_SoundMix.SO_SoundMix" "/Game/Blueprints/Sound/SO_SE.SO_SE" (/ (`KismetMathLibrary.Conv_IntToDouble` (`/Game/Blueprints/System/BP_GlobalData.Volume_SE` _asbp_global_data)) 10.0) 1.0 0.0) ; 音量情報の上書き
      (`GameplayStatics.PushSoundMixModifier` "/Game/Blueprints/Sound/SO_SoundMix.SO_SoundMix") ; 音量情報の更新
    )))

(fn `UserConstructionScript`)