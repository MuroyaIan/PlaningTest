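; Debug UI actor that toggles a camera debug widget and drives its sliders from the keyboard.
; On BeginPlay it enables input from the player controller, then C adds the widget to or removes it from the viewport.
; Left/Right call the widget's slider value function and Up/Down its slider color function.
; Boolean latches, cleared on key release, limit input to one action per press.
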(event `self.ReceiveBeginPlay`
  (bind _asbp_player_controller (cast `/Game/Blueprints/Player/BP_PlayerController` (`GameplayStatics.GetPlayerController` 0)))
  (`self.EnableInput` _asbp_player_controller) ; 入力有効化
)

(event `Key|C` :consume false
  (params (Key :type "Key Structure"))
  (bind _widget_debugui (`self.GetWidget`))
  (:`Pressed`
    (if (not (`self.DispUITrigger`))
      (bind _returnisdisp (`self.DispWidget` _widget_debugui (`/Game/Maps/TestMap/Kitayama/UI/Widget_CameraUI.IsDisp` _widget_debugui))) ; カメラUIの表示非常時を切り替え
      (set `/Game/Maps/TestMap/Kitayama/UI/Widget_CameraUI.IsDisp` _returnisdisp _widget_debugui)
      (set `self.DispUITrigger` true)))
  (:`Released`
    (set `self.DispUITrigger` false) ; トリガー処理（入力可能状態に遷移）
  ))

(event `Key|Right` :consume false
  (params (Key :type "Key Structure"))
  (:`Pressed`
    (if (not (`self.InputTrigger`))
      (`/Game/Maps/TestMap/Kitayama/UI/Widget_CameraUI.SetSlinderValue` (`self.GetWidget`) 1)
      (set `self.InputTrigger` true)))
  (:`Released`
    (set `self.InputTrigger` false)))

(event `Key|Left` :consume false
  (params (Key :type "Key Structure"))
  (:`Pressed`
    (if (not (`self.InputTrigger`))
      (`/Game/Maps/TestMap/Kitayama/UI/Widget_CameraUI.SetSlinderValue` (`self.GetWidget`) -1)
      (set `self.InputTrigger` true)))
  (:`Released`
    (set `self.InputTrigger` false)))

(event `Key|Down` :consume false
  (params (Key :type "Key Structure"))
  (:`Pressed`
    (if (not (`self.InputTrigger`))
      (`/Game/Maps/TestMap/Kitayama/UI/Widget_CameraUI.Set Slinder Color` (`self.GetWidget`) 1)
      (set `self.InputTrigger` true)))
  (:`Released`
    (set `self.InputTrigger` false)))

(event `Key|Up` :consume false
  (params (Key :type "Key Structure"))
  (:`Pressed`
    (if (not (`self.InputTrigger`))
      (`/Game/Maps/TestMap/Kitayama/UI/Widget_CameraUI.Set Slinder Color` (`self.GetWidget`) 0)
      (set `self.InputTrigger` true)))
  (:`Released`
    (set `self.InputTrigger` false)))

(fn `DispWidget`
  (params (Widget :type "UserWidget Object Reference") (IsDisp :type Boolean))
  (returns (ReturnIsDisp :type Boolean))
  (if IsDisp
    (`Widget.RemoveFromParent` Widget) ; UIの非表示にする
    (else
      (`UserWidget.AddToViewport` Widget 0) ; UIを表示する
    ))
  (return (not IsDisp)))

(fn `GetWidget`
  (returns (Widget_DebugUI :type "/Game/Maps/TestMap/Kitayama/UI/Widget_CameraUI Object Reference"))
  (return (`|ConvertAsset` (`self.Widget_DebugUI`))))

(fn `UserConstructionScript`)