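; Cutscene camera actor for the player weapon's boss-suction sequence.
; Tick watches the weapon's SuckBoss flag and, once per activation, places the camera 200 units behind the player camera manager's view with matching rotation.
; It blends the view to itself until BossSucked is set, then a DoOnce triggers a delayed ease-out blend back to the player pawn.
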(event `self.ReceiveBeginPlay`)

(event `self.ReceiveTick`
  (params (DeltaSeconds :type "Float (single-precision)"))
  (bind _returnvalue (`GameplayStatics.GetPlayerController` 0))
  (set `self.DeltaSec` DeltaSeconds)
  (bind _asbp_player (cast `/Game/Blueprints/Player/BP_Player` (`GameplayStatics.GetPlayerPawn` 0)))
  (if (`/Game/Blueprints/Weapon/BP_Weapon.bSuckBoss` (`/Game/Blueprints/Player/BP_Player.GetWeapon` _asbp_player))
    (`|ExecutionSequence`
      (:`then_0`
        (`/Engine/EditorBlueprintResources/StandardMacros.DoOnce` false :!label _label
          (:`Completed`
            (bind _asbp_player_camera_manager (cast `/Game/Blueprints/Player/BP_PlayerCameraManager` (`GameplayStatics.GetPlayerCameraManager` 0)))
            (`self.K2_SetActorLocation` (+ (`PlayerCameraManager.GetCameraLocation` _asbp_player_camera_manager) (* (`/Game/Blueprints/Player/BP_PlayerCameraManager.GetForwardVector` _asbp_player_camera_manager) -200.0))) ; 位置更新
            (bind _rotation (`/Game/Blueprints/Player/BP_PlayerCameraManager.GetCameraRotationEx` _asbp_player_camera_manager true true true))
            (`self.K2_SetActorRotation` _rotation) ; 回転更新
            (goto _label_2 :!via `Reset`))))
      (:`then_1`
        (if (not (`/Game/Blueprints/Player/BP_Player.bBossSucked` _asbp_player))
          (`PlayerController.SetViewTargetWithBlend` _returnvalue self 1.0 "VTBlend_EaseIn" 0.5 false) ; 演出カメラ切替
          (else
            (`/Engine/EditorBlueprintResources/StandardMacros.DoOnce` false :!label _label_2
              (:`Completed`
                (`KismetSystemLibrary.Delay` 3.0) ; 演出待ち時間
                (`PlayerController.SetViewTargetWithBlend` _returnvalue (`GameplayStatics.GetPlayerPawn` 0) 1.0 "VTBlend_EaseOut" 0.5 false) ; メインカメラ切替
              ))))))
    (else
      (goto _label :!via `Reset`))))

(fn `UserConstructionScript`)