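; BP_Camera_StageStart is a stage-start camera that sweeps around the player along a spline.
; The construction script shapes the spline as a half-circle arc with points from CalcSplinePoint, using StartRadius and interpolating height from StartHeight to EndHeight.
; Tick advances distance by MoveSpeed, offsets the spline's local position by the player pawn's location, and rotates the camera to face the player.
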(event `self.ReceiveTick`
  (params (DeltaSeconds :type "Float (single-precision)"))
  (bind _cameracomponent (`self.CameraComponent`))
  (bind _output_get (set `self.CurrentDistance` (+ (* DeltaSeconds (`self.MoveSpeed`)) (`self.CurrentDistance`))))
  (`SceneComponent.K2_SetWorldLocation` _cameracomponent (+ (`SplineComponent.GetLocationAtDistanceAlongSpline` (`self.Spline_StageStart`) _output_get "Local") (`self.K2_GetActorLocation` (`GameplayStatics.GetPlayerPawn` 0))) true false)
  (`SceneComponent.K2_SetWorldRotation` _cameracomponent (`KismetMathLibrary.FindLookAtRotation` (`SceneComponent.K2_GetComponentLocation` _cameracomponent) (`self.K2_GetActorLocation` (`GameplayStatics.GetPlayerPawn` 0))) true false))

(fn `Calc Spline Point`
  (params (alpha :type "Float (double-precision)"))
  (returns (ReturnValue :type "Vector Structure"))
  (bind _returnvalue (* alpha 180.0))
  (bind _startradius (`self.StartRadius`))
  (return (`KismetMathLibrary.MakeVector` (* (`KismetMathLibrary.DegCos` _returnvalue) _startradius) (* _startradius (`KismetMathLibrary.DegSin` _returnvalue)) (`KismetMathLibrary.Lerp` (`self.StartHeight`) (`self.EndHeight`) alpha))))

(fn `UserConstructionScript`
  (bind _spline_stagestart (`self.Spline_StageStart`))
  (`SplineComponent.SetLocationAtSplinePoint` _spline_stagestart 0 (`self.Calc Spline Point` 0.0) "Local" true)
  (`SplineComponent.SetRotationAtSplinePoint` _spline_stagestart 0 (`KismetMathLibrary.MakeRotator` 0.0 0.0 90.0) "Local" true)
  (`SplineComponent.AddSplinePoint` _spline_stagestart (`self.Calc Spline Point` 0.5) "Local" true)
  (`SplineComponent.AddSplinePoint` _spline_stagestart (`self.Calc Spline Point` 1.0) "Local" true))