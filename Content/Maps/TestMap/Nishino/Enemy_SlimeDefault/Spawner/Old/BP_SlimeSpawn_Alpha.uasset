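; BP_SlimeSpawn_Alpha is a slime spawner that keeps an array of BP_SlimeDefault enemies populated.
; Every Tick it loops up to MaxSpawn, refilling any invalid SpawnSlime slot through Spawn.
; Spawn creates the slime and its default controller, then passes in the spawner's stats and a random size, printing a debug string on failure.
; The random-location math in Make_SpawnTransform is left unconnected.
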(event `self.ReceiveTick`
  (params (DeltaSeconds :type "Float (single-precision)"))
  (bind _spawnslime (`self.SpawnSlime`))
  (for _index (range (+ (`self.MaxSpawn`) 1))
    (if (not (`KismetSystemLibrary.IsValid` (`|GetArrayItem` _spawnslime _index)))
      (bind _return (`self.Spawn`)) ; スライムの生成
      (`KismetArrayLibrary.Array_Set` _spawnslime _index _return true) ; 情報保存
    )))

(fn `Spawn`
  (returns (Return :type "/Game/Maps/TestMap/Nishino/Enemy_SlimeDefault/BP_SlimeDefault Object Reference"))
  ;[1 0.5 1] BP_SlimeDedaultを作成する
  (bind _returnvalue (`|SpawnActorFromClass` "/Game/Maps/TestMap/Nishino/Enemy_SlimeDefault/BP_SlimeDefault.BP_SlimeDefault_C" (`self.Make_SpawnTransform`) "Undefined" "OverrideRootScale" null null))
  (if (`KismetSystemLibrary.IsValid` _returnvalue)
    (`Pawn.SpawnDefaultController` _returnvalue)
    ;[0.5 1 1] ステータスを設定する
    (`/Game/Maps/TestMap/Nishino/Enemy_SlimeDefault/BP_SlimeDefault.SetStatus` _returnvalue (`self.Hitpoint`) (`self.Damage`) (`self.SpawnTime`) (`KismetMathLibrary.RandomIntegerInRange` 3 5) (`self.Speed`) 3000.0)
    (return _returnvalue)
    (else
      (`KismetSystemLibrary.PrintString` "Spawn_Note!!!!!!!!!!!!") ; なんかうまく作成できていなかったことがあった、たまたま同じ座標とかでスポーンすると作成できないかも
      (return null))))

(fn `UserConstructionScript`)