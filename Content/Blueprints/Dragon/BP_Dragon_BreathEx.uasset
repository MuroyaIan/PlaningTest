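; BP_Dragon_BreathEx is a dragon breath attack variant that turns into a meteor crystal on striking terrain.
; It sets damage and knockback power before running the parent's BeginPlay.
; The first capsule hit on an actor named "Landscape" spawns a Niagara impact effect, then after a short delay hides the breath, spawns BP_Dragon_MeteorCrystal in its place and schedules its own destruction.
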(event `self.ReceiveBeginPlay`
  (set `self.Damage` 4.0)
  (set `self.KnockBackPow` 3000.0)
  (`parent.ReceiveBeginPlay`))

(event `self.CapsuleCollision.OnComponentHit`
  (params (HitComponent :type "PrimitiveComponent Object Reference") (OtherActor :type "Actor Object Reference") (OtherComp :type "PrimitiveComponent Object Reference") (NormalImpulse :type "Vector Structure") (Hit :type "HitResult Structure (by ref)"))
  (if (`KismetStringLibrary.EqualEqual_StrStr` (`KismetSystemLibrary.GetDisplayName` OtherActor) "Landscape")
    (`/Engine/EditorBlueprintResources/StandardMacros.DoOnce` false
      (:`Completed`
        (`NiagaraFunctionLibrary.SpawnSystemAtLocation` "/Game/Resource/FX/VFX/Dragon/FX_VFX_StrongBrethHit_Gr.FX_VFX_StrongBrethHit_Gr" (- (`self.K2_GetActorLocation`) (0.0 0.0 30.0)) (`KismetMathLibrary.MakeRotator` 0.0 0.0 (- (.yaw (`self.K2_GetActorRotation`)) 90.0)) (1.0 1.0 1.0) true true "AutoRelease")
        (`KismetSystemLibrary.Delay` 0.7)
        (`self.SetActorHiddenInGame` true)
        (`|SpawnActorFromClass` "/Game/Blueprints/Dragon/BP_Dragon_MeteorCrystal.BP_Dragon_MeteorCrystal_C" (`KismetMathLibrary.MakeTransform` (`self.K2_GetActorLocation`)) "Undefined" "OverrideRootScale" null null)
        (`self.SetLifeSpan` 1.0)))))

(fn `UserConstructionScript`
  (`parent.UserConstructionScript`))