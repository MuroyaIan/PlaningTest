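; AI controller for the Slime King enemy that starts its blackboard and behavior tree on BeginPlay.
; While the PatrolFlag key is false, Tick moves the pawn along its PatrolRoute spline in a loop, alternating timed walking and rest.
; During movement, the spline is re-pinned each tick to the starting location with zero rotation.
; Tick also mirrors the pawn's active attack states (jump, spin, left/right bash and thrust) into blackboard flags.
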(event `self.ReceiveBeginPlay`
  ;[1 0 0] Begin
  (bind _blackboardcomponent (`self.UseBlackboard` "/Game/Maps/TestMap/Nishino/Enemy_SlimeKing/AI/BB_SlimeKing.BB_SlimeKing")) ; ブラックボードの使用
  (set `self.Blackboard Component` _blackboardcomponent) ; 情報の保存
  (`self.RunBehaviorTree` "/Game/Maps/TestMap/Nishino/Enemy_SlimeKing/AI/BT_Slimeking.BT_SlimeKing") ; ビヘイビアツリー実行
  (bind _asbp_slime_king (cast `/Game/Maps/TestMap/Nishino/Enemy_SlimeKing/BP_SlimeKing` (`self.K2_GetPawn`))) ; 操作しているアクタの保存
  (set `self.SlimeKing` _asbp_slime_king)
  (`self.Init Patrol Route`) ; パトロールルート初期化
)

(event `self.ReceiveTick`
  (params (DeltaSeconds :type "Float (single-precision)"))
  (bind _blackboard_component (`self.Blackboard Component`))
  (set `self.DeltaSec` DeltaSeconds)
  (`self.RunPatrol`)
  (`|ExecutionSequence`
    (:`then_0`
      (bind (_jumpattack _spinattack _bashattack_left _bashattack_right _thrustattack_left _thrustattack_right) (`/Game/Maps/TestMap/Nishino/Enemy_SlimeKing/BP_SlimeKing.Get_ActiveActionStates` (`self.SlimeKing`))) ; 情報の獲得
      (`BlackboardComponent.SetValueAsBool` _blackboard_component "Active_JumpAttackFlg" _jumpattack) ; ジャンプ攻撃情報設定
      (`BlackboardComponent.SetValueAsBool` _blackboard_component "Active_SpinAttackFlg" _spinattack) ; 回転攻撃情報設定
      (`BlackboardComponent.SetValueAsBool` _blackboard_component "Active_BashAttack_LeftFlg" _bashattack_left) ; 叩きつけ(左)攻撃情報設定
      (`BlackboardComponent.SetValueAsBool` _blackboard_component "Active_BashAttack_RightFlg" _bashattack_right) ; 叩きつけ(右)攻撃情報設定
      (`BlackboardComponent.SetValueAsBool` _blackboard_component "Active_ThrustAttack_LeftFlg" _thrustattack_left) ; 突っつき(左)攻撃情報設定
      (`BlackboardComponent.SetValueAsBool` _blackboard_component "Active_ThrustAttack_RightFlg" _thrustattack_right) ; 突っつき(右)攻撃情報設定
    )))

(fn `Init Patrol Route`
  (bind _asbp_slime_king (cast `/Game/Maps/TestMap/Nishino/Enemy_SlimeKing/BP_SlimeKing` (`self.K2_GetPawn`)))
  (set `self.PatrolRoute` (`|ConvertAsset` (`/Game/Maps/TestMap/Nishino/Enemy_SlimeKing/BP_SlimeKing.PatrolRoute` _asbp_slime_king)))
  (set `self.PatrolBasePos` (`self.K2_GetActorLocation` (`self.K2_GetPawn`))))

(fn `RunPatrol`
  (bind _returnvalue (`self.K2_GetPawn`))
  (bind _output (`|ConvertAsset` (`self.PatrolRoute`)))
  (bind _returnvalue_2 (- (`SplineComponent.GetLocationAtDistanceAlongSpline` (`|ConvertAsset` (`self.PatrolRoute`)) (`self.CurrentDistance`) "World") (`self.K2_GetActorLocation` _returnvalue)))
  (bind (_returnvalue_roll _returnvalue_pitch _returnvalue_yaw) (`KismetMathLibrary.BreakRotator` (`KismetMathLibrary.Conv_VectorToRotator` _returnvalue_2)))
  (if (not (`BlackboardComponent.GetValueAsBool` (`self.Blackboard Component`) "PatrolFlag"))
    (if (<= (`self.RestTime`) 0.0)
      (set `self.WorkTime` (- (`self.WorkTime`) (`self.DeltaSec`))) ; 仕事時間計測
      (`SceneComponent.K2_SetWorldLocation` _output (`self.PatrolBasePos`) false false) ; スプライン初期位置固定
      (`SceneComponent.K2_SetWorldRotation` :`self` _output) ; スプライン初期回転固定
      (set `self.CurrentDistance` (+ (`self.CurrentDistance`) (* 800.0 (`self.DeltaSec`)))) ; 距離更新
      (`Pawn.AddMovementInput` _returnvalue _returnvalue_2 1.0 false) ; ルート移動
      (`self.K2_SetActorRotation` _returnvalue (`KismetMathLibrary.MakeRotator` _returnvalue_roll 0.0 _returnvalue_yaw) false) ; 向き更新
      (`|ExecutionSequence`
        (:`then_0`
          (if (>= (`self.CurrentDistance`) (`SplineComponent.GetSplineLength` (`|ConvertAsset` (`self.PatrolRoute`))))
            (set `self.CurrentDistance` 0.0)))
        (:`then_1`
          (if (<= (`self.WorkTime`) 0.0)
            (set `self.WorkTime` 10.0)
            (set `self.RestTime` 2.0))))
      (else
        (set `self.RestTime` (- (`self.RestTime`) (`self.DeltaSec`))) ; 休憩時間観測
      ))))

(fn `UserConstructionScript`)