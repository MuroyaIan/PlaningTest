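; BP_Camera_SuckBoss02 is a camera actor that circles the player during the boss-suction cinematic.
; Once Start is set, each Tick checks the player weapon's SuckBoss flag and places the actor at a rotated forward offset, slightly raised, aimed at the player.
; The orbit yaw advances at a constant rate toward a fixed end angle and resets to its starting angle while suction is inactive.
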(event `self.ReceiveBeginPlay`)

(event `self.ReceiveTick`
  (params (DeltaSeconds :type "Float (single-precision)"))
  (set `self.DeltaSec` DeltaSeconds)
  (if (`self.bStart`)
    (bind _asbp_player (cast `/Game/Blueprints/Player/BP_Player` (`GameplayStatics.GetPlayerPawn` 0)))
    (if (`/Game/Blueprints/Weapon/BP_Weapon.bSuckBoss` (`/Game/Blueprints/Player/BP_Player.GetWeapon` _asbp_player))
      (bind _asbp_player_2 (cast `/Game/Blueprints/Player/BP_Player` (`GameplayStatics.GetPlayerPawn` 0)))
      (bind _returnvalue (`self.K2_GetActorLocation` _asbp_player_2))
      (bind _returnvalue_2 (+ (`KismetMathLibrary.GreaterGreater_VectorRotator` (* (`self.GetActorForwardVector` _asbp_player_2) 300.0) (`self.Rot`)) (* (`self.GetActorUpVector` _asbp_player_2) 30.0) _returnvalue))
      (`self.K2_SetActorLocation` _returnvalue_2) ; カメラ回転
      (`self.K2_SetActorRotation` (`KismetMathLibrary.FindLookAtRotation` _returnvalue_2 _returnvalue))
      (set `self.Rot` (`KismetMathLibrary.MakeRotator` 0.0 0.0 (`KismetMathLibrary.FInterpTo_Constant` (.yaw (`self.Rot`)) -270.0 (`self.DeltaSec`) 20.0))) ; 回転角更新
      (else
        (set `self.bStart` true)
        (set `self.Rot` (struct :`Yaw` -135.0))))))

(fn `UserConstructionScript`)