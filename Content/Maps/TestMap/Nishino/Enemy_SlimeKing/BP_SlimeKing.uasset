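; Slime King enemy Blueprint that tracks cooldown timers for jump, spin, bash and thrust attacks.
; Tick counts each timer down by delta time, clamped at zero, through per-attack functions and prints the values for debugging.
; Overlap events on the jump-attack damage component set a flag while the player pawn is inside.
; The child-actor cast event is an empty stub, and no attack execution logic appears here.
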(event `カスタムイベント_0`
  (`KismetSystemLibrary.PrintString` (`KismetStringLibrary.Conv_DoubleToString` (`self.T_JumpAttack`)) true true (struct :`R` 1.0 :`G` 0.085229 :`B` 0.998954 :`A` 1.0) 0.0)
  (`KismetSystemLibrary.PrintString` (`KismetStringLibrary.Conv_DoubleToString` (`self.T_SpinAttack`)) true true (struct :`R` 1.0 :`G` 0.085229 :`B` 0.998954 :`A` 1.0) 0.0)
  (`KismetSystemLibrary.PrintString` (`KismetStringLibrary.Conv_DoubleToString` (`self.T_BashAttack`)) true true (struct :`R` 1.0 :`G` 0.085229 :`B` 0.998954 :`A` 1.0) 0.0)
  (`KismetSystemLibrary.PrintString` (`KismetStringLibrary.Conv_DoubleToString` (`self.T_ThrustAttack`)) true true (struct :`R` 1.0 :`G` 0.085229 :`B` 0.998954 :`A` 1.0) 0.0))

(event `self.ReceiveBeginPlay`
  ;[1 0 0] Begin Play
  (`self.Cast_ChildActor`) ; キャスト処理
)

(event `self.ReceiveTick`
  (params (DeltaSeconds :type "Float (single-precision)"))
  ;[1 0 0] Tick
  (`self.UpdateCoolTime` DeltaSeconds) ; 攻撃のクールタイム確認
  (`self.カスタムイベント_0`))

(event `Cast_ChildActor`
  ;[0 1 0] キャスト処理
)

(event `UpdateCoolTime`
  (params (Sec :type "Float (double-precision)"))
  ;[1 1 0] クールタイムの更新
  (set `self.T_JumpAttack` (`KismetMathLibrary.FClamp` (- (`self.T_JumpAttack`) Sec) 0.0 60000.0))
  (set `self.T_SpinAttack` (`KismetMathLibrary.FClamp` (- (`self.T_SpinAttack`) Sec) 0.0 60000.0))
  (set `self.T_BashAttack` (`KismetMathLibrary.FClamp` (- (`self.T_BashAttack`) Sec) 0.0 60000.0))
  (set `self.T_ThrustAttack` (`KismetMathLibrary.FClamp` (- (`self.T_ThrustAttack`) Sec) 0.0 60000.0)))

(event `self.DMG_JumpAttack.OnComponentBeginOverlap`
  (params (OverlappedComponent :type "PrimitiveComponent Object Reference") (OtherActor :type "Actor Object Reference") (OtherComp :type "PrimitiveComponent Object Reference") (OtherBodyIndex :type Integer) (bFromSweep :type Boolean) (SweepResult :type "HitResult Structure (by ref)"))
  ;[0 0 1] フラグ管理_JumpAttack
  (if (== OtherActor (`GameplayStatics.GetPlayerPawn` 0))
    (set `self.F_JumpAttack` true)))

(event `self.DMG_JumpAttack.OnComponentEndOverlap`
  (params (OverlappedComponent :type "PrimitiveComponent Object Reference") (OtherActor :type "Actor Object Reference") (OtherComp :type "PrimitiveComponent Object Reference") (OtherBodyIndex :type Integer))
  ;[0 0 1] フラグ管理_JumpAttack
  (if (== (`GameplayStatics.GetPlayerPawn` 0) OtherActor)
    (set `self.F_JumpAttack` false)))

(fn `UserConstructionScript`)