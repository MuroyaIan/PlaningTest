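; Timed dragon meteor spawner that rains BP_Dragon_BreathMeteor actors for 30 seconds, then expires.
; Tick fires on a short fixed interval, spawning each meteor slightly offset from the spawner toward a computed target, which it passes as TargetPos.
; CalcSpawnPos occasionally targets the player's XY at spawner height, otherwise picks a random point in a surrounding square, rerolling coordinates that fall near the centre.
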(event `self.ReceiveBeginPlay`
  (`self.SetLifeSpan` 30.0))

(event `self.ReceiveTick`
  (params (DeltaSeconds :type "Float (single-precision)"))
  (bind _returnvalue (`GameplayStatics.GetTimeSeconds`))
  (if (<= (+ (`self.PreviousSpawnTime`) 0.15) _returnvalue)
    (set `self.PreviousSpawnTime` _returnvalue)
    (bind _pos (`self.CalcSpawnPos`))
    (`|SpawnActorFromClass` "/Game/Blueprints/Dragon/BP_Dragon_BreathMeteor.BP_Dragon_BreathMeteor_C" (`KismetMathLibrary.MakeTransform` (+ (* (`KismetMathLibrary.Normal` (- _pos (`self.K2_GetActorLocation`))) 100.0) (`self.K2_GetActorLocation`))) "Undefined" "OverrideRootScale" null _pos 0.0 -1.0 null)))

(fn `CalcSpawnPos`
  (returns (Pos :type "Vector Structure"))
  (bind _returnvalue (`self.K2_GetActorLocation`))
  (bind (_returnvalue_x _returnvalue_y) (`KismetMathLibrary.BreakVector` (`self.K2_GetActorLocation` (`GameplayStatics.GetPlayerPawn` 0))))
  (bind (_returnvalue_x_2 _returnvalue_y_2 _returnvalue_z) (`KismetMathLibrary.BreakVector` (`KismetMathLibrary.MakeVector` (`KismetMathLibrary.RandomFloatInRange` -2000.0 2000.0) (`KismetMathLibrary.RandomFloatInRange` -2000.0 2000.0))))
  (bind _returnvalue_2 (> _returnvalue_x_2 -200.0))
  (return (`KismetMathLibrary.SelectVector` (`KismetMathLibrary.MakeVector` _returnvalue_x _returnvalue_y (.z _returnvalue)) (+ _returnvalue (`KismetMathLibrary.MakeVector` (`KismetMathLibrary.SelectFloat` (`KismetMathLibrary.RandomFloatInRange` (`KismetMathLibrary.Conv_BoolToDouble` _returnvalue_2) 2000.0) _returnvalue_x_2 (and _returnvalue_2 (< _returnvalue_x_2 200.0))) (`KismetMathLibrary.SelectFloat` (`KismetMathLibrary.RandomFloatInRange` -2000.0) _returnvalue_y_2 (and (> _returnvalue_y_2 -200.0) (< _returnvalue_y_2 200.0))) _returnvalue_z)) (<= (`KismetMathLibrary.RandomIntegerInRange` 1 10) 1))))

(fn `UserConstructionScript`)