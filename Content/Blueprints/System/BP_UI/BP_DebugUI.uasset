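; BP_DebugUI is an input-driven controller that shows and hides a debug UI widget and relays navigation to it.
; BeginPlay enables input from the first BP_PlayerController.
; DebugUI_Disp adds or removes the widget from the viewport, stores IsDisp on it and mirrors that into InputTrigger.
; While InputTrigger is set, directional actions call the widget's input functions and page back/forward actions call InputMode.
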(event `self.ReceiveBeginPlay`
  (bind _asbp_player_controller (cast `/Game/Blueprints/Player/BP_PlayerController` (`GameplayStatics.GetPlayerController` 0)))
  (`self.EnableInput` _asbp_player_controller) ; 入力有効化
)

(event `InputAction|DebugUI_Disp`
  (params (Key :type "Key Structure"))
  (bind _widget_debugui (`self.GetWidget`))
  ;[1 1 1] UIの表示切替
  (:`Pressed`
    (bind _returnisdisp (`self.DispWidget` _widget_debugui (`/Game/Maps/TestMap/Kitayama/UI_Kitayama/Widget_UI/DebugWidget/UMG_DebugUI.IsDisp` _widget_debugui))) ; カメラUIの表示非常時を切り替え
    (bind _output_get (set `/Game/Maps/TestMap/Kitayama/UI_Kitayama/Widget_UI/DebugWidget/UMG_DebugUI.IsDisp` _returnisdisp _widget_debugui))
    (set `self.InputTrigger` _output_get) ; 入力制御更新
  ))

(event `InputAction|UI_Right`
  (params (Key :type "Key Structure"))
  (:`Pressed`
    (if (`self.InputTrigger`)
      (`/Game/Maps/TestMap/Kitayama/UI_Kitayama/Widget_UI/DebugWidget/UMG_DebugUI.InputRight` (`self.GetWidget`)))))

(event `InputAction|UI_Left`
  (params (Key :type "Key Structure"))
  (:`Pressed`
    (if (`self.InputTrigger`)
      (`/Game/Maps/TestMap/Kitayama/UI_Kitayama/Widget_UI/DebugWidget/UMG_DebugUI.InputLeft` (`self.GetWidget`)))))

(event `InputAction|UI_Up`
  (params (Key :type "Key Structure"))
  (:`Pressed`
    (if (`self.InputTrigger`)
      (`/Game/Maps/TestMap/Kitayama/UI_Kitayama/Widget_UI/DebugWidget/UMG_DebugUI.Input_Up` (`self.GetWidget`)))))

(event `InputAction|UI_Down`
  (params (Key :type "Key Structure"))
  (:`Pressed`
    (if (`self.InputTrigger`)
      (`/Game/Maps/TestMap/Kitayama/UI_Kitayama/Widget_UI/DebugWidget/UMG_DebugUI.Input_Down` (`self.GetWidget`)))))

(event `InputAction|UI_PageBack`
  (params (Key :type "Key Structure"))
  ;[1 1 1] モード選択
  (:`Pressed`
    (if (`self.InputTrigger`)
      (`/Game/Maps/TestMap/Kitayama/UI_Kitayama/Widget_UI/DebugWidget/UMG_DebugUI.InputMode` (`self.GetWidget`) 0))))

(event `InputAction|UI_PageForward`
  (params (Key :type "Key Structure"))
  ;[1 1 1] モード選択
  (:`Pressed`
    (if (`self.InputTrigger`)
      (`/Game/Maps/TestMap/Kitayama/UI_Kitayama/Widget_UI/DebugWidget/UMG_DebugUI.InputMode` (`self.GetWidget`) 1))))

(fn `DispWidget`
  (params (Widget :type "UserWidget Object Reference") (IsDisp :type Boolean))
  (returns (ReturnIsDisp :type Boolean))
  (if IsDisp
    (`Widget.RemoveFromParent` Widget) ; UIの非表示にする
    (else
      (`UserWidget.AddToViewport` Widget 0) ; UIを表示する
    ))
  (return (not IsDisp)))

(fn `GetWidget`
  (returns (Widget_DebugUI :type "/Game/Maps/TestMap/Kitayama/UI_Kitayama/Widget_UI/DebugWidget/UMG_DebugUI Object Reference"))
  (return (`|ConvertAsset` (`self.Widget_DebugUI`))))

(fn `UserConstructionScript`)