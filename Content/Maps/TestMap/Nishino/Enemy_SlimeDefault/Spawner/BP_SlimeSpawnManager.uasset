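; Slime spawn manager that refills the tracked slime population as slimes become invalid.
; Every Tick, it scans slime slots up to SlimeMaxNum, removes invalid entries and rebuilds the list of usable spawn points via each point's CanActive.
; If any are usable, one random point spawns SlimeSpawnNum times, and successful spawns join the tracked array.
; Tick also prints slime names and "DIN" as debug output.
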(event `self.ReceiveTick`
  (params (DeltaSeconds :type "Float (single-precision)"))
  ;[1 0 0] Tick
  (`self.Chack_Slime`)
  (for _array_element (`self.Slime`)
    (`KismetSystemLibrary.PrintString` (`KismetSystemLibrary.GetDisplayName` _array_element) true true (struct :`G` 0.66 :`B` 1.0 :`A` 1.0) 0.0))
  (`KismetSystemLibrary.PrintString` "DIN" true true (struct :`G` 0.66 :`B` 1.0 :`A` 1.0) 0.0))

(event `Chack_Slime`
  (bind _slime (`self.Slime`))
  ;[0 1 0] スライムの状態を確認する
  (for _index (range (+ (`self.SlimeMaxNum`) 1))
    (bind _output (`|GetArrayItem` _slime _index))
    (`/Engine/EditorBlueprintResources/StandardMacros.IsValid` _output ; スライムが使い物になるかどうか確認
      (:`Is Not Valid`
        (`KismetArrayLibrary.Array_RemoveItem` _slime _output) ; 使えない情報を消去
        (bind _success (`self.Chack_Point`)) ; 使えるスポナーを確認
        (if _success
          (`self.Spawn_Slime`) ; スライムの作成
        )))))

(event `Spawn_Slime`
  (bind _activepoint (`self.ActivePoint`))
  ;[1 1 0] スライムの作成処理
  (bind _output_get (set `self.SelectSpawn` (`KismetMathLibrary.RandomInteger` (`KismetArrayLibrary.Array_Length` _activepoint)))) ; 使うスポナ番号を保存
  (for _ (range (+ (`self.SlimeSpawnNum`) 1))
    (bind (_success _bp) (`/Game/Maps/TestMap/Nishino/Enemy_SlimeDefault/Spawner/BP_SlimeSpawnPoint.Slime_Spawn` (`|GetArrayItem` _activepoint _output_get))) ; スライムの生成
    (if _success
      (`KismetArrayLibrary.Array_AddUnique` (`self.Slime`) _bp))))

(fn `Chack_Point`
  (returns (Success :type Boolean))
  (bind _activepoint (`self.ActivePoint`))
  (`KismetArrayLibrary.Array_Clear` _activepoint) ; 初期化
  (for _array_element (`self.SpawnPoint`)
    (bind _return (`/Game/Maps/TestMap/Nishino/Enemy_SlimeDefault/Spawner/BP_SlimeSpawnPoint.Can_Active` _array_element)) ; 実行可能かどうか確認する
    (if _return
      (`KismetArrayLibrary.Array_Add` _activepoint _array_element) ; 使用可能スポナを追加する
    ))
  (if (!= (`KismetArrayLibrary.Array_Length` _activepoint) 0)
    (return true) ; 使用可能
    (else
      (return false) ; 使用不可
    )))

(fn `UserConstructionScript`)