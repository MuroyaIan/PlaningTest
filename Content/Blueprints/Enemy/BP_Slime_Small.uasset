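; BP_Slime_Small is a small slime that the player's weapon sucks in, or that flies as a bullet.
; While not a bullet, it moves each tick toward the weapon's nozzle mesh, then calls EDSucked and destroys itself on overlapping the weapon.
; SetToBullet launches it via ProjectileMovement with gravity enabled after a timer; EndSuck also switches it to bullet mode.
; A nearly stopped bullet plays a hit effect and expires after a short lifespan.
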(event `self.ReceiveBeginPlay`
  (`|ExecutionSequence`
    (:`then_0`
      ;[0.4166 0.9901 1] プレイヤーの参照取得
      (bind _asbp_player_controller (cast `/Game/Blueprints/Player/BP_PlayerController` (`GameplayStatics.GetPlayerController` 0)))
      (set `self.PlayerRef` (`|ConvertAsset` (`/Game/Blueprints/Player/BP_PlayerController.GetPlayerPawn` _asbp_player_controller))))
    (:`then_1`
      ;[1 1 1] 重力無効化(もっといい方法知りたい)
      (`ActorComponent.Deactivate` (`self.CharacterMovement`))
      (`ActorComponent.Deactivate` (`self.ProjectileMovement`)))))

(event `self.ReceiveTick`
  (params (DeltaSeconds :type "Float (single-precision)"))
  (`|ExecutionSequence`
    (:`then_0`
      ;[0.3955 0.9801 1] 武器の参照取得
      (`/Engine/EditorBlueprintResources/StandardMacros.DoOnce` false
        (:`Completed`
          (bind _output_get (set `self.WeaponRef` (`/Game/Blueprints/Player/BP_Player.GetWeapon` (`|ConvertAsset` (`self.PlayerRef`)))))
          ;[0.2599 0.2366 1] イベントバインド
          (add `self.ED_Sucked` (`|CreateDelegate` (`|ConvertAsset` _output_get) :!event `AddSlime`)))))
    (:`then_1`
      (if (not (`self.IsBullet`))
        ;[0.3969 1 0.3036] 武器の方に近づく
        (bind _output_get_2 (set `self.PlayerDir` (`self.Get Wpeapon Direction Normalized`)))
        (`self.K2_AddActorWorldOffset` (* _output_get_2 (* DeltaSeconds (`self.Speed`))))
        (else
          ;[1 0.4695 0.8533] 接地したか?(速度が小さい==接地したとみなす)
          (if (< (`KismetMathLibrary.VSize` (`MovementComponent.Velocity` (`self.ProjectileMovement`))) 5.0)
            (`/Engine/EditorBlueprintResources/StandardMacros.DoOnce` false
              (:`Completed`
                (`self.SetLifeSpan` 3.0) ; 3秒後に消す
                (`ActorComponent.Activate` (`self.FX_VFX_PlayerHit`) false) ; ヒットエフェクト再生
              ))))))))

(event `End Suck`
  ;[1 0.7854 0.3782] 吸い込みをやめたとき
  (set `self.IsBullet` true)
  (`ActorComponent.Activate` (`self.ProjectileMovement`) false))

(event `self.StaticMesh.OnComponentBeginOverlap`
  (params (OverlappedComponent :type "PrimitiveComponent Object Reference") (OtherActor :type "Actor Object Reference") (OtherComp :type "PrimitiveComponent Object Reference") (OtherBodyIndex :type Integer) (bFromSweep :type Boolean) (SweepResult :type "HitResult Structure (by ref)"))
  ;[1 1 1] 武器に吸い込まれた(完全に)
  (if (`self.IsBullet`)
    ;[1 1 1] 付着スライムのスポーン
    (if (`self.ActorHasTag` "Weapon")
      _)
    (elif (`self.ActorHasTag` OtherActor "Weapon")
      (`self.ED_Sucked`)
      (`self.K2_DestroyActor`))))

(event `SetToBullet`
  (bind _projectilemovement (`self.ProjectileMovement`))
  ;[1 1 1] 弾モードにする
  (set `self.IsBullet` true)
  (`ActorComponent.Activate` _projectilemovement true)
  (set `ProjectileMovementComponent.ProjectileGravityScale` 0.0 _projectilemovement)
  (bind _output_get (set `MovementComponent.Velocity` (* (`self.GetActorForwardVector`) (`self.Bullet Initial Speed`)) _projectilemovement))
  (`self.K2_SetActorLocation` (- (`self.K2_GetActorLocation`) (* _output_get (`GameplayStatics.GetWorldDeltaSeconds`))))
  (`KismetSystemLibrary.K2_SetTimerDelegate` (delegate `EnableProjectileGravity`) (`self.TimeEnableGravity`)))

(event `EnableProjectileGravity`
  ;[1 1 1] 重力をかける
  (set `ProjectileMovementComponent.ProjectileGravityScale` 1.0 (`self.ProjectileMovement`)))

(fn `Get Wpeapon Direction Normalized`
  (returns (`Dir Normalized` :type "Vector Structure"))
  (return (`KismetMathLibrary.Normal` (- (`SceneComponent.K2_GetComponentLocation` (`|GetArrayItem` (`self.K2_GetComponentsByClass` (`|ConvertAsset` (`self.WeaponRef`)) "/Script/Engine.StaticMeshComponent") 1)) (`self.K2_GetActorLocation`)))))

(fn `UserConstructionScript`)