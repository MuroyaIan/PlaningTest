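; BP_Dragon_BreathLast is a dragon breath hazard actor that damages and knocks back the player on sphere overlap.
; On overlap it records the damage position, briefly ignores the Pawn channel on the player's capsule, and launches them horizontally away before applying damage.
; The sphere then disables collision for a few seconds as a hit cooldown, and OnCancelled destroys the actor.
; Tick's radius check has no effect, and the radius setter is unconnected.
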(event `self.ReceiveTick`
  (params (DeltaSeconds :type "Float (single-precision)"))
  (if (<= (+ (`SphereComponent.SphereRadius` (`self.PlayerCollsion`)) (* DeltaSeconds 1000.0)) 0.0)
    _))

(event `self.PlayerCollsion.OnComponentBeginOverlap`
  (params (OverlappedComponent :type "PrimitiveComponent Object Reference") (OtherActor :type "Actor Object Reference") (OtherComp :type "PrimitiveComponent Object Reference") (OtherBodyIndex :type Integer) (bFromSweep :type Boolean) (SweepResult :type "HitResult Structure (by ref)"))
  (bind _playercollsion (`self.PlayerCollsion`))
  (bind _asbp_player (cast `/Game/Blueprints/Player/BP_Player` OtherActor))
  (bind _output_get (set `/Game/Blueprints/Player/BP_Player.DamagePos` (`self.K2_GetActorLocation`) _asbp_player))
  (`PrimitiveComponent.SetCollisionResponseToChannel` (`Character.CapsuleComponent` _asbp_player) "ECC_Pawn" "ECR_Ignore")
  (`Character.LaunchCharacter` _asbp_player (* (`/Game/Blueprints/BP_FuncLibrary.Vector to 2D(NormalizeXY)` (`KismetMathLibrary.GetDirectionUnitVector` _output_get (`self.K2_GetActorLocation` _asbp_player))) 1000.0) false false)
  (`KismetSystemLibrary.Delay` 0.1)
  (`PrimitiveComponent.SetCollisionResponseToChannel` (`Character.CapsuleComponent` _asbp_player) "ECC_Pawn" "ECR_Block")
  (`GameplayStatics.ApplyDamage` _asbp_player 4.0)
  (`PrimitiveComponent.SetCollisionEnabled` _playercollsion "NoCollision")
  (`KismetSystemLibrary.Delay` 2.9)
  (`PrimitiveComponent.SetCollisionEnabled` _playercollsion "QueryOnly"))

(event `OnCancelled`
  (`self.K2_DestroyActor`))

(fn `UserConstructionScript`)