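; BP_Dragon_RedRing is an effect Blueprint, by name and folder a red ring decal for a dragon, animated through a dynamic material instance.
; Tick runs the parent, then advances a Time counter at double real-time speed and feeds it to the material's Time parameter.
; Once Time passes a fixed threshold, Opacity falls linearly with it, fading the ring out.
; The MID is not created in these graphs.
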(event `self.ReceiveTick`
  (params (DeltaSeconds :type "Float (single-precision)"))
  (`parent.ReceiveTick` DeltaSeconds)
  (`MaterialInstanceDynamic.SetScalarParameterValue` (`self.MID`) "Time" (`self.Time`))
  (bind _output_get (set `self.Time` (+ (`self.Time`) (* DeltaSeconds 2.0))))
  (if (> _output_get 2.0)
    (`MaterialInstanceDynamic.SetScalarParameterValue` (`self.MID`) "Opacity" (- (+ 2.0 1.0) (`self.Time`)))))

(fn `UserConstructionScript`
  (`parent.UserConstructionScript`))