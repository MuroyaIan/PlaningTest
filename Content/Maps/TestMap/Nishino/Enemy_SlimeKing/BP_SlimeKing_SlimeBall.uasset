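; Slime ball actor for the Slime King enemy in Nishino's test map, with a visible slime and a sphere for hit detection.
; On BeginPlay it scales the Slime component by SlimeScale times HitPar, while a separate SetSphereSize event sets the hit sphere's radius.
; The sphere's overlap handler only prints a debug string, so no hit effect is implemented in its graphs.
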(event `self.ReceiveBeginPlay`
  (`self.ChangeSlimeScale`))

(event `ChangeSlimeScale`
  ;[1 0 0] スライムの大きさ調整
  (`SceneComponent.SetRelativeScale3D` (`self.Slime`) (* (`self.SlimeScale`) (`self.HitPar`))))

(event `SetSphereSize`
  (params (Size :type "Float (double-precision)"))
  ;[0 1 0] 当たり判定大きさ変更処理
  (`SphereComponent.SetSphereRadius` (`self.HitSphere`) Size true))

(event `self.HitSphere.OnComponentBeginOverlap`
  (params (OverlappedComponent :type "PrimitiveComponent Object Reference") (OtherActor :type "Actor Object Reference") (OtherComp :type "PrimitiveComponent Object Reference") (OtherBodyIndex :type Integer) (bFromSweep :type Boolean) (SweepResult :type "HitResult Structure (by ref)"))
  (`KismetSystemLibrary.PrintString` "Hello"))

(fn `UserConstructionScript`)