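; Title-screen camera that travels along a spline route as a scene transition once Start is set.
; Each Tick it advances distance by MoveSpeed and targets the yaw toward the next spline point, with a fixed slight upward pitch.
; Rotation continuously eases to that target via constant-rate interpolation, whose speed ramps up per frame to a cap.
; That ramp also triggers a delayed Fade flag on BP_GlobalData in the GameInstance.
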(event `self.ReceiveBeginPlay`)

(event `self.ReceiveTick`
  (params (DeltaSeconds :type "Float (single-precision)"))
  (bind _cameracomponent (`self.CameraComponent`))
  (bind _rotspeed (`self.RotSpeed`))
  (bind _returnvalue (`SplineComponent.GetLocationAtDistanceAlongSpline` (`self.Spline_CameraRoute`) (`self.CurrentDistance`) "World"))
  (set `self.DeltaSec` DeltaSeconds)
  (`|ExecutionSequence`
    (:`then_0`
      (if (`self.bStart`)
        (set `self.CurrentDistance` (+ (`self.CurrentDistance`) (* (`self.MoveSpeed`) (`self.DeltaSec`)))) ; 移動先位置取得
        (set `self.TgtCamRot` (`KismetMathLibrary.MakeRotator` 0.0 10.0 (.yaw (`KismetMathLibrary.FindLookAtRotation` (`/Game/Blueprints/BP_FuncLibrary.Vector to 2D(XY)` (`SceneComponent.K2_GetComponentLocation` _cameracomponent)) (`/Game/Blueprints/BP_FuncLibrary.Vector to 2D(XY)` _returnvalue))))) ; 回転目標更新
        (`SceneComponent.K2_SetWorldLocation` _cameracomponent _returnvalue false false) ; 位置更新
        (if (< _rotspeed 13.0)
          (set `self.RotSpeed` (+ _rotspeed 1.0))
          (`KismetSystemLibrary.Delay` 2.0)
          (bind _asbp_global_data (cast `/Game/Blueprints/System/BP_GlobalData` (`GameplayStatics.GetGameInstance`)))
          (set `/Game/Blueprints/System/BP_GlobalData.bFade` true _asbp_global_data)
          (else
            (set `self.RotSpeed` 13.0)))))
    (:`then_1`
      (`SceneComponent.K2_SetWorldRotation` (`self.CameraComponent`) (`self.CamRot`) false false) ; 回転更新
      (set `self.CamRot` (`KismetMathLibrary.RInterpTo_Constant` (`self.CamRot`) (`self.TgtCamRot`) (`self.DeltaSec`) (`self.RotSpeed`))))))

(fn `UserConstructionScript`)