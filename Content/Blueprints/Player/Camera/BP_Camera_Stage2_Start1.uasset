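; BP_Camera_Stage2_Start1 is a camera Blueprint that, judging by its name, plays a Stage 2 opening camera move.
; While Start is set and Fin is not, Tick advances a distance by MoveSpeed times delta time and places the camera component at that point on SplineStageStart.
; Only location follows the spline, and Fin is set once the distance reaches the spline's length.
; Nothing in this Blueprint sets Start.
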(event `self.ReceiveTick`
  (params (DeltaSeconds :type "Float (single-precision)"))
  (if (and (`self.bStart`) (not (`self.bFin`)))
    (set `self.CurrentDistance` (+ (`self.CurrentDistance`) (* (`self.MoveSpeed`) DeltaSeconds)))
    (`SceneComponent.K2_SetWorldLocation` (`self.CameraComponent`) (`SplineComponent.GetLocationAtDistanceAlongSpline` (`self.Spline_StageStart`) (`self.CurrentDistance`) "World") false false)
    (if (>= (`self.CurrentDistance`) (`SplineComponent.GetSplineLength` (`self.Spline_StageStart`)))
      (set `self.bFin` true))))

(fn `UserConstructionScript`)