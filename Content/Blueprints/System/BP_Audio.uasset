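; BP_Audio applies the player's saved BGM and SE volume settings to the game's audio when it begins play.
; InitSound reads the two volume values from the BP_GlobalData game instance and divides each by ten.
; It then sets them as class overrides for the SO_BGM and SO_SE sound classes on the SO_SoundMix, pushing the mix after each override.
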(event `self.ReceiveBeginPlay`
  (`self.InitSound`))

(event `self.ReceiveTick`
  (params (DeltaSeconds :type "Float (single-precision)")))

(fn `InitSound`
  (bind _asbp_global_data (cast `/Game/Blueprints/System/BP_GlobalData` (`GameplayStatics.GetGameInstance`)))
  (`|ExecutionSequence`
    (:`then_0`
      (`GameplayStatics.SetSoundMixClassOverride` "/Game/Blueprints/Sound/SO_SoundMix.SO_SoundMix" "/Game/Blueprints/Sound/SO_BGM.SO_BGM" (/ (`KismetMathLibrary.Conv_IntToDouble` (`/Game/Blueprints/System/BP_GlobalData.Volume_BGM` _asbp_global_data)) 10.0) 1.0 0.0) ; 音量情報の上書き
      (`GameplayStatics.PushSoundMixModifier` "/Game/Blueprints/Sound/SO_SoundMix.SO_SoundMix") ; 音量情報の更新
    )
    (:`then_1`
      (`GameplayStatics.SetSoundMixClassOverride` "/Game/Blueprints/Sound/SO_SoundMix.SO_SoundMix" "/Game/Blueprints/Sound/SO_SE.SO_SE" (/ (`KismetMathLibrary.Conv_IntToDouble` (`/Game/Blueprints/System/BP_GlobalData.Volume_SE` _asbp_global_data)) 10.0) 1.0 0.0) ; 音量情報の上書き
      (`GameplayStatics.PushSoundMixModifier` "/Game/Blueprints/Sound/SO_SoundMix.SO_SoundMix") ; 音量情報の更新
    )))

(fn `UserConstructionScript`)