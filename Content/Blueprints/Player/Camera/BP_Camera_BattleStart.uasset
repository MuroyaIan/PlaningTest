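; Battle-start intro camera that frames the boss from the player's side and orbits it.
; Tick keeps it at a set distance and height, looking at the boss, until Start is set.
; It then orbits left or right, chosen once by a 2D cross product of player forward and direction to boss.
; Delays blend the view back to the player pawn after 3 seconds and destroy the camera after 5.
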(event `self.ReceiveBeginPlay`
  (set `self.PlayerPos` (`GameplayStatics.GetPlayerPawn` 0)) ; プレイヤー座標初期化
)

(event `self.ReceiveTick`
  (params (DeltaSeconds :type "Float (single-precision)"))
  (set `self.DeltaSec` DeltaSeconds)
  (if (not (`self.bStart`))
    (`self.SetPosAndRot`)
    (else
      (`|ExecutionSequence`
        (:`then_0`
          (`/Engine/EditorBlueprintResources/StandardMacros.DoOnce` false
            (:`Completed`
              (if (>= (`KismetMathLibrary.CrossProduct2D` (`KismetMathLibrary.Normal2D` (`KismetMathLibrary.Conv_VectorToVector2D` (`self.GetActorForwardVector` (`self.PlayerPos`)))) (`KismetMathLibrary.Normal2D` (`KismetMathLibrary.Conv_VectorToVector2D` (- (`self.K2_GetActorLocation` (`self.BossPos`)) (`self.K2_GetActorLocation` (`self.PlayerPos`)))))) 0.0)
                (set `self.bTurnRight` true)
                (else
                  (set `self.bTurnRight` false)))
              (`KismetSystemLibrary.Delay` 3.0)
              (`PlayerController.SetViewTargetWithBlend` (`GameplayStatics.GetPlayerController` 0) (`GameplayStatics.GetPlayerPawn` 0) 1.0 "VTBlend_Cubic" 0.0 false) ; 戦闘開始演出
            )))
        (:`then_1`
          (`|ExecutionSequence`
            (:`then_0`
              (if (`self.bTurnRight`)
                (`self.SetPosAndRot_R`)
                (else
                  (`self.SetPosAndRot_L`))))
            (:`then_1`
              (`KismetSystemLibrary.Delay` 5.0)
              (`self.K2_DestroyActor`))))))))

(fn `SetPosAndRot`
  (bind _returnvalue (`self.K2_GetActorLocation` (`self.BossPos`)))
  (`self.K2_SetActorLocation` (+ (* (`/Game/Blueprints/BP_FuncLibrary.Vector to 2D(NormalizeXY)` (- (`self.K2_GetActorLocation` (`self.PlayerPos`)) _returnvalue)) (`self.CameraDistance`)) _returnvalue (`KismetMathLibrary.MakeVector` 0.0 0.0 (`self.CameraHeight`))))
  (`self.K2_SetActorRotation` (`KismetMathLibrary.FindLookAtRotation` (`self.K2_GetActorLocation`) _returnvalue)))

(fn `SetPosAndRot_L`
  (bind _returnvalue (`self.K2_GetActorLocation` (`self.BossPos`)))
  (`self.K2_SetActorLocation` (+ (`KismetMathLibrary.GreaterGreater_VectorRotator` (* (`/Game/Blueprints/BP_FuncLibrary.Vector to 2D(NormalizeXY)` (- (`self.K2_GetActorLocation` (`self.PlayerPos`)) _returnvalue)) (`self.CameraDistance`)) (`KismetMathLibrary.MakeRotator` 0.0 0.0 (`self.TurnDegree`))) _returnvalue (`KismetMathLibrary.MakeVector` 0.0 0.0 (`self.CameraHeight`))))
  (`self.K2_SetActorRotation` (`KismetMathLibrary.FindLookAtRotation` (`self.K2_GetActorLocation`) _returnvalue))
  (set `self.TurnDegree` (+ (`self.TurnDegree`) (* (`self.DeltaSec`) (* (`self.TurnSpeed`) -1.0)))))

(fn `SetPosAndRot_R`
  (bind _returnvalue (`self.K2_GetActorLocation` (`self.BossPos`)))
  (`self.K2_SetActorLocation` (+ (`KismetMathLibrary.GreaterGreater_VectorRotator` (* (`/Game/Blueprints/BP_FuncLibrary.Vector to 2D(NormalizeXY)` (- (`self.K2_GetActorLocation` (`self.PlayerPos`)) _returnvalue)) (`self.CameraDistance`)) (`KismetMathLibrary.MakeRotator` 0.0 0.0 (`self.TurnDegree`))) _returnvalue (`KismetMathLibrary.MakeVector` 0.0 0.0 (`self.CameraHeight`))))
  (`self.K2_SetActorRotation` (`KismetMathLibrary.FindLookAtRotation` (`self.K2_GetActorLocation`) _returnvalue))
  (set `self.TurnDegree` (+ (`self.TurnDegree`) (* (`self.DeltaSec`) (`self.TurnSpeed`)))))

(fn `UserConstructionScript`)