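; Intro cinematic camera for the start of Stage 2 that orbits BP_Player, then hands over to gameplay.
; While Start is set, Tick pulls back and raises the camera per frame, swinging its yaw past a distance threshold while looking at the player.
; During the rise, it runs the player toward PlayerDirection.
; After a one-shot delay, it blends to the player's view and updates BP_GlobalData's StageStart and Cinema flags.
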(event `self.ReceiveTick`
  (params (DeltaSeconds :type "Float (single-precision)"))
  (bind _returnvalue (`GameplayStatics.GetPlayerPawn` 0))
  (bind _campos (`self.CamPos`))
  (bind _cameraheight (`self.CameraHeight`))
  (set `self.DeltaSec` DeltaSeconds)
  (if (and (`self.bStart`) (not (`self.bFin`)))
    (bind _asbp_player (cast `/Game/Blueprints/Player/BP_Player` (`GameplayStatics.GetPlayerPawn` 0)))
    (`|ExecutionSequence`
      (:`then_0`
        (`/Engine/EditorBlueprintResources/StandardMacros.DoOnce` false
          (:`Completed`
            (bind _returnvalue_2 (`self.K2_GetActorLocation` _asbp_player))
            (set `self.CamPos` (+ (`KismetMathLibrary.GreaterGreater_VectorRotator` (* (`self.GetActorForwardVector` _asbp_player) 140.0) (`self.Rot`)) (* (`self.GetActorUpVector` _asbp_player) -60.0) _returnvalue_2)) ; 視点初期化
            (set `self.GazePoint` (+ _returnvalue_2 (0.0 0.0 -60.0))) ; 注視点初期化
            (`KismetSystemLibrary.Delay` 2.8) ; カメラ切替
            (set `self.bFin` true)
            (`PlayerController.SetViewTargetWithBlend` (`GameplayStatics.GetPlayerController` 0) (`GameplayStatics.GetPlayerPawn` 0) 1.0 "VTBlend_EaseOut" 0.9 false) ; メインカメラ切替
            (bind _asbp_global_data (cast `/Game/Blueprints/System/BP_GlobalData` (`GameplayStatics.GetGameInstance`)))
            (set `/Game/Blueprints/System/BP_GlobalData.bStageStart` true _asbp_global_data)
            (set `/Game/Blueprints/System/BP_GlobalData.bCinema` false _asbp_global_data))))
      (:`then_1`
        (`|ExecutionSequence`
          (:`then_0`
            (`self.K2_SetActorLocation` _campos) ; カメラ更新
            (`self.K2_SetActorRotation` (`KismetMathLibrary.FindLookAtRotation` _campos (`self.GazePoint`)))
            (bind _returnvalue_3 (`self.K2_GetActorLocation` _asbp_player))
            (set `self.CamPos` (+ (`KismetMathLibrary.GreaterGreater_VectorRotator` (* (`self.GetActorForwardVector` _asbp_player) (`self.CameraDistance`)) (`self.Rot`)) (* (`self.GetActorUpVector` _asbp_player) (`self.CameraHeight`)) _returnvalue_3)) ; 視点更新
            (set `self.GazePoint` (+ _returnvalue_3 (`KismetMathLibrary.MakeVector` 0.0 0.0 (`self.CameraHeight`)))) ; 注視点初期化
            (if (>= (`self.CameraDistance`) 146.0)
              (set `self.Rot` (`KismetMathLibrary.MakeRotator` 0.0 0.0 (`KismetMathLibrary.FInterpTo_Constant` (.yaw (`self.Rot`)) -270.0 (`self.DeltaSec`) 80.0)))))
          (:`then_1`
            (set `self.CameraDistance` (+ (`self.CameraDistance`) 0.3)) ; カメラ距離更新
            (if (<= _cameraheight 60.0)
              (set `self.CameraHeight` (+ _cameraheight 0.6)) ; カメラ高さ更新
              (`self.K2_SetActorRotation` _returnvalue (`KismetMathLibrary.FindLookAtRotation` (`/Game/Blueprints/BP_FuncLibrary.Vector to 2D(XY)` (`self.K2_GetActorLocation` _returnvalue)) (`/Game/Blueprints/BP_FuncLibrary.Vector to 2D(XY)` (`self.K2_GetActorLocation` (`self.PlayerDirection`)))) false) ; プレイヤー向き更新
              (`Pawn.AddMovementInput` _returnvalue (`self.GetActorForwardVector` _returnvalue) 1.0 false) ; プレイヤー走行
            )))))))

(fn `UserConstructionScript`)