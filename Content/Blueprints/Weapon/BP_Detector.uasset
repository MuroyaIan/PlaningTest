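; BP_Detector is the suction detector that follows the player's weapon and vacuums up slimes and vulnerable boss parts.
; While scanning in aim mode, it runs a sphere trace along its up axis each tick and plays airflow FX with two alternating looping sounds.
; Hits trigger slime suction or Golem, Dragon and Slime King checks, which flag boss suction and snap the player's position and facing for the sequence.
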(event `self.ReceiveBeginPlay`)

(event `self.ReceiveTick`
  (params (DeltaSeconds :type "Float (single-precision)"))
  (`self.SetLocation`)
  (`self.SetRotation`)
  (`self.UpdateScan`)
  (`self.UpdateSuckFX`))

(event `StartScan`
  ;[1 1 1] 吸込みモード
  (`KismetSystemLibrary.Delay` 0.1) ; 回転終了まで吸込み開始しない
  (bind _asbp_player_controller (cast `/Game/Blueprints/Player/BP_PlayerController` (`GameplayStatics.GetPlayerController` 0)))
  (if (`/Game/Blueprints/Player/BP_PlayerController.AimMode` _asbp_player_controller)
    (set `self.ScanMode` true)
    (`ActorComponent.SetActive` (`self.AirFlow`) true false) ; エフェクトオン
    (`self.PlaySE_AirFlow`) ; 吸込み風SE
    (`KismetSystemLibrary.K2_SetTimer` null "PlaySE_AirFlow" 4.8 true)))

(event `EndScan`
  ;[1 1 1] 吸込みモード
  (if (`self.ScanMode`)
    (set `self.ScanMode` false)
    (`ActorComponent.SetActive` (`self.AirFlow`) false false) ; エフェクトオフ
    (`KismetSystemLibrary.K2_ClearTimer` null "PlaySE_AirFlow") ; 吸込み風SE
    (`self.StopSE_AirFlow`)))

(event `UpdateScan`
  (bind _returnvalue (`self.GetActorUpVector`))
  (bind _returnvalue_2 (`self.K2_GetActorLocation`))
  ;[1 1 1] 吸込みモード
  (if (`self.ScanMode`)
    (bind (_outhits _returnvalue_3) (`KismetSystemLibrary.SphereTraceMulti` :`Start` (+ _returnvalue_2 (* _returnvalue 122)) :`End` (+ _returnvalue_2 (* _returnvalue 322)) :`Radius` 100.0 :`TraceChannel` "TraceTypeQuery3" :`DrawTime` 1.0)) ; スライムスキャン開始
    (if _returnvalue_3
      (for _array_element _outhits
        (`|ExecutionSequence`
          (:`then_0`
            (bind (_bblockinghit _binitialoverlap _time _distance _location _impactpoint _normal _impactnormal _physmat _hitactor _hitcomponent) (`GameplayStatics.BreakHitResult` _array_element))
            (`self.HitSlime` _hitactor))
          (:`then_1`
            (`self.HitBoss` _hitactor _hitcomponent)))))))

(event `UpdateSuckFX`
  (bind _airflow (`self.AirFlow`))
  (bind _output (`|ConvertAsset` (`self.Weapon`)))
  ;[1 1 1] 吸込みモード
  (bind _asbp_player (cast `/Game/Blueprints/Player/BP_Player` (`GameplayStatics.GetPlayerPawn` 0)))
  (if (`/Game/Blueprints/Weapon/BP_Weapon.bSuckBoss` _output)
    (`/Engine/EditorBlueprintResources/StandardMacros.DoOnce` false :!label _label
      (:`Completed`
        (set `/Game/Blueprints/Weapon/BP_Weapon.Flask_Capacity` 1.0 _output)
        (`/Game/Blueprints/Player/BP_Player.UpdatePipeMID` _asbp_player false false)
        (if (`ActorComponent.IsActive` _airflow)
          (`ActorComponent.SetActive` _airflow false false) ; エフェクトオフ
          (`self.StopSE_AirFlow`))))
    (else
      (goto _label :!via `Reset`))))

(fn `HitBoss`
  (params (ActorRef :type "Actor Object Reference (by ref)") (ComponentRef :type "PrimitiveComponent Object Reference (by ref)"))
  (bind _returnvalue (`SceneComponent.K2_GetComponentLocation` ComponentRef))
  (bind _returnvalue_2 (`SceneComponent.K2_GetComponentLocation` ComponentRef))
  (bind _returnvalue_3 (`SceneComponent.K2_GetComponentLocation` ComponentRef))
  (bind _returnvalue_4 (`SceneComponent.K2_GetComponentLocation` ComponentRef))
  (bind _returnvalue_5 (`SceneComponent.K2_GetComponentLocation` ComponentRef))
  (bind _returnvalue_6 (`SceneComponent.K2_GetComponentLocation` ComponentRef))
  (`|ExecutionSequence`
    (:`then_0`
      (if (`self.ActorHasTag` ActorRef "SlimeKing")
        (bind _asbp_slime_king (cast `/Game/Maps/TestMap/Nishino/Enemy_SlimeKing/BP_SlimeKing` ActorRef)) ; スライム情報獲得
        (if (and (`/Game/Maps/TestMap/Nishino/Enemy_SlimeKing/BP_SlimeKing.ShieldFlg_Left` _asbp_slime_king) (`/Game/Maps/TestMap/Nishino/Enemy_SlimeKing/BP_SlimeKing.SmallFull_Left` _asbp_slime_king) (not (`/Game/Maps/TestMap/Nishino/Enemy_SlimeKing/BP_SlimeKing.ShieldSuckOn_Left` _asbp_slime_king)) (`ActorComponent.ComponentHasTag` ComponentRef "SlimeKing_Left"))
          (set `/Game/Maps/TestMap/Nishino/Enemy_SlimeKing/BP_SlimeKing.ShieldSuckOn_Left` true _asbp_slime_king)
          (set `/Game/Blueprints/Weapon/BP_Weapon.bSuckBoss` true (`|ConvertAsset` (`self.Weapon`))) ; 吸込み演出開始
          (`/Game/Maps/TestMap/Nishino/Enemy_SlimeKing/BP_SlimeKing.Look_StageOrigin` _asbp_slime_king)
          (bind _asbp_player (cast `/Game/Blueprints/Player/BP_Player` (`GameplayStatics.GetPlayerPawn` 0)))
          (bind _returnvalue_7 (`self.GetActorRightVector` _asbp_slime_king))
          (bind _returnvalue_8 (`KismetMathLibrary.MakeVector` (.x (+ _returnvalue_5 (* (`self.GetActorForwardVector` _asbp_slime_king) 600.0) (* _returnvalue_7 0.0))) (.y (+ _returnvalue_5 (* (`self.GetActorForwardVector` _asbp_slime_king) 600.0) (* _returnvalue_7 0.0))) (.z (`self.K2_GetActorLocation` _asbp_player))))
          (`self.K2_SetActorLocation` _asbp_player _returnvalue_8 false false) ; 演出スタンバイ
          (bind _playercontroller (`/Game/Blueprints/Player/BP_Player.GetUserController` _asbp_player))
          (bind _output_get (set `/Game/Blueprints/Player/BP_PlayerController.TargetRotation` (`KismetMathLibrary.FindLookAtRotation` (`/Game/Blueprints/BP_FuncLibrary.Vector to 2D(XY)` _returnvalue_8) (`/Game/Blueprints/BP_FuncLibrary.Vector to 2D(XY)` (+ _returnvalue_5 (* _returnvalue_7 110.0)))) _playercontroller))
          (bind _output_get_2 (set `/Game/Blueprints/Player/BP_PlayerController.Rotation` _output_get _playercontroller))
          (set `/Game/Blueprints/Player/BP_Player.CameraRot` _output_get_2 _asbp_player)
          (elif (and (`/Game/Maps/TestMap/Nishino/Enemy_SlimeKing/BP_SlimeKing.ShieldFlg_Right` _asbp_slime_king) (`/Game/Maps/TestMap/Nishino/Enemy_SlimeKing/BP_SlimeKing.SmallFull_Right` _asbp_slime_king) (not (`/Game/Maps/TestMap/Nishino/Enemy_SlimeKing/BP_SlimeKing.ShieldSuckOn_Right` _asbp_slime_king)) (`ActorComponent.ComponentHasTag` ComponentRef "SlimeKing_Right"))
            (set `/Game/Maps/TestMap/Nishino/Enemy_SlimeKing/BP_SlimeKing.ShieldSuckOn_Right` true _asbp_slime_king)
            (set `/Game/Blueprints/Weapon/BP_Weapon.bSuckBoss` true (`|ConvertAsset` (`self.Weapon`))) ; 吸込み演出開始
            (`/Game/Maps/TestMap/Nishino/Enemy_SlimeKing/BP_SlimeKing.Look_StageOrigin` _asbp_slime_king)
            (bind _asbp_player_2 (cast `/Game/Blueprints/Player/BP_Player` (`GameplayStatics.GetPlayerPawn` 0)))
            (bind _returnvalue_9 (`self.GetActorRightVector` _asbp_slime_king))
            (bind _returnvalue_10 (`KismetMathLibrary.MakeVector` (.x (+ _returnvalue_6 (* (`self.GetActorForwardVector` _asbp_slime_king) 600.0) (* _returnvalue_9 0.0))) (.y (+ _returnvalue_6 (* (`self.GetActorForwardVector` _asbp_slime_king) 600.0) (* _returnvalue_9 0.0))) (.z (`self.K2_GetActorLocation` _asbp_player_2))))
            (`self.K2_SetActorLocation` _asbp_player_2 _returnvalue_10 false false) ; 演出スタンバイ
            (bind _playercontroller_2 (`/Game/Blueprints/Player/BP_Player.GetUserController` _asbp_player_2))
            (bind _output_get_3 (set `/Game/Blueprints/Player/BP_PlayerController.TargetRotation` (`KismetMathLibrary.FindLookAtRotation` (`/Game/Blueprints/BP_FuncLibrary.Vector to 2D(XY)` _returnvalue_10) (`/Game/Blueprints/BP_FuncLibrary.Vector to 2D(XY)` (+ _returnvalue_6 (* _returnvalue_9 110.0)))) _playercontroller_2))
            (bind _output_get_4 (set `/Game/Blueprints/Player/BP_PlayerController.Rotation` _output_get_3 _playercontroller_2))
            (set `/Game/Blueprints/Player/BP_Player.CameraRot` _output_get_4 _asbp_player_2)
            (elif (and (not (`/Game/Maps/TestMap/Nishino/Enemy_SlimeKing/BP_SlimeKing.ShieldFlg_Left` _asbp_slime_king)) (not (`/Game/Maps/TestMap/Nishino/Enemy_SlimeKing/BP_SlimeKing.ShieldFlg_Right` _asbp_slime_king)) (not (`/Game/Maps/TestMap/Nishino/Enemy_SlimeKing/BP_SlimeKing.ShieldSuckOn_Main` _asbp_slime_king)) (`/Game/Maps/TestMap/Nishino/Enemy_SlimeKing/BP_SlimeKing.ShieldSuckOn_Left` _asbp_slime_king) (`/Game/Maps/TestMap/Nishino/Enemy_SlimeKing/BP_SlimeKing.ShieldSuckOn_Right` _asbp_slime_king) (`ActorComponent.ComponentHasTag` ComponentRef "SlimeKing_Body"))
              (set `/Game/Maps/TestMap/Nishino/Enemy_SlimeKing/BP_SlimeKing.ShieldSuckOn_Main` true _asbp_slime_king)
              (set `/Game/Blueprints/Weapon/BP_Weapon.bSuckBoss` true (`|ConvertAsset` (`self.Weapon`))) ; 吸込み演出開始
              (bind _asbp_player_3 (cast `/Game/Blueprints/Player/BP_Player` (`GameplayStatics.GetPlayerPawn` 0)))
              (set `/Game/Blueprints/Player/BP_Player.bKillBoss` true _asbp_player_3) ; 最終吸込み
              (`/Game/Maps/TestMap/Nishino/Enemy_SlimeKing/BP_SlimeKing.Look_StageOrigin` _asbp_slime_king)
              (bind _asbp_player_4 (cast `/Game/Blueprints/Player/BP_Player` (`GameplayStatics.GetPlayerPawn` 0)))
              (bind _returnvalue_11 (`self.GetActorRightVector` _asbp_slime_king))
              (bind _returnvalue_12 (`KismetMathLibrary.MakeVector` (.x (+ _returnvalue_4 (* (`self.GetActorForwardVector` _asbp_slime_king) 600.0) (* _returnvalue_11 0.0))) (.y (+ _returnvalue_4 (* (`self.GetActorForwardVector` _asbp_slime_king) 600.0) (* _returnvalue_11 0.0))) (.z (`self.K2_GetActorLocation` _asbp_player_4))))
              (`self.K2_SetActorLocation` _asbp_player_4 _returnvalue_12 false false) ; 演出スタンバイ
              (bind _playercontroller_3 (`/Game/Blueprints/Player/BP_Player.GetUserController` _asbp_player_4))
              (bind _output_get_5 (set `/Game/Blueprints/Player/BP_PlayerController.TargetRotation` (`KismetMathLibrary.FindLookAtRotation` (`/Game/Blueprints/BP_FuncLibrary.Vector to 2D(XY)` _returnvalue_12) (`/Game/Blueprints/BP_FuncLibrary.Vector to 2D(XY)` (+ _returnvalue_4 (* _returnvalue_11 110.0)))) _playercontroller_3))
              (bind _output_get_6 (set `/Game/Blueprints/Player/BP_PlayerController.Rotation` _output_get_5 _playercontroller_3))
              (set `/Game/Blueprints/Player/BP_Player.CameraRot` _output_get_6 _asbp_player_4)
              (elif (and (or (`/Game/Maps/TestMap/Nishino/Enemy_SlimeKing/BP_SlimeKing.ShieldFlg_Left` _asbp_slime_king) (`/Game/Maps/TestMap/Nishino/Enemy_SlimeKing/BP_SlimeKing.ShieldFlg_Right` _asbp_slime_king)) (`ActorComponent.ComponentHasTag` ComponentRef "SlimeKing"))
                (set `/Game/Maps/TestMap/Nishino/Enemy_SlimeKing/BP_SlimeKing.SuckFlg` true _asbp_slime_king)
                (`KismetSystemLibrary.PrintString` "SLIME KING SUCK" true true (struct :`R` 0.785329 :`G` 1.0 :`A` 1.0) 0.0)))))))
    (:`then_1`
      (if (`self.ActorHasTag` ActorRef "Golem")
        (bind _asbp_golem (cast `/Game/Blueprints/Golem/BP_Golem` ActorRef))
        (`|ExecutionSequence`
          (:`then_0`
            (if (not (`/Game/Blueprints/Golem/BP_Golem.bRightArmLose` _asbp_golem))
              (if (`/Game/Blueprints/Golem/BP_Golem.bCoverArm_R` _asbp_golem)
                (if (`ActorComponent.ComponentHasTag` ComponentRef "Golem_ArmR")
                  (set `/Game/Blueprints/Weapon/BP_Weapon.bSuckBoss` true (`|ConvertAsset` (`self.Weapon`))) ; 吸込み演出開始
                  (bind _asbp_player_5 (cast `/Game/Blueprints/Player/BP_Player` (`GameplayStatics.GetPlayerPawn` 0)))
                  (bind _returnvalue_13 (`self.GetActorRightVector` _asbp_golem))
                  (bind _returnvalue_14 (`KismetMathLibrary.MakeVector` (.x (+ _returnvalue_2 (* (`self.GetActorForwardVector` _asbp_golem) 500.0) (* _returnvalue_13 0.0))) (.y (+ _returnvalue_2 (* (`self.GetActorForwardVector` _asbp_golem) 500.0) (* _returnvalue_13 0.0))) (.z (`self.K2_GetActorLocation` _asbp_player_5))))
                  (`self.K2_SetActorLocation` _asbp_player_5 _returnvalue_14 false false) ; 演出スタンバイ
                  (bind _playercontroller_4 (`/Game/Blueprints/Player/BP_Player.GetUserController` _asbp_player_5))
                  (bind _output_get_7 (set `/Game/Blueprints/Player/BP_PlayerController.TargetRotation` (`KismetMathLibrary.FindLookAtRotation` (`/Game/Blueprints/BP_FuncLibrary.Vector to 2D(XY)` _returnvalue_14) (`/Game/Blueprints/BP_FuncLibrary.Vector to 2D(XY)` (+ _returnvalue_2 (* _returnvalue_13 110.0)))) _playercontroller_4))
                  (bind _output_get_8 (set `/Game/Blueprints/Player/BP_PlayerController.Rotation` _output_get_7 _playercontroller_4))
                  (set `/Game/Blueprints/Player/BP_Player.CameraRot` _output_get_8 _asbp_player_5)))))
          (:`then_1`
            (if (not (`/Game/Blueprints/Golem/BP_Golem.bLeftArmLose` _asbp_golem))
              (if (`/Game/Blueprints/Golem/BP_Golem.bCoverArm_L` _asbp_golem)
                (if (`ActorComponent.ComponentHasTag` ComponentRef "Golem_ArmL")
                  (set `/Game/Blueprints/Weapon/BP_Weapon.bSuckBoss` true (`|ConvertAsset` (`self.Weapon`))) ; 吸込み演出開始
                  (bind _asbp_player_6 (cast `/Game/Blueprints/Player/BP_Player` (`GameplayStatics.GetPlayerPawn` 0)))
                  (bind _returnvalue_15 (`self.GetActorRightVector` _asbp_golem))
                  (bind _returnvalue_16 (`KismetMathLibrary.MakeVector` (.x (+ _returnvalue_3 (* (`self.GetActorForwardVector` _asbp_golem) 500.0) (* _returnvalue_15 -15.0))) (.y (+ _returnvalue_3 (* (`self.GetActorForwardVector` _asbp_golem) 500.0) (* _returnvalue_15 -15.0))) (.z (`self.K2_GetActorLocation` _asbp_player_6))))
                  (`self.K2_SetActorLocation` _asbp_player_6 _returnvalue_16 false false) ; 演出スタンバイ
                  (bind _playercontroller_5 (`/Game/Blueprints/Player/BP_Player.GetUserController` _asbp_player_6))
                  (bind _output_get_9 (set `/Game/Blueprints/Player/BP_PlayerController.TargetRotation` (`KismetMathLibrary.FindLookAtRotation` (`/Game/Blueprints/BP_FuncLibrary.Vector to 2D(XY)` _returnvalue_16) (`/Game/Blueprints/BP_FuncLibrary.Vector to 2D(XY)` (+ _returnvalue_3 (* _returnvalue_15 110.0)))) _playercontroller_5))
                  (bind _output_get_10 (set `/Game/Blueprints/Player/BP_PlayerController.Rotation` _output_get_9 _playercontroller_5))
                  (set `/Game/Blueprints/Player/BP_Player.CameraRot` _output_get_10 _asbp_player_6)))))
          (:`then_2`
            (if (not (`/Game/Blueprints/Golem/BP_Golem.bBodyLose` _asbp_golem))
              (if (`/Game/Blueprints/Golem/BP_Golem.bCoverBody` _asbp_golem)
                (if (`ActorComponent.ComponentHasTag` ComponentRef "Golem_Body")
                  (set `/Game/Blueprints/Weapon/BP_Weapon.bSuckBoss` true (`|ConvertAsset` (`self.Weapon`))) ; 吸込み演出開始
                  (bind _asbp_player_7 (cast `/Game/Blueprints/Player/BP_Player` (`GameplayStatics.GetPlayerPawn` 0)))
                  (set `/Game/Blueprints/Player/BP_Player.bKillBoss` true _asbp_player_7) ; 最終吸込み
                  (bind _asbp_player_8 (cast `/Game/Blueprints/Player/BP_Player` (`GameplayStatics.GetPlayerPawn` 0)))
                  (bind _returnvalue_17 (`self.GetActorRightVector` _asbp_golem))
                  (bind _returnvalue_18 (`KismetMathLibrary.MakeVector` (.x (+ _returnvalue (* (`self.GetActorForwardVector` _asbp_golem) 1000.0) (* _returnvalue_17 0.0))) (.y (+ _returnvalue (* (`self.GetActorForwardVector` _asbp_golem) 1000.0) (* _returnvalue_17 0.0))) (.z (`self.K2_GetActorLocation` _asbp_player_8))))
                  (`self.K2_SetActorLocation` _asbp_player_8 _returnvalue_18 false false) ; 演出スタンバイ
                  (bind _playercontroller_6 (`/Game/Blueprints/Player/BP_Player.GetUserController` _asbp_player_8))
                  (bind _output_get_11 (set `/Game/Blueprints/Player/BP_PlayerController.TargetRotation` (`KismetMathLibrary.FindLookAtRotation` (`/Game/Blueprints/BP_FuncLibrary.Vector to 2D(XY)` _returnvalue_18) (`/Game/Blueprints/BP_FuncLibrary.Vector to 2D(XY)` (+ _returnvalue (* _returnvalue_17 50.0)))) _playercontroller_6))
                  (bind _output_get_12 (set `/Game/Blueprints/Player/BP_PlayerController.Rotation` _output_get_11 _playercontroller_6))
                  (set `/Game/Blueprints/Player/BP_Player.CameraRot` _output_get_12 _asbp_player_8))))))))
    (:`then_2`
      (if (`self.ActorHasTag` ActorRef "Boss_Dragon")
        (bind _asbp_dragon (cast `/Game/Blueprints/Dragon/BP_Dragon` ActorRef))
        (if (`/Game/Blueprints/Dragon/BP_Dragon.ReadyToSuck` _asbp_dragon)
          (set `/Game/Blueprints/Dragon/BP_Dragon.ReadyToSuck` false _asbp_dragon)
          (set `/Game/Blueprints/Weapon/BP_Weapon.bSuckBoss` true (`|ConvertAsset` (`self.Weapon`)))
          (bind _asbp_player_9 (cast `/Game/Blueprints/Player/BP_Player` (`GameplayStatics.GetPlayerPawn` 0)))
          (switch `int` (`/Game/Blueprints/Dragon/BP_Dragon.GetCurrentForm` _asbp_dragon)
            (:`1`
              _)
            (:`3`
              (set `/Game/Blueprints/Player/BP_Player.bKillBoss` true _asbp_player_9)))
          (bind _returnvalue_19 (`self.K2_GetActorLocation` _asbp_dragon))
          (bind _returnvalue_20 (`self.GetActorRightVector` _asbp_dragon))
          (bind _returnvalue_21 (`KismetMathLibrary.MakeVector` (.x (+ _returnvalue_19 (* (`self.GetActorForwardVector` _asbp_dragon) 750.0) (* _returnvalue_20 0.0))) (.y (+ _returnvalue_19 (* (`self.GetActorForwardVector` _asbp_dragon) 750.0) (* _returnvalue_20 0.0))) (.z (`self.K2_GetActorLocation` _asbp_player_9))))
          (`self.K2_SetActorLocation` _asbp_player_9 _returnvalue_21 false false) ; 演出スタンバイ
          (bind _playercontroller_7 (`/Game/Blueprints/Player/BP_Player.GetUserController` _asbp_player_9))
          (bind _output_get_13 (set `/Game/Blueprints/Player/BP_PlayerController.TargetRotation` (`KismetMathLibrary.FindLookAtRotation` (`/Game/Blueprints/BP_FuncLibrary.Vector to 2D(XY)` _returnvalue_21) (`/Game/Blueprints/BP_FuncLibrary.Vector to 2D(XY)` (+ _returnvalue_19 (* _returnvalue_20 110.0)))) _playercontroller_7))
          (bind _output_get_14 (set `/Game/Blueprints/Player/BP_PlayerController.Rotation` _output_get_13 _playercontroller_7))
          (set `/Game/Blueprints/Player/BP_Player.CameraRot` _output_get_14 _asbp_player_9))))))

(fn `HitSlime`
  (params (ActorRef :type "Actor Object Reference (by ref)"))
  (if (`self.ActorHasTag` ActorRef "Slime")
    (bind _asbp_slime_default (cast `/Game/Maps/TestMap/Nishino/Enemy_SlimeDefault/BP_SlimeDefault` ActorRef))
    (`|ExecutionSequence`
      (:`then_0`
        (bind _ifbind (`/Game/Maps/TestMap/Nishino/Enemy_SlimeDefault/BP_SlimeDefault.Check_Bind` _asbp_slime_default))
        (if _ifbind
          (add `self.StartSuck` (`|CreateDelegate` _asbp_slime_default :!event `HitSuck`))))
      (:`then_1`
        (`/Game/Maps/TestMap/Nishino/Enemy_SlimeDefault/BP_SlimeDefault.Check_Hit` _asbp_slime_default true)
        (`self.StartSuck`)))))

(fn `PlaySE_AirFlow`
  (if (`self.bChangeSoundSlot`)
    (`AudioComponent.Play` (`self.SE_SO_Garnet_AirFlow_Cue_1`) 0.0)
    (set `self.bChangeSoundSlot` false)
    (`AudioComponent.StopDelayed` (`self.SE_SO_Garnet_AirFlow_Cue_2`) 0.1)
    (else
      (`AudioComponent.Play` (`self.SE_SO_Garnet_AirFlow_Cue_2`) 0.0)
      (set `self.bChangeSoundSlot` true)
      (`AudioComponent.StopDelayed` (`self.SE_SO_Garnet_AirFlow_Cue_1`) 0.1))))

(fn `SetLocation`
  (`self.K2_SetActorLocation` (`self.K2_GetActorLocation` (`|ConvertAsset` (`self.Weapon`)))) ; 武器の位置と同期
  (bind _asbp_player (cast `/Game/Blueprints/Player/BP_Player` (`GameplayStatics.GetPlayerPawn` 0)))
  (bind _returnvalue (`SceneComponent.GetSocketLocation` (`Character.Mesh` _asbp_player) "JNT_weapon5"))
  (`SceneComponent.K2_SetWorldLocation` (`self.SE_SO_Garnet_AirFlow_Cue_1`) _returnvalue false false) ; SE位置更新
  (`SceneComponent.K2_SetWorldLocation` (`self.SE_SO_Garnet_AirFlow_Cue_2`) _returnvalue false false))

(fn `SetRotation`
  (`self.K2_SetActorRotation` (`self.K2_GetActorRotation` (`|ConvertAsset` (`self.Weapon`)))) ; 武器の回転と同期
)

(fn `StopSE_AirFlow`
  (`AudioComponent.Stop` (`self.SE_SO_Garnet_AirFlow_Cue_1`))
  (`AudioComponent.Stop` (`self.SE_SO_Garnet_AirFlow_Cue_2`)))

(fn `UserConstructionScript`)