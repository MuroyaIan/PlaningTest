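; Player character that spawns BP_Weapon and handles damage, footstep sounds and an offset spring-arm camera with aim zoom.
; Dynamic material instances drive the face, sun direction, flask liquid and suck/fire pipe flow.
; Damage is ignored during boss suction; otherwise it cancels weapon actions, turns toward heavy hits and flags stage loss in BP_GlobalData at zero Life.
; Tick updates materials, camera and hurt cooldown, and also resets Life to 20 every frame.
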(event `self.ReceiveBeginPlay`
  ;[1 1 1] マテリアル初期化
  (`self.InitBodyMID`)
  (`self.InitFlaskMID`)
  (`self.InitPipeMID`)
  (`self.InitCamera`)
  (bind _returnvalue (`|SpawnActorFromClass` "/Game/Blueprints/Weapon/BP_Weapon.BP_Weapon_C" (`self.GetTransform`) "Undefined" "OverrideRootScale" null null)) ; 武器生成
  (set `self.Weapon` (`|ConvertAsset` _returnvalue)) ; 参照設定
)

(event `self.ReceiveTick`
  (params (DeltaSeconds :type "Float (single-precision)"))
  (bind _weapon (`self.GetWeapon`))
  (bind _sunlight (`self.SunLight`))
  (set `self.DeltaSec` DeltaSeconds)
  ;[1 1 1] マテリアル更新
  (`|ExecutionSequence`
    (:`then_0`
      (if (`KismetSystemLibrary.IsValidSoftObjectReference` _sunlight)
        (`/Engine/EditorBlueprintResources/StandardMacros.DoOnce` false
          (:`Completed`
            (`MaterialInstanceDynamic.SetVectorParameterValue` (`self.MID_Body`) "LightVector" (`KismetMathLibrary.Conv_VectorToLinearColor` (* (`self.GetActorForwardVector` (`|ConvertAsset` _sunlight)) -1))) ; 太陽の向き更新
          ))))
    (:`then_1`
      (`self.UpdateFlaskMID_BottomFlask`)
      (`|ExecutionSequence`
        (:`then_0`
          (if (`self.bCheckPipeWhenSuck`)
            (set `self.Timer_PipeStopSuck` 0.5)
            (set `self.bCheckPipeWhenSuck` false))
          (if (> (`self.Timer_PipeStopSuck`) 0.0)
            (set `self.Timer_PipeStopSuck` (- (`self.Timer_PipeStopSuck`) (`self.DeltaSec`))) ; タイマ計測
            (goto _label :!via `Reset`)
            (else
              (set `self.Timer_PipeStopSuck` 0.0)
              (`/Engine/EditorBlueprintResources/StandardMacros.DoOnce` false :!label _label
                (:`Completed`
                  (if (and (not (`/Game/Blueprints/Weapon/BP_Weapon.bSuckSuccess` _weapon)) (not (`/Game/Blueprints/Weapon/BP_Weapon.bFireSuccess` _weapon)))
                    (`self.UpdatePipeMID` false) ; パイプFX終了
                  ))))))
        (:`then_1`
          (`self.UpdateCamera`)
          (`self.UpdateHurtProcess`)
          (`self.PrintPlayerInfo`)
          (`self.PrintCameraInfo`)
          (set `self.Life` 20))))))

(event `self.ReceiveAnyDamage`
  (params (Damage :type "Float (single-precision)") (DamageType :type "DamageType Object Reference") (InstigatedBy :type "Controller Object Reference") (DamageCauser :type "Actor Object Reference"))
  (bind _playercontroller (`self.GetUserController`))
  (bind _playercontroller_2 (`self.GetUserController`))
  ;[1 1 1] ダメージ処理
  (bind _suckboss (`self.CheckIfSuck`))
  (if _suckboss
    (if (not (`self.bHurt`))
      (if (`self.bCanHurt`)
        (`|ExecutionSequence`
          (:`then_0`
            (bind _output_get (set `self.Life` (- (`self.Life`) (`KismetMathLibrary.Round` Damage)))) ; ライフ更新
            (set `self.bHurt` true) ; 連続ダメージ防止
            (if (<= _output_get 0)
              (set `self.Life` 0)
              (bind _asbp_global_data (cast `/Game/Blueprints/System/BP_GlobalData` (`GameplayStatics.GetGameInstance`)))
              (set `/Game/Blueprints/System/BP_GlobalData.bStageEnd_Lose` true _asbp_global_data) ; ステージ敗北
            ))
          (:`then_1`
            (`|ExecutionSequence`
              (:`then_0`
                (`/Game/Blueprints/Player/BP_PlayerController.FireOff` _playercontroller) ; 武器状態リセット
                (`/Game/Blueprints/Player/BP_PlayerController.SuckOff` _playercontroller)
                (`MaterialInstanceDynamic.SetScalarParameterValue` (`self.MID_Body`) "Face" 1.0) ; 表情更新
              )
              (:`then_1`
                (bind _asbp_global_data_2 (cast `/Game/Blueprints/System/BP_GlobalData` (`GameplayStatics.GetGameInstance`))) ; ステージ敗北時処理をスルー
                (if (not (`/Game/Blueprints/System/BP_GlobalData.bStageEnd_Lose` _asbp_global_data_2))
                  (if (> Damage 1.0)
                    (set `self.bBadHurt` true)
                    (else
                      (set `self.bBadHurt` false)))
                  (if (`self.bBadHurt`)
                    (bind _output_get_2 (set `/Game/Blueprints/Player/BP_PlayerController.TargetRotation` (`KismetMathLibrary.FindLookAtRotation` (`/Game/Blueprints/BP_FuncLibrary.Vector to 2D(XY)` (`self.K2_GetActorLocation`)) (`/Game/Blueprints/BP_FuncLibrary.Vector to 2D(XY)` (`self.DamagePos`))) _playercontroller_2)) ; ダメージ処理方向更新
                    (bind _output_get_3 (set `/Game/Blueprints/Player/BP_PlayerController.Rotation` _output_get_2 _playercontroller_2))
                    (set `self.CameraRot` _output_get_3) ; カメラ向き更新
                  ))))))))))

(event `UpdateHurtProcess`
  ;[1 1 1] ダメージ処理
  (if (not (`self.bCanHurt`))
    (`|ExecutionSequence`
      (:`then_0`
        (`KismetSystemLibrary.Delay` 0.2) ; CD（警告：0.2s以上）
        (set `self.bCanHurt` true)
        (`MaterialInstanceDynamic.SetScalarParameterValue` (`self.MID_Body`) "Face" 0.0) ; 表情リセット
        (goto _label_2 :!via `Reset`))
      (:`then_1`
        (`/Engine/EditorBlueprintResources/StandardMacros.DoOnce` false :!label _label_2
          (:`Completed`
            (`/Game/Blueprints/Player/BP_PlayerController.CheckWeaponWhenStop` (`self.GetUserController`)) ; 武器状態確認
          ))))))

(fn `AddCameraPitch`
  (params (Value :type "Float (double-precision) (by ref)"))
  (locals (CameraRot_Local :type "Rotator Structure"))
  (bind _asbp_player_controller (cast `/Game/Blueprints/Player/BP_PlayerController` (`GameplayStatics.GetPlayerController` 0)))
  (bind _cameramanager (`/Game/Blueprints/Player/BP_PlayerController.GetCameraManager` _asbp_player_controller))
  (set `local.CameraRot_Local` (`KismetMathLibrary.MakeRotator` (.roll (`self.CameraRot`)) (`KismetMathLibrary.ClampAngle` (+ (.pitch (`self.CameraRot`)) Value) (`PlayerCameraManager.ViewPitchMin` _cameramanager) (`PlayerCameraManager.ViewPitchMax` _cameramanager)) (.yaw (`self.CameraRot`))))
  (if (`/Game/Blueprints/Player/BP_PlayerController.AimMode` _asbp_player_controller)
    (set `self.CameraRot` (`KismetMathLibrary.MakeRotator` (.roll (`local.CameraRot_Local`)) (`KismetMathLibrary.ClampAngle` (.pitch (`local.CameraRot_Local`)) -40.0 35.0) (.yaw (`local.CameraRot_Local`)))) ; ピッチ回転更新
    (else
      (set `self.CameraRot` (`local.CameraRot_Local`)) ; ピッチ回転更新
    )))

(fn `AddCameraYaw`
  (params (Value :type "Float (double-precision) (by ref)"))
  (if (!= 0.0 Value)
    (set `self.CameraRot` (`KismetMathLibrary.MakeRotator` (.roll (`self.CameraRot`)) (.pitch (`self.CameraRot`)) (+ (.yaw (`self.CameraRot`)) Value))) ; ヨー回転更新
  ))

(fn `CheckIfSuck`
  (returns (SuckBoss :type Boolean))
  (return (not (`/Game/Blueprints/Weapon/BP_Weapon.bSuckBoss` (`self.GetWeapon`)))))

(fn `GetUserController`
  (returns (PlayerController :type "/Game/Blueprints/Player/BP_PlayerController Object Reference"))
  (bind _asbp_player_controller (cast `/Game/Blueprints/Player/BP_PlayerController` (`self.GetController`)))
  (return _asbp_player_controller))

(fn `GetWeapon`
  (returns (Weapon :type "/Game/Blueprints/Weapon/BP_Weapon Object Reference"))
  (bind _weapon (`self.Weapon`))
  (if (`KismetSystemLibrary.IsValidSoftObjectReference` _weapon)
    (return (`|ConvertAsset` _weapon))))

(fn `InitBodyMID`
  (bind _mesh (`self.Mesh`))
  (bind _returnvalue (`PrimitiveComponent.CreateDynamicMaterialInstance` _mesh 0 (`PrimitiveComponent.GetMaterial` _mesh 0) "None")) ; 本体用MID
  (bind _output_get (set `self.MID_Body` _returnvalue))
  (`MaterialInstanceDynamic.SetScalarParameterValue` _output_get "Face" 0.0) ; 表情初期化
  (`MaterialInstanceDynamic.SetScalarParameterValue` _output_get "MaskMode" 2.0) ; プレイヤー隠し機能初期化
)

(fn `InitCamera`
  (bind _springarm (`self.SpringArm`))
  (bind _output_get (set `self.ArmLength` (`KismetMathLibrary.Hypotenuse` 100.0 250.0))) ; アーム長さ設定
  (set `SpringArmComponent.TargetArmLength` _output_get _springarm) ; 長さ初期化
  (bind _output_get_2 (set `self.ArmRot` (`KismetMathLibrary.Conv_VectorToRotator` (`KismetMathLibrary.MakeVector` 250.0 -100.0)))) ; アーム回転設定
  (`SceneComponent.K2_SetWorldRotation` _springarm _output_get_2 false false) ; 回転初期化
  (`SceneComponent.K2_SetRelativeRotation` (`self.Camera`) (* _output_get_2 -1.0) false false) ; カメラ回転初期化（アームの回転分を打ち消す）
)

(fn `InitFlaskMID`
  (bind _mesh (`self.Mesh`))
  (`|ExecutionSequence`
    (:`then_0`
      (bind _returnvalue (`PrimitiveComponent.CreateDynamicMaterialInstance` _mesh 2 (`PrimitiveComponent.GetMaterial` _mesh 2) "None")) ; フラスコ容量表示MID
      (bind _output_get (set `self.MID_Flask` _returnvalue))
      (`MaterialInstanceDynamic.SetScalarParameterValue` _output_get "TankCapacity" 0.0) ; フラスコ容量初期化
      (`MaterialInstanceDynamic.SetScalarParameterValue` _output_get "BottomFlask" (`self.FlaskRefPos`)) ; フラスコ参照位置更新
      (`MaterialInstanceDynamic.SetScalarParameterValue` _output_get "WaveStrength" 0.5) ; フラスコ揺れ具合更新
      (`MaterialInstanceDynamic.SetScalarParameterValue` _output_get "MaskMode" 1.0) ; プレイヤー隠し機能初期化
    )
    (:`then_1`
      (`|ExecutionSequence`
        (:`then_0`
          (bind _returnvalue_2 (`PrimitiveComponent.CreateDynamicMaterialInstance` _mesh 4 (`PrimitiveComponent.GetMaterial` _mesh 4) "None")) ; フラスコガラス用MID
          (bind _output_get_2 (set `self.MID_FlaskGlass` _returnvalue_2))
          (`MaterialInstanceDynamic.SetScalarParameterValue` _output_get_2 "TankCapacity" 0.0) ; フラスコ容量初期化
          (`MaterialInstanceDynamic.SetScalarParameterValue` _output_get_2 "BottomFlask" (`self.FlaskRefPos`)) ; フラスコ参照位置更新
          (`MaterialInstanceDynamic.SetScalarParameterValue` _output_get_2 "WaveStrength" 0.5) ; フラスコ揺れ具合更新
          (`MaterialInstanceDynamic.SetScalarParameterValue` _output_get_2 "MaskMode" 1.0) ; プレイヤー隠し機能初期化
        )
        (:`then_1`
          (bind _returnvalue_3 (`PrimitiveComponent.CreateDynamicMaterialInstance` _mesh 1 (`PrimitiveComponent.GetMaterial` _mesh 1) "None")) ; フラスコガラス（外側）用MID
          (bind _output_get_3 (set `self.MID_FlaskGlassOut` _returnvalue_3))
          (`MaterialInstanceDynamic.SetScalarParameterValue` _output_get_3 "MaskMode" 1.0) ; プレイヤー隠し機能初期化
        )))))

(fn `InitPipeMID`
  (bind _mesh (`self.Mesh`))
  (bind _returnvalue (`PrimitiveComponent.CreateDynamicMaterialInstance` _mesh 3 (`PrimitiveComponent.GetMaterial` _mesh 3) "None")) ; パイプ用MID
  (bind _output_get (set `self.MID_Pipe` _returnvalue))
  (`MaterialInstanceDynamic.SetScalarParameterValue` _output_get "MaskMode" 1.0) ; プレイヤー隠し機能初期化
  (`self.UpdatePipeMID` false))

(fn `PlaySE_FootStep`
  (bind _returnvalue (`SceneComponent.GetSocketLocation` (`self.Mesh`) "JNT_foot_R0_0"))
  (bind _returnvalue_2 (`SceneComponent.GetSocketLocation` (`self.Mesh`) "JNT_foot_R0_0"))
  (bind _returnvalue_3 (`SceneComponent.GetSocketLocation` (`self.Mesh`) "JNT_foot_R0_0"))
  (bind _asbp_global_data (cast `/Game/Blueprints/System/BP_GlobalData` (`GameplayStatics.GetGameInstance`)))
  (switch `int` (`/Game/Blueprints/System/BP_GlobalData.StageSelect` _asbp_global_data)
    (:`0`
      (if (`/Game/Blueprints/Player/BP_PlayerController.AimMode` (`self.GetUserController`))
        (`GameplayStatics.PlaySoundAtLocation` "/Game/Resource/SO/SE/Garnet/FootStep/SO_SE_Garnet_FootStep_Grass_Cue.SO_SE_Garnet_FootStep_Grass_Cue" _returnvalue (struct) 0.5 1.0 0.0 null null null)
        (else
          (`GameplayStatics.PlaySoundAtLocation` "/Game/Resource/SO/SE/Garnet/FootStep/SO_SE_Garnet_FootStep_Grass_Cue.SO_SE_Garnet_FootStep_Grass_Cue" _returnvalue (struct) 1.0 1.0 0.0 null null null))))
    (:`1`
      (if (`/Game/Blueprints/Player/BP_PlayerController.AimMode` (`self.GetUserController`))
        (`GameplayStatics.PlaySoundAtLocation` "/Game/Resource/SO/SE/Garnet/FootStep/SO_SE_Garnet_FootStep_Gravel_Cue.SO_SE_Garnet_FootStep_Gravel_Cue" _returnvalue_3 (struct) 0.5 1.0 0.0 null null null)
        (else
          (`GameplayStatics.PlaySoundAtLocation` "/Game/Resource/SO/SE/Garnet/FootStep/SO_SE_Garnet_FootStep_Gravel_Cue.SO_SE_Garnet_FootStep_Gravel_Cue" _returnvalue_3 (struct) 1.0 1.0 0.0 null null null))))
    (:`2`
      (if (`/Game/Blueprints/Player/BP_PlayerController.AimMode` (`self.GetUserController`))
        (`GameplayStatics.PlaySoundAtLocation` "/Game/Resource/SO/SE/Garnet/FootStep/SO_SE_Garnet_FootStep_Hard_Cue.SO_SE_Garnet_FootStep_Hard_Cue" _returnvalue_2 (struct) 0.5 1.0 0.0 null null null)
        (else
          (`GameplayStatics.PlaySoundAtLocation` "/Game/Resource/SO/SE/Garnet/FootStep/SO_SE_Garnet_FootStep_Hard_Cue.SO_SE_Garnet_FootStep_Hard_Cue" _returnvalue_2 (struct) 1.0 1.0 0.0 null null null))))))

(fn `PrintCameraInfo`
  (bind _camera (`self.Camera`))
  (bind _bdebug (`/Game/Blueprints/BP_FuncLibrary.CheckDebugPrint`))
  (if _bdebug
    (`KismetSystemLibrary.PrintString` (`KismetStringLibrary.Concat_StrStr` "[CameraInfo] \nAngleRoll:" (`KismetStringLibrary.Conv_IntToString` (`KismetMathLibrary.Round` (.roll (`SceneComponent.K2_GetComponentRotation` _camera)))) " \nAnglePitch:" (`KismetStringLibrary.Conv_IntToString` (`KismetMathLibrary.Round` (.pitch (`SceneComponent.K2_GetComponentRotation` _camera)))) " \nAngleYaw:" (`KismetStringLibrary.Conv_IntToString` (`KismetMathLibrary.Round` (.yaw (`SceneComponent.K2_GetComponentRotation` _camera)))) " \nDistance:" (`KismetStringLibrary.Conv_IntToString` (`KismetMathLibrary.Round` (`KismetMathLibrary.Vector_Distance` (`SceneComponent.K2_GetComponentLocation` _camera) (`SceneComponent.K2_GetComponentLocation` (`self.SpringArm`))))) " \nFOV:" (`KismetStringLibrary.Conv_IntToString` (`KismetMathLibrary.Round` (`self.CameraFOV`)))) true false (struct :`R` 1.0 :`A` 1.0) 0.0)))

(fn `PrintPlayerInfo`
  (bind _bdebug (`/Game/Blueprints/BP_FuncLibrary.CheckDebugPrint`))
  (if _bdebug
    (`KismetSystemLibrary.PrintString` (`KismetStringLibrary.Concat_StrStr` "[PlayerInfo] \nRotX:" (`KismetStringLibrary.Conv_IntToString` (`KismetMathLibrary.Round` (.roll (`self.K2_GetActorRotation`)))) " \nRotY:" (`KismetStringLibrary.Conv_IntToString` (`KismetMathLibrary.Round` (.pitch (`self.K2_GetActorRotation`)))) " \nRotZ:" (`KismetStringLibrary.Conv_IntToString` (`KismetMathLibrary.Round` (.yaw (`self.K2_GetActorRotation`)))) " \nSpeed:" (`KismetStringLibrary.Conv_IntToString` (`KismetMathLibrary.Round` (`KismetMathLibrary.VSize` (`self.GetVelocity`)))) " \nHP:" (`KismetStringLibrary.Conv_IntToString` (`self.Life`))) true false (struct :`G` 0.66 :`B` 1.0 :`A` 1.0) 0.0)))

(fn `UpdateCamera`
  (bind _camera (`self.Camera`))
  (bind _armrot (`self.ArmRot`))
  (`SceneComponent.K2_SetWorldRotation` (`self.SpringArm`) (`KismetMathLibrary.ComposeRotators` _armrot (`self.CameraRot`)) false false) ; アーム回転更新
  (`SceneComponent.K2_SetRelativeRotation` (`self.Camera`) (* _armrot -1.0) false false) ; カメラ回転更新（アームの回転分を打ち消す）
  ;[1 1 1] 照準中のズーム処理
  (if (`/Game/Blueprints/Player/BP_PlayerController.AimMode` (`self.GetUserController`))
    (bind _output_get (set `self.CameraFOV` (`KismetMathLibrary.FInterpTo_Constant` (`self.CameraFOV`) 88.0 (`self.DeltaSec`) (`self.FOV_Speed`))))
    (`CameraComponent.SetFieldOfView` _camera _output_get) ; ズームイン
    (else
      (bind _output_get_2 (set `self.CameraFOV` (`KismetMathLibrary.FInterpTo_Constant` (`self.CameraFOV`) 90.0 (`self.DeltaSec`) (`self.FOV_Speed`))))
      (`CameraComponent.SetFieldOfView` _camera _output_get_2) ; ズームアウト
    ))
  (if (`/Game/Blueprints/Weapon/BP_Weapon.bSuckBoss` (`self.GetWeapon`))
    (set `/Game/Blueprints/Player/BP_PlayerController.AimMode` false (`self.GetUserController`))))

(fn `UpdateFlaskMID`
  (params (FlaskLevel :type Integer))
  (bind _flaskcapacity (`self.FlaskCapacity`))
  (`|ExecutionSequence`
    (:`then_0`
      (switch `int` FlaskLevel
        (:`0`
          (set `self.FlaskCapacity` 0.0))
        (:`1`
          (set `self.FlaskCapacity` 0.3))
        (:`2`
          (set `self.FlaskCapacity` 0.4))
        (:`3`
          (set `self.FlaskCapacity` 0.5))
        (:`4`
          (set `self.FlaskCapacity` 0.6))
        (:`5`
          (set `self.FlaskCapacity` 0.7))
        (:`6`
          (set `self.FlaskCapacity` 0.8))
        (:`7`
          (set `self.FlaskCapacity` 0.9))
        (:`8`
          (set `self.FlaskCapacity` 1.0))))
    (:`then_1`
      (`MaterialInstanceDynamic.SetScalarParameterValue` (`self.MID_Flask`) "TankCapacity" _flaskcapacity) ; フラスコ容量更新
      (`MaterialInstanceDynamic.SetScalarParameterValue` (`self.MID_FlaskGlass`) "TankCapacity" _flaskcapacity) ; フラスコ容量更新
    )))

(fn `UpdateFlaskMID_BottomFlask`
  (bind _output_get (set `self.FlaskRefPos` (- (* (.z (`SceneComponent.GetSocketLocation` (`self.Mesh`) "JNT_flaskbottom_C0")) 1.0) 150.0)))
  (`MaterialInstanceDynamic.SetScalarParameterValue` (`self.MID_Flask`) "BottomFlask" _output_get) ; フラスコ参照位置更新
  (`MaterialInstanceDynamic.SetScalarParameterValue` (`self.MID_FlaskGlass`) "BottomFlask" _output_get) ; フラスコ参照位置更新
)

(fn `UpdateFlaskMID_WaveStrength`
  (params (BigWave :type Boolean))
  (bind _mid_flask (`self.MID_Flask`))
  (if BigWave
    (`MaterialInstanceDynamic.SetScalarParameterValue` _mid_flask "WaveStrength" 1.0) ; フラスコ揺れ具合更新（強）
    (else
      (`MaterialInstanceDynamic.SetScalarParameterValue` _mid_flask "WaveStrength" 0.5) ; フラスコ揺れ具合更新（弱）
    )))

(fn `UpdatePipeMID`
  (params (UsePipe :type Boolean) (SuckMode :type Boolean))
  (bind _mid_pipe (`self.MID_Pipe`))
  (bind _mid_pipe_2 (`self.MID_Pipe`))
  (if UsePipe
    (`MaterialInstanceDynamic.SetScalarParameterValue` _mid_pipe_2 "PipeFlow" 0.0)
    (if SuckMode
      (`MaterialInstanceDynamic.SetScalarParameterValue` _mid_pipe "Reverse" 1.0)
      (else
        (`MaterialInstanceDynamic.SetScalarParameterValue` _mid_pipe "Reverse" 0.0)))
    (else
      (`MaterialInstanceDynamic.SetScalarParameterValue` _mid_pipe_2 "PipeFlow" 1.0))))

(fn `UserConstructionScript`)