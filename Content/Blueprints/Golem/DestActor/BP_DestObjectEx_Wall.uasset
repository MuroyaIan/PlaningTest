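; Breakable wall that shatters when a Golem-tagged actor overlaps any of its three boxes.
; It swaps the static mesh for a damaged destructible component pushed along the Golem's forward vector, with slot-configured FX and a rock-break sound.
; After a delay, Tick fades the debris through a dynamic material's opacity mask, then destroys the actor.
; Box hits also destroy it during the player weapon's SuckBoss state, behind a Player tag check.
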(event `self.ReceiveBeginPlay`)

(event `self.ReceiveTick`
  (params (DeltaSeconds :type "Float (single-precision)"))
  (set `self.DeltaSec` DeltaSeconds)
  (if (`self.bStartDestroy`)
    (bind _output_get (set `self.MID_Opacity` (- (`self.MID_Opacity`) (* (`self.DeltaSec`) 0.25)))) ; 4秒で消える
    (`MaterialInstanceDynamic.SetScalarParameterValue` (`self.MID_DestMesh`) "Opacity Mask" _output_get) ; 透明度更新
    (if (<= (`self.MID_Opacity`) 0.0)
      (`self.K2_DestroyActor`))))

(event `self.Box_Origin.OnComponentBeginOverlap`
  (params (OverlappedComponent :type "PrimitiveComponent Object Reference") (OtherActor :type "Actor Object Reference") (OtherComp :type "PrimitiveComponent Object Reference") (OtherBodyIndex :type Integer) (bFromSweep :type Boolean) (SweepResult :type "HitResult Structure (by ref)"))
  (bind _actorisgolem (`self.CreateDestMesh` OtherActor))
  (if _actorisgolem
    (`KismetSystemLibrary.Delay` 5.0 :!label _label) ; 消滅処理
    (set `self.bStartDestroy` true)))

(event `self.Box_1.OnComponentBeginOverlap`
  (params (OverlappedComponent :type "PrimitiveComponent Object Reference") (OtherActor :type "Actor Object Reference") (OtherComp :type "PrimitiveComponent Object Reference") (OtherBodyIndex :type Integer) (bFromSweep :type Boolean) (SweepResult :type "HitResult Structure (by ref)"))
  (bind _actorisgolem (`self.CreateDestMesh` OtherActor))
  (if _actorisgolem
    (goto _label)))

(event `self.Box_2.OnComponentBeginOverlap`
  (params (OverlappedComponent :type "PrimitiveComponent Object Reference") (OtherActor :type "Actor Object Reference") (OtherComp :type "PrimitiveComponent Object Reference") (OtherBodyIndex :type Integer) (bFromSweep :type Boolean) (SweepResult :type "HitResult Structure (by ref)"))
  (bind _actorisgolem (`self.CreateDestMesh` OtherActor))
  (if _actorisgolem
    (goto _label)))

(event `self.Box_Origin.OnComponentHit`
  (params (HitComponent :type "PrimitiveComponent Object Reference") (OtherActor :type "Actor Object Reference") (OtherComp :type "PrimitiveComponent Object Reference") (NormalImpulse :type "Vector Structure") (Hit :type "HitResult Structure (by ref)"))
  (if (`self.ActorHasTag` "Player") :!label _label_2
    (bind _asbp_player (cast `/Game/Blueprints/Player/BP_Player` (`GameplayStatics.GetPlayerPawn` 0))) ; 演出中プレイヤーと重なる場合破棄
    (if (`/Game/Blueprints/Weapon/BP_Weapon.bSuckBoss` (`/Game/Blueprints/Player/BP_Player.GetWeapon` _asbp_player))
      (`self.K2_DestroyActor`))))

(event `self.Box_1.OnComponentHit`
  (params (HitComponent :type "PrimitiveComponent Object Reference") (OtherActor :type "Actor Object Reference") (OtherComp :type "PrimitiveComponent Object Reference") (NormalImpulse :type "Vector Structure") (Hit :type "HitResult Structure (by ref)"))
  (goto _label_2))

(event `self.Box_2.OnComponentHit`
  (params (HitComponent :type "PrimitiveComponent Object Reference") (OtherActor :type "Actor Object Reference") (OtherComp :type "PrimitiveComponent Object Reference") (NormalImpulse :type "Vector Structure") (Hit :type "HitResult Structure (by ref)"))
  (goto _label_2))

(fn `CreateDestMesh`
  (params (ActorRef :type "Actor Object Reference (by ref)"))
  (returns (ActorIsGolem :type Boolean))
  (bind _destpower (`self.DestPower`))
  (if (`self.ActorHasTag` ActorRef "Golem")
    (`ActorComponent.K2_DestroyComponent` (`self.StaticMesh`))
    (`self.DestroyBoxCollision`)
    (bind _returnvalue (`AddComponent|NODE_AddDestructibleComponent-0` :`RelativeTransform` (`KismetMathLibrary.MakeTransform` (0.0 0.0 -432.0)))) ; 破壊メッシュ置換
    (`DestructibleComponent.SetDestructibleMesh` _returnvalue (`self.DestMeshSlot`))
    (bind _returnvalue_2 (`PrimitiveComponent.CreateDynamicMaterialInstance` _returnvalue 0 (`PrimitiveComponent.GetMaterial` _returnvalue 0) "None"))
    (bind _output_get (set `self.MID_DestMesh` _returnvalue_2))
    (`MaterialInstanceDynamic.SetScalarParameterValue` _output_get "Opacity Mask" (`self.MID_Opacity`)) ; 透明度設定
    (`DestructibleComponent.ApplyDamage` _returnvalue _destpower (`KismetMathLibrary.MakeVector` (.x (`SceneComponent.K2_GetComponentLocation` _returnvalue)) (.y (`SceneComponent.K2_GetComponentLocation` _returnvalue)) (+ (.z (`SceneComponent.K2_GetComponentLocation` _returnvalue)) 82.0)) (`self.GetActorForwardVector` ActorRef) _destpower) ; ダメージ設定
    (for _index (range (`self.FX_SlotNum`))
      (`NiagaraFunctionLibrary.SpawnSystemAtLocation` (`|GetArrayItem` (`self.DestFX_Slot`) _index) (+ (`self.K2_GetActorLocation`) (`KismetMathLibrary.GreaterGreater_VectorRotator` (`|GetArrayItem` (`self.FX_SpawnPos`) _index) (`self.K2_GetActorRotation`)))))
    (`GameplayStatics.PlaySoundAtLocation` "/Game/Resource/SO/SE/Golem/Attack/SO_SE_Golem_Rock_Break_Cue.SO_SE_Golem_Rock_Break_Cue" (`self.K2_GetActorLocation`) (struct) 1.0 1.0 0.0 null null null)
    (return true)
    (else
      (return false))))

(fn `DestroyBoxCollision`
  (`ActorComponent.K2_DestroyComponent` (`self.Box_Origin`))
  (`ActorComponent.K2_DestroyComponent` (`self.Box_1`))
  (`ActorComponent.K2_DestroyComponent` (`self.Box_2`)))

(fn `UserConstructionScript`
  (bind _fx_slotnum (`self.FX_SlotNum`))
  (`KismetArrayLibrary.Array_Resize` (`self.DestFX_Slot`) _fx_slotnum) ; 破壊FX初期化
  (`KismetArrayLibrary.Array_Resize` (`self.FX_SpawnPos`) _fx_slotnum))