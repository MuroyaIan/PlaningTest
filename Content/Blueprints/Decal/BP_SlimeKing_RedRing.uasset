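; BP_SlimeKing_RedRing is a red ring decal Blueprint, named for the Slime King, that animates through a material.
; A timeline named Play starts on BeginPlay and drives the Opacity and Time scalar parameters on the MID from its Alpha and Time tracks.
; A PlayRing event also triggers the timeline, while Tick and the construction script only call the parent.
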(event `self.ReceiveBeginPlay`
  (`parent.ReceiveBeginPlay`)
  (bind (_direction _alpha _time) (`Timeline|Play` :!label _label)
    (:`Update`
      (`MaterialInstanceDynamic.SetScalarParameterValue` (`self.MID`) "Opacity" _alpha)
      (`MaterialInstanceDynamic.SetScalarParameterValue` (`self.MID`) "Time" _time))))

(event `self.ReceiveTick`
  (params (DeltaSeconds :type "Float (single-precision)"))
  (`parent.ReceiveTick` DeltaSeconds))

(event `PlayRing`
  (goto _label))

(fn `UserConstructionScript`
  (`parent.UserConstructionScript`))