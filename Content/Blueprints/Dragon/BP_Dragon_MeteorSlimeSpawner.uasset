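; Slime spawner for the dragon's meteor that periodically spawns small groups of BP_SlimeDefault around itself while enabled.
; It starts disabled; EnableSpawner toggles Tick, which prunes invalid slime references and runs the cooldown.
; SpawnSlime requires the player within range and a tracked count below the cap, then randomizes offset and size.
; External events snap it to an actor's XY at fixed height or flag all slimes to escape.
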(event `self.ReceiveBeginPlay`
  (`self.EnableSpawner` false))

(event `self.ReceiveTick`
  (params (DeltaSeconds :type "Float (single-precision)"))
  (`|ExecutionSequence`
    (:`then_0`
      (`self.CheckArray`))
    (:`then_1`
      (bind _output_get (set `self.SpawnCoolTimeRemain` (- (`self.SpawnCoolTimeRemain`) DeltaSeconds)))
      (if (<= _output_get 0.0)
        (set `self.SpawnCoolTimeRemain` 30.0)
        (`self.SpawnSlime`)
        (`self.SpawnSlime`)))))

(event `EnableSpawner`
  (params (Enable :type Boolean))
  (`self.SetActorTickEnabled` Enable)
  (if (not Enable)
    (set `self.SpawnCoolTimeRemain` 5.0)))

(event `KillAllSlime`
  (for _array_element (`self.SlimeRef`)
    (if (`KismetSystemLibrary.IsValid` _array_element)
      (set `/Game/Maps/TestMap/Nishino/Enemy_SlimeDefault/BP_SlimeDefault.EscapeFlg` true _array_element)))
  (`KismetArrayLibrary.Array_Clear` (`self.SlimeRef`)))

(event `SetLocation`
  (params (Actor :type "Actor Object Reference"))
  (`self.K2_SetActorLocation` (`KismetMathLibrary.MakeVector` (.x (`self.K2_GetActorLocation` Actor)) (.y (`self.K2_GetActorLocation` Actor)) 10.0)))

(fn `CheckArray`
  (for (_array_element _array_index) (`self.SlimeRef`)
    (if (not (`KismetSystemLibrary.IsValid` _array_element))
      (`KismetArrayLibrary.Array_Remove` (`self.SlimeRef`) _array_index))))

(fn `SpawnSlime`
  (if (<= (`KismetMathLibrary.Vector_Distance2D` (`self.K2_GetActorLocation` (`GameplayStatics.GetPlayerPawn` 0)) (`self.K2_GetActorLocation`)) (`self.SpawnLimitDistance`))
    (if (<= (`KismetArrayLibrary.Array_Length` (`self.SlimeRef`)) 8)
      (bind _returnvalue (`|SpawnActorFromClass` "/Game/Maps/TestMap/Nishino/Enemy_SlimeDefault/BP_SlimeDefault.BP_SlimeDefault_C" (`KismetMathLibrary.MakeTransform` (+ (`self.K2_GetActorLocation`) (`KismetMathLibrary.MakeVector` (* (`KismetMathLibrary.SelectFloat` -1.0 1.0 (`KismetMathLibrary.RandomBool`)) (`KismetMathLibrary.RandomFloatInRange` 0.0 250.0)) (* (`KismetMathLibrary.SelectFloat` -1.0 1.0 (`KismetMathLibrary.RandomBool`)) (`KismetMathLibrary.RandomFloatInRange` 0.0 250.0))))) "AdjustIfPossibleButAlwaysSpawn" "OverrideRootScale" null null))
      (`/Game/Maps/TestMap/Nishino/Enemy_SlimeDefault/BP_SlimeDefault.SetStatus` _returnvalue 10.0 0.46 0.1 (`KismetMathLibrary.RandomIntegerInRange` 3 5) 4000.0)
      (`Pawn.SpawnDefaultController` _returnvalue)
      (`KismetArrayLibrary.Array_Add` (`self.SlimeRef`) _returnvalue))))

(fn `UserConstructionScript`)