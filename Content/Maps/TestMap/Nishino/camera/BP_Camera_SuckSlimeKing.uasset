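; Camera actor that frames the Slime King while the player sucks it in for the boss kill.
; On BeginPlay it caches the BP_Player pawn, then each Tick waits until both BossSucked and KillBoss are true.
; While they are, it copies the boss's rotation and sits offset along the mesh's right vector, with a height that eases at constant speed toward a fixed value.
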(event `self.ReceiveBeginPlay`
  (bind _asbp_player (cast `/Game/Blueprints/Player/BP_Player` (`GameplayStatics.GetPlayerPawn` 0)))
  (set `self.PlayerReference` _asbp_player))

(event `self.ReceiveTick`
  (params (DeltaSeconds :type "Float (single-precision)"))
  (bind _slimekingreference (`self.SlimeKingReference`))
  (bind _playerreference (`self.PlayerReference`))
  (if (and (`/Game/Blueprints/Player/BP_Player.bBossSucked` _playerreference) (`/Game/Blueprints/Player/BP_Player.bKillBoss` _playerreference))
    (`self.K2_SetActorRotation` (`self.K2_GetActorRotation` _slimekingreference))
    (`self.K2_SetActorLocation` (+ (`self.K2_GetActorLocation` _slimekingreference) (* (`SceneComponent.GetRightVector` (`Character.Mesh` _slimekingreference)) -100.0) (`KismetMathLibrary.MakeVector` 0.0 0.0 (`self.Zheight`))))
    (set `self.Zheight` (`KismetMathLibrary.FInterpTo_Constant` (`self.Zheight`) 10.0 (`GameplayStatics.GetWorldDeltaSeconds`) 80.0))))

(fn `UserConstructionScript`)