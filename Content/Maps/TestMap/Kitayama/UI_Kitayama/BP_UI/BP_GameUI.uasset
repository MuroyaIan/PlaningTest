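; Game UI Blueprint that puts the game widget on screen at play start and controls the visibility of its flask gauge.
; It enables input from the player controller, then starts with the flask gauge removed.
; Pressing Weapon_Suck or Weapon_Fire shows the gauge and releasing either hides it, guarded by one shared display flag.
; A DispWidget toggle helper is defined but not called here.
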(event `self.ReceiveBeginPlay`
  (bind _widget_debugui (`self.GetWidget`))
  (bind _asbp_player_controller (cast `/Game/Blueprints/Player/BP_PlayerController` (`GameplayStatics.GetPlayerController` 0)))
  (`self.EnableInput` _asbp_player_controller) ; 入力有効化
  (`UserWidget.AddToViewport` _widget_debugui 0)
  (`Widget.RemoveFromParent` (`/Game/Maps/TestMap/Kitayama/UI_Kitayama/Widget_UI/GameWidget/UMG_GameUI.UMG_Flask` _widget_debugui)) ; 初期状態はフラスコゲージが消えているように
)

(event `InputAction|Weapon_Suck` :consume false
  (params (Key :type "Key Structure"))
  (:`Pressed`
    (if (not (`self.IsDispFlaskGauge`)) :!label _label
      (`UserWidget.AddToViewport` (`/Game/Maps/TestMap/Kitayama/UI_Kitayama/Widget_UI/GameWidget/UMG_GameUI.UMG_Flask` (`self.GetWidget`)) 0)
      (set `self.IsDispFlaskGauge` true)))
  (:`Released`
    (if (`self.IsDispFlaskGauge`) :!label _label_2
      (`Widget.RemoveFromParent` (`/Game/Maps/TestMap/Kitayama/UI_Kitayama/Widget_UI/GameWidget/UMG_GameUI.UMG_Flask` (`self.GetWidget`)))
      (set `self.IsDispFlaskGauge` false))))

(event `InputAction|Weapon_Fire` :consume false
  (params (Key :type "Key Structure"))
  (:`Pressed`
    (goto _label))
  (:`Released`
    (goto _label_2)))

(fn `DispWidget`
  (params (Widget :type "UserWidget Object Reference") (IsDisp :type Boolean))
  (returns (ReturnIsDisp :type Boolean))
  (if IsDisp
    (`Widget.RemoveFromParent` Widget) ; UIの非表示にする
    (else
      (`UserWidget.AddToViewport` Widget 0) ; UIを表示する
    ))
  (return (not IsDisp)))

(fn `GetWidget`
  (returns (Widget_DebugUI :type "/Game/Maps/TestMap/Kitayama/UI_Kitayama/Widget_UI/GameWidget/UMG_GameUI Object Reference"))
  (return (`|ConvertAsset` (`self.Widget_GameUI`))))

(fn `UserConstructionScript`)