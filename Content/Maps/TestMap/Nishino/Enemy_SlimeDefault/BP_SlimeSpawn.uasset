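; Slime spawner actor that keeps an array of BP_SlimeDefault enemies filled around its placement.
; Every Tick it scans the slots up to SlimeMaxSpawn and immediately respawns any invalid entry.
; Each new slime gets a default controller and the spawner's detection, health, damage and interval settings.
; MakeTransfrom supplies the spawn transform; its graph holds a random offset around the transform saved at BeginPlay.
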(event `self.ReceiveBeginPlay`
  ;[0.5 1 1] 変数の初期化
  (set `self.SpawnTransfrom` (`self.GetTransform`)))

(event `self.ReceiveTick`
  (params (DeltaSeconds :type "Float (single-precision)"))
  (`self.Chack_Spawn`))

(fn `Chack_Spawn`
  (bind _slimespawn (`self.SlimeSpawn`))
  (for _index (range (+ (`self.Slime_MaxSpawn`) 1))
    (if (not (`KismetSystemLibrary.IsValid` (`|GetArrayItem` _slimespawn _index)))
      (bind _spown_slime (`self.Spawn_SlimeDefault`))
      (`KismetArrayLibrary.Array_Set` _slimespawn _index _spown_slime true) ; 情報保存
    )))

(fn `Spawn_SlimeDefault`
  (returns (Spown_Slime :type "/Game/Maps/TestMap/Nishino/Enemy_SlimeDefault/BP_SlimeDefault Object Reference"))
  ;[1 0.5 1] BP_SlimeDedaultを作成する
  (bind _returnvalue (`|SpawnActorFromClass` "/Game/Maps/TestMap/Nishino/Enemy_SlimeDefault/BP_SlimeDefault.BP_SlimeDefault_C" (`self.MakeTransfrom`) "Undefined" "OverrideRootScale" null null))
  (if (`KismetSystemLibrary.IsValid` _returnvalue)
    (`Pawn.SpawnDefaultController` _returnvalue)
    ;[0.5 1 1] ステータスを設定する
    (set `/Game/Maps/TestMap/Nishino/Enemy_SlimeDefault/BP_SlimeDefault.Find_Distance` (`self.Find_Distance`) _returnvalue) ; 見つける距離
    (set `/Game/Maps/TestMap/Nishino/Enemy_SlimeDefault/BP_SlimeDefault.Miss_Distance` (`self.Miss_Distance`) _returnvalue) ; 見逃す距離
    (set `/Game/Maps/TestMap/Nishino/Enemy_SlimeDefault/BP_SlimeDefault.SlimeHitpoint` (`self.SlimeHitpoint`) _returnvalue) ; 体力
    (set `/Game/Maps/TestMap/Nishino/Enemy_SlimeDefault/BP_SlimeDefault.SlimeDamage` (`self.SlimeDamage`) _returnvalue) ; 受けるダメージ
    (set `/Game/Maps/TestMap/Nishino/Enemy_SlimeDefault/BP_SlimeDefault.Spawn_Interval` (`self.Spone_Interval`) _returnvalue) ; 生成頻度
    (return _returnvalue)
    (else
      (`KismetSystemLibrary.PrintString` "Spawn_Note!!!!!!!!!!!!") ; なんかうまく作成できていなかったことがあった、たまたま同じ座標とかでスポーンすると作成できないかも
      (return null))))

(fn `UserConstructionScript`)