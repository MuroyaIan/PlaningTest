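; Small-slime hit zone for the Slime King enemy that builds up a fill level as bullets hit it.
; Each overlap on its Hit capsule adds Damage to SlimePercent, clamped to one, and raises FullFlg once full.
; SetStatus assigns the group, index, damage increment and capsule rotation and size.
; GetScale returns the fill level as a uniform scale vector along with the stored index of the target to edit.
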(event `self.Hit.OnComponentBeginOverlap`
  (params (OverlappedComponent :type "PrimitiveComponent Object Reference") (OtherActor :type "Actor Object Reference") (OtherComp :type "PrimitiveComponent Object Reference") (OtherBodyIndex :type Integer) (bFromSweep :type Boolean) (SweepResult :type "HitResult Structure (by ref)"))
  ;[1 0 0] 弾が当たった時の処理
  (bind _output_get (set `self.SlimePercent` (`KismetMathLibrary.FClamp` (+ (`self.SlimePercent`) (`self.Damage`)))))
  (if (== _output_get 1.0)
    (set `self.FullFlg` true) ; 満タンのフラグ
  ))

(fn `GetScale`
  (returns (Scale :type "Vector Structure") (Index :type Integer))
  (return (`KismetMathLibrary.Conv_DoubleToVector` (`self.SlimePercent`)) (`self.Index`)))

(fn `Set Status`
  (params (Group :type Integer) (Index :type Integer) (Damage :type "Float (double-precision)" :default 0.1) (Rotate :type "Rotator Structure") (Hit_Height :type "Float (double-precision)" :default 100.0) (Hit_Radius :type "Float (double-precision)" :default 100.0))
  (bind _hit (`self.Hit`))
  (set `self.Group` Group) ; グループ設定
  (set `self.Index` Index) ; 編集先設定
  (set `self.Damage` Damage) ; ダメージ設定
  (`SceneComponent.K2_SetRelativeRotation` _hit Rotate false false) ; 角度
  (`CapsuleComponent.SetCapsuleHalfHeight` _hit Hit_Height true) ; 高さ
  (`CapsuleComponent.SetCapsuleRadius` _hit Hit_Radius true) ; 半径
)

(fn `UserConstructionScript`)