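; Prototype boar-style enemy that winds up and charges at the player, dealing contact damage only while charging.
; Entering the watch sphere raises walk speed and starts a timed wait, after which the player's position is saved as the charge target.
; Tick re-arms on nearing that point if ReChargeFlg is set, else ends the charge.
; State flags drive debug prints, material swaps and mesh spin; movement toward the target is not handled here.
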(event `self.ReCharge.OnComponentBeginOverlap`
  (params (OverlappedComponent :type "PrimitiveComponent Object Reference") (OtherActor :type "Actor Object Reference") (OtherComp :type "PrimitiveComponent Object Reference") (OtherBodyIndex :type Integer) (bFromSweep :type Boolean) (SweepResult :type "HitResult Structure (by ref)"))
  ;[1 0.7 1] 突撃範囲に入っているか確認
  (if (== OtherActor (`GameplayStatics.GetPlayerPawn` 0))
    (set `self.ReChargeFlg` true) ; とりあえず
  ))

(event `self.DamageBox.OnComponentBeginOverlap`
  (params (OverlappedComponent :type "PrimitiveComponent Object Reference") (OtherActor :type "Actor Object Reference") (OtherComp :type "PrimitiveComponent Object Reference") (OtherBodyIndex :type Integer) (bFromSweep :type Boolean) (SweepResult :type "HitResult Structure (by ref)"))
  ;[1 0 0.01801] ダメージ判定
  (if (`self.ChargerFlg`)
    (if (`self.WaitFlg`)
      _
      (elif (== OtherActor (`GameplayStatics.GetPlayerPawn` 0))
        (`GameplayStatics.ApplyDamage` null 10.0)
        (`KismetSystemLibrary.PrintString` "INOSISI_Damage!" true true (struct :`R` 1.0 :`B` 0.141862 :`A` 1.0))))))

(event `self.ReCharge.OnComponentEndOverlap`
  (params (OverlappedComponent :type "PrimitiveComponent Object Reference") (OtherActor :type "Actor Object Reference") (OtherComp :type "PrimitiveComponent Object Reference") (OtherBodyIndex :type Integer))
  ;[1 0.7 1] 突撃範囲に入っているか確認
  (if (== (`GameplayStatics.GetPlayerPawn` 0) OtherActor)
    (set `self.ReChargeFlg` false) ; とりあえず
  ))

(event `self.WachSphere.OnComponentBeginOverlap`
  (params (OverlappedComponent :type "PrimitiveComponent Object Reference") (OtherActor :type "Actor Object Reference") (OtherComp :type "PrimitiveComponent Object Reference") (OtherBodyIndex :type Integer) (bFromSweep :type Boolean) (SweepResult :type "HitResult Structure (by ref)"))
  ;[1 0.5 1] プレイヤーが近くにいた時に突っ込み準備
  (if (== OtherActor (`GameplayStatics.GetPlayerPawn` 0))
    (set `self.ReChargeFlg` true) ; とりあえず
    (if (not (`self.ChargerFlg`))
      (set `self.ChargerLocation` (`self.K2_GetActorLocation`)) ; 待機するため自身の座標を代入
      (set `CharacterMovementComponent.MaxWalkSpeed` (`self.Speed_Charger`) (`self.CharacterMovement`)) ; 突撃スピードに設定
      (`self.SetWaitTimer`) ; 待機時間の開始
    )))

(event `SetWaitTimer`
  ;[0.5 0.5 1] 待機時間の開始
  (set `self.WaitFlg` true)
  (set `self.ChargerFlg` true)
  (bind _returnvalue (`KismetSystemLibrary.K2_SetTimer` null "SetCharger" 2.0)))

(event `SetCharger`
  ;[0.5 0.5 1] 突撃開始
  (`KismetSystemLibrary.K2_ClearAndInvalidateTimerHandle` (stale `SetWaitTimer` _returnvalue))
  (set `self.WaitFlg` false)
  (set `self.ChargerLocation` (`self.K2_GetActorLocation` (`GameplayStatics.GetPlayerPawn` 0))) ; 待機するため自身の座標を代入
)

(event `self.ReceiveTick`
  (params (DeltaSeconds :type "Float (single-precision)"))
  (`self.TickCastData`) ; 情報の代入
  (`self.SetMaterial`) ; 色変えるだけ
  (`self.ChackLocation`) ; 距離で確認
  (`KismetSystemLibrary.PrintString` (`KismetStringLibrary.Conv_BoolToString` (`self.WaitFlg`)) true true (struct :`G` 0.66 :`B` 1.0 :`A` 1.0) 0.0)
  (`KismetSystemLibrary.PrintString` (`KismetStringLibrary.Conv_BoolToString` (`self.ChargerFlg`)) true true (struct :`G` 0.66 :`B` 1.0 :`A` 1.0) 0.0)
  (`KismetSystemLibrary.PrintString` (`KismetStringLibrary.Conv_BoolToString` (`self.ReChargeFlg`)) true true (struct :`G` 0.66 :`B` 1.0 :`A` 1.0) 0.0)
  (`KismetSystemLibrary.PrintString` "POS" true true (struct :`G` 0.66 :`B` 1.0 :`A` 1.0) 0.0)
  (`KismetSystemLibrary.PrintString` (`KismetStringLibrary.Conv_VectorToString` (`self.K2_GetActorLocation`)) true true (struct :`G` 0.66 :`B` 1.0 :`A` 1.0) 0.0)
  (`KismetSystemLibrary.PrintString` (`KismetStringLibrary.Conv_VectorToString` (`self.ChargerLocation`)) true true (struct :`G` 0.66 :`B` 1.0 :`A` 1.0) 0.0))

(event `ChackLocation`
  ;[0.5 0.5 1] 突進位置と現在の位置を確認　近ければ突進を終了する
  (if (`self.WaitFlg`)
    _
    (elif (== (`self.Vector_XY` (`self.K2_GetActorLocation`)) (`self.Vector_XY` (`self.ChargerLocation`)) :`ErrorTolerance` 50.0)
      (if (`self.ReChargeFlg`)
        (`self.SetWaitTimer`) ; 待機時間の開始
        (else
          (set `self.ChargerFlg` false) ; フラグ設定
          (set `self.ChargerLocation` (0.0 0.0 0.0)) ; 適当な処理、いつか直す
        )))))

(fn `SetMaterial`
  (bind _test_fbx_nisinoenemy (`self.TEST_FBX_NisinoEnemy`))
  (if (`self.ChargerFlg`)
    (if (`self.WaitFlg`)
      (`PrimitiveComponent.SetMaterial` _test_fbx_nisinoenemy 0 "/AnimationSharing/AnimSharingGreen.AnimSharingGreen")
      (else
        (`PrimitiveComponent.SetMaterial` _test_fbx_nisinoenemy 0 "/AnimationSharing/AnimSharingBlue.AnimSharingBlue")
        (`SceneComponent.K2_AddLocalRotation` _test_fbx_nisinoenemy (struct :`Pitch` 10.0) false false)))
    (else
      (`PrimitiveComponent.SetMaterial` _test_fbx_nisinoenemy 0 "/Game/Maps/TestMap/Nishino/Enemy_Puroto/M_NisinoEnemy.M_NisinoEnemy"))))

(fn `TickCastData`
  (set `self.PlayerPawn` (`GameplayStatics.GetPlayerPawn` 0)))

(fn `UserConstructionScript`)