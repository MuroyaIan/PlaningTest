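; BP_HouseWall01 is a breakable house wall actor that shatters when something overlaps its Box trigger.
; On overlap it destroys the static broken-wall mesh and the trigger, then adds a Destructible component at a fixed downward offset using DestMesh.
; It immediately applies heavy damage at the overlapping actor's location, with impulse along that actor's forward vector, so the pieces fly away from the impact.
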(event `self.Box.OnComponentBeginOverlap`
  (params (OverlappedComponent :type "PrimitiveComponent Object Reference") (OtherActor :type "Actor Object Reference") (OtherComp :type "PrimitiveComponent Object Reference") (OtherBodyIndex :type Integer) (bFromSweep :type Boolean) (SweepResult :type "HitResult Structure (by ref)"))
  (`ActorComponent.K2_DestroyComponent` (`self.EN_SM_HouseWallBroken_01`))
  (`ActorComponent.K2_DestroyComponent` (`self.Box`))
  (bind _returnvalue (`AddComponent|NODE_AddDestructibleComponent-0` :`RelativeTransform` (`KismetMathLibrary.MakeTransform` (`KismetMathLibrary.MakeVector` 0.0 0.0 -210.0))))
  (`DestructibleComponent.SetDestructibleMesh` _returnvalue (`self.DestMesh`))
  (`DestructibleComponent.ApplyDamage` _returnvalue 30000.0 (`self.K2_GetActorLocation` OtherActor) (`self.GetActorForwardVector` OtherActor) 30000.0))

(fn `UserConstructionScript`)