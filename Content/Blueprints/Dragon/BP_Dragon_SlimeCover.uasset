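; Dragon boss helper actor that follows a mesh socket with a collision sphere and tracks how slime-covered that spot becomes.
; Overlapping small slimes first raise wetness, then slime size, only while the dragon's form matches the one derived from the socket name.
; Tick eases both values toward their targets, pushing them to the dragon's material parameter and slime scale, and flags when size reaches the threshold.
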(event `self.ReceiveBeginPlay`
  (`SphereComponent.SetSphereRadius` (`self.BulletCollision`) (`self.SphereRadius`) true))

(event `self.ReceiveTick`
  (params (DeltaSeconds :type "Float (single-precision)"))
  (`self.UpdateTransform`)
  (`self.UpdateSlimeSize` DeltaSeconds)
  (`self.UpdateWetFx` DeltaSeconds)
  (`self.UpdateDebugDraw`))

(event `self.BulletCollision.OnComponentBeginOverlap`
  (params (OverlappedComponent :type "PrimitiveComponent Object Reference") (OtherActor :type "Actor Object Reference") (OtherComp :type "PrimitiveComponent Object Reference") (OtherBodyIndex :type Integer) (bFromSweep :type Boolean) (SweepResult :type "HitResult Structure (by ref)"))
  (if (not (`self.ReadyToSuck`))
    (cast `/Game/Blueprints/Slime/BP_Slime_Small` OtherActor)
    (bind _return_value (`self.IsEqualCurrentForm`))
    (if _return_value
      (if (>= (`self.CurrentWetValue`) 1.0)
        (set `self.TargetSlimeSize` (`KismetMathLibrary.FMin` (+ (`self.TargetSlimeSize`) 0.2) 1.0))
        (else
          (set `self.TargetWetValue` (+ (`self.TargetWetValue`) 0.5))
          (if (>= (`self.CurrentWetValue`) 1.0)
            (set `self.TargetSlimeSize` 0.6)))))))

(fn `IsEqualCurrentForm`
  (returns (`Return Value` :type Boolean))
  (return (== (`self.form`) (`/Game/Blueprints/Dragon/BP_Dragon.GetCurrentForm` (`self.DragonRef`)))))

(fn `SetInfomation`
  (params (SocketName :type Name) (DebugFlag :type Boolean) (SlimeThreshold :type "Float (double-precision)"))
  (bind _output_get (set `self.SocketName` SocketName))
  (set `self.SlimeThreashold` SlimeThreshold)
  (set `self.Debug` DebugFlag)
  (bind _returnvalue (`KismetStringLibrary.Conv_NameToString` _output_get))
  (if (`KismetStringLibrary.Contains` _returnvalue "A")
    (set `self.form` 1)
    (elif (`KismetStringLibrary.EqualEqual_StrStr` _returnvalue "JNT_SlimeB")
      (set `self.form` 3)
      (elif (`KismetStringLibrary.Contains` _returnvalue "B")
        (set `self.form` 2)
        (else
          (set `self.form` 0))))))

(fn `UpdateDebugDraw`
  (bind _bulletcollision (`self.BulletCollision`))
  (if (`self.Debug`)
    (switch `int` (`self.form`) ; 形態で分ける
      (:`1`
        (if (`/Game/Blueprints/Dragon/BP_Dragon.GetFlag` (`self.DragonRef`) "firstform")
          (`SceneComponent.SetHiddenInGame` _bulletcollision false false :!label _label)
          (else
            (`SceneComponent.SetHiddenInGame` _bulletcollision true false :!label _label_2))))
      (:`2`
        (if (`/Game/Blueprints/Dragon/BP_Dragon.GetFlag` (`self.DragonRef`) "secondform")
          (goto _label)
          (else
            (goto _label_2)))))))

(fn `UpdateSlimeSize`
  (params (DeltaSec :type "Float (double-precision)"))
  (if (not (`KismetMathLibrary.NearlyEqual_FloatFloat` (`self.CurrentSlimeSize`) (`self.TargetSlimeSize`) 0.01))
    (bind _output_get (set `self.CurrentSlimeSize` (`KismetMathLibrary.FInterpTo_Constant` (`self.CurrentSlimeSize`) (`self.TargetSlimeSize`) DeltaSec 1.0)))
    (set `self.ReadyToBig` (>= _output_get (`self.SlimeThreashold`)))
    (`/Game/Blueprints/Dragon/BP_Dragon.SetSlimeScale` (`self.DragonRef`) (`self.SlimeMapKey`) _output_get)))

(fn `UpdateTransform`
  (if (`KismetSystemLibrary.IsValid` (`self.DragonRef`))
    (`self.K2_SetActorLocation` (`SceneComponent.GetSocketLocation` (`Character.Mesh` (`self.DragonRef`)) (`self.SocketName`)))))

(fn `UpdateWetFx`
  (params (DeltaSec :type "Float (double-precision)"))
  (if (not (`KismetMathLibrary.NearlyEqual_FloatFloat` (`self.CurrentWetValue`) (`self.TargetWetValue`) 0.01))
    (set `self.CurrentWetValue` (`KismetMathLibrary.FInterpTo_Constant` (`self.CurrentWetValue`) (`self.TargetWetValue`) DeltaSec 1.0))
    (bind _return_value (`self.IsEqualCurrentForm`))
    (if _return_value
      (`/Game/Blueprints/Dragon/BP_Dragon.UpdateMaterialParameter` (`self.DragonRef`) (`self.SocketName`) (`self.CurrentWetValue`)))))

(fn `UserConstructionScript`)