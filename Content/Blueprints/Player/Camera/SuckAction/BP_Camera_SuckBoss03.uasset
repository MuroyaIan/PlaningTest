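; Cutscene camera actor for the player's boss-suck action, active while Start is set and the weapon's SuckBoss flag is on.
; Each tick it swings around the player, eases its gaze point from ahead onto the player, and narrows FOV to zoom in.
; After a delay it blends the view back to the player pawn and resets its state; the SlowMotion time-dilation routine is never called.
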(event `self.ReceiveBeginPlay`)

(event `self.ReceiveTick`
  (params (DeltaSeconds :type "Float (single-precision)"))
  (bind _campos (`self.CamPos`))
  (set `self.DeltaSec` DeltaSeconds)
  (if (`self.bStart`)
    (bind _asbp_player (cast `/Game/Blueprints/Player/BP_Player` (`GameplayStatics.GetPlayerPawn` 0)))
    (if (`/Game/Blueprints/Weapon/BP_Weapon.bSuckBoss` (`/Game/Blueprints/Player/BP_Player.GetWeapon` _asbp_player))
      (`|ExecutionSequence`
        (:`then_0`
          (`/Engine/EditorBlueprintResources/StandardMacros.DoOnce` false :!label _label
            (:`Completed`
              (bind _returnvalue (`self.GetActorForwardVector` _asbp_player))
              (bind _returnvalue_2 (* (`self.GetActorUpVector` _asbp_player) 30.0))
              (bind _returnvalue_3 (`self.K2_GetActorLocation` _asbp_player))
              (set `self.CamPos` (+ (`KismetMathLibrary.GreaterGreater_VectorRotator` (* _returnvalue 300.0) (`self.Rot`)) _returnvalue_2 _returnvalue_3)) ; 視点初期化
              (set `self.GazePoint` (+ (+ _returnvalue_2 _returnvalue_3) (* _returnvalue 800.0))) ; 注視点初期化
              (`|ExecutionSequence`
                (:`then_0`
                  (`KismetSystemLibrary.Delay` 4.5) ; カメラ切替
                  (`PlayerController.SetViewTargetWithBlend` (`GameplayStatics.GetPlayerController` 0) (`GameplayStatics.GetPlayerPawn` 0) 0.5 "VTBlend_Cubic" 0.0 false) ; メインカメラ切替
                  (set `self.bStart` false)
                  (set `self.Rot` (struct :`Yaw` 90.0))
                  (set `self.FOV` 150.0)
                  (goto _label :!via `Reset`))))))
        (:`then_1`
          (`|ExecutionSequence`
            (:`then_0`
              (`self.K2_SetActorLocation` _campos) ; カメラ更新
              (`self.K2_SetActorRotation` (`KismetMathLibrary.FindLookAtRotation` _campos (`self.GazePoint`)))
              (set `self.GazePoint` (`KismetMathLibrary.VInterpTo_Constant` (`self.GazePoint`) (+ (* (`self.GetActorUpVector` _asbp_player) 30.0) (`self.K2_GetActorLocation` _asbp_player)) (`self.DeltaSec`) 700.0)) ; 注視点更新
              (set `self.CamPos` (+ (`KismetMathLibrary.GreaterGreater_VectorRotator` (* (`self.GetActorForwardVector` _asbp_player) 300.0) (`self.Rot`)) (* (`self.GetActorUpVector` _asbp_player) 30.0) (`self.K2_GetActorLocation` _asbp_player))) ; 視点更新
              (set `self.Rot` (`KismetMathLibrary.MakeRotator` 0.0 0.0 (`KismetMathLibrary.FInterpTo_Constant` (.yaw (`self.Rot`)) 30.0 (`self.DeltaSec`) 35.0))) ; 回転角更新
            )
            (:`then_1`
              (bind _output_get (set `self.FOV` (`KismetMathLibrary.FInterpTo_Constant` (`self.FOV`) 70.0 (`self.DeltaSec`) 40.0)))
              (`CameraComponent.SetFieldOfView` (`self.CameraComponent`) _output_get) ; ズームイン
            )))))))

(fn `UserConstructionScript`)