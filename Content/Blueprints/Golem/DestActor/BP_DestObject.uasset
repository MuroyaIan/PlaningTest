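; BP_DestObject is a breakable prop that shatters when an actor tagged "Golem" overlaps its static mesh.
; The overlap destroys the static mesh and adds a destructible component using the configured fracture mesh.
; It then applies either directional point damage along the Golem's forward vector or radial damage, and destroys itself after a short delay.
; The construction script assigns the mesh and positions a DamageDraw sphere showing the damage origin and radius.
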(event `self.ReceiveBeginPlay`)

(event `self.StaticMesh.OnComponentBeginOverlap`
  (params (OverlappedComponent :type "PrimitiveComponent Object Reference") (OtherActor :type "Actor Object Reference") (OtherComp :type "PrimitiveComponent Object Reference") (OtherBodyIndex :type Integer) (bFromSweep :type Boolean) (SweepResult :type "HitResult Structure (by ref)"))
  (bind _destpower (`self.DestPower`))
  (bind _destpower_2 (`self.DestPower`))
  (if (`self.ActorHasTag` OtherActor "Golem")
    (`ActorComponent.K2_DestroyComponent` (`self.StaticMesh`))
    (bind _returnvalue (`AddComponent|NODE_AddDestructibleComponent-0`)) ; 破壊メッシュ置換
    (`DestructibleComponent.SetDestructibleMesh` _returnvalue (`self.DestMeshSlot`))
    (if (not (`self.bRadiusDamage`))
      (bind _returnvalue_2 (+ (`self.DestPos`) (`SceneComponent.K2_GetComponentLocation` _returnvalue)))
      (`DestructibleComponent.ApplyDamage` _returnvalue _destpower_2 _returnvalue_2 (`self.GetActorForwardVector` OtherActor) _destpower_2) ; ダメージ設定
      (else
        (`DestructibleComponent.ApplyRadiusDamage` _returnvalue _destpower _returnvalue_2 (`self.DamageRadius`) _destpower true)))
    (`KismetSystemLibrary.Delay` 5.0) ; 消滅処理
    (`self.K2_DestroyActor`)))

(fn `UserConstructionScript`
  (bind _damagedraw (`self.DamageDraw`))
  (`StaticMeshComponent.SetStaticMesh` (`self.StaticMesh`) (`self.StaticMeshSlot`)) ; SMをセット
  (`SceneComponent.K2_SetWorldLocation` _damagedraw (+ (`SceneComponent.K2_GetComponentLocation` (`self.StaticMesh`)) (`self.DestPos`)) false false)
  (`SphereComponent.SetSphereRadius` _damagedraw (`self.DamageRadius`) false))