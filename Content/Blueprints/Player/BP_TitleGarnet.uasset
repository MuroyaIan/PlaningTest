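; Title-screen Garnet actor that plays a timed, scripted run, suck and idle performance.
; BeginPlay creates dynamic materials for body, flask and pipe; Tick feeds the flask-bottom socket height to the liquid and glass materials.
; DoOnce-gated Tick calls delay-driven Turn1/Turn2 sequences that toggle forward movement and end in teleports.
; Turn1 hands off to Turn2, which re-arms itself despite its comment indicating a return to pattern A.
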(event `self.ReceiveBeginPlay`
  ;[1 1 1] マテリアル初期化
  (`self.InitBodyMID`)
  (`self.InitFlaskMID`)
  (`self.InitPipeMID`))

(event `self.ReceiveTick`
  (params (DeltaSeconds :type "Float (single-precision)"))
  (set `self.DeltaSec` DeltaSeconds)
  (`self.UpdateFlaskMID_BottomFlask`)
  (`|ExecutionSequence`
    (:`then_0`
      (if (`self.bTurn1`)
        (`/Engine/EditorBlueprintResources/StandardMacros.DoOnce` false :!label _label
          (:`Completed`
            (`KismetSystemLibrary.Delay` 14.0)
            (`SkeletalMeshComponent.PlayAnimation` (`self.Mesh_Garnet`) "/Game/Resource/CH/Garnet/Anim/CH_MO_GarnetRun.CH_MO_GarnetRun" true) ; 走り出す
            (set `self.bRun` true)
            (`KismetSystemLibrary.Delay` 1.0)
            (set `self.bRun` false)
            (`SkeletalMeshComponent.PlayAnimation` (`self.Mesh_Garnet`) "/Game/Resource/CH/Garnet/Anim/Title/BS1D_GarnetSuck.BS1D_GarnetSuck" true) ; 吸われ開始
            (`KismetSystemLibrary.Delay` 5.0)
            (`SkeletalMeshComponent.PlayAnimation` (`self.Mesh_Garnet`) "/Game/Resource/CH/Garnet/Anim/CH_MO_GarnetIdle.CH_MO_GarnetIdle" true) ; 待機開始
            (`KismetSystemLibrary.Delay` 2.0)
            (`SkeletalMeshComponent.PlayAnimation` (`self.Mesh_Garnet`) "/Game/Resource/CH/Garnet/Anim/CH_MO_GarnetRun.CH_MO_GarnetRun" true) ; 走り出す
            (set `self.bRun` true)
            (`KismetSystemLibrary.Delay` 2.0) ; パターンBへ移行
            (set `self.bRun` false)
            (set `self.bTurn1` false)
            (set `self.bTurn2` true)
            (`self.K2_SetActorRotation` (struct :`Yaw` 290.0))
            (`self.K2_SetActorLocation` (-1901.0 515.0 10.0))
            (goto _label :!via `Reset`)))))
    (:`then_1`
      (if (`self.bTurn2`)
        (`/Engine/EditorBlueprintResources/StandardMacros.DoOnce` false :!label _label_2
          (:`Completed`
            (`KismetSystemLibrary.Delay` 14.0)
            (`SkeletalMeshComponent.PlayAnimation` (`self.Mesh_Garnet`) "/Game/Resource/CH/Garnet/Anim/CH_MO_GarnetRun.CH_MO_GarnetRun" true) ; 走り出す
            (set `self.bRun` true)
            (`KismetSystemLibrary.Delay` 1.0)
            (set `self.bRun` false)
            (`SkeletalMeshComponent.PlayAnimation` (`self.Mesh_Garnet`) "/Game/Resource/CH/Garnet/Anim/Title/BS1D_GarnetSuck.BS1D_GarnetSuck" true) ; 吸われ開始
            (`KismetSystemLibrary.Delay` 5.0)
            (`SkeletalMeshComponent.PlayAnimation` (`self.Mesh_Garnet`) "/Game/Resource/CH/Garnet/Anim/CH_MO_GarnetIdle.CH_MO_GarnetIdle" true) ; 待機開始
            (`KismetSystemLibrary.Delay` 2.0)
            (`SkeletalMeshComponent.PlayAnimation` (`self.Mesh_Garnet`) "/Game/Resource/CH/Garnet/Anim/CH_MO_GarnetRun.CH_MO_GarnetRun" true) ; 走り出す
            (set `self.bRun` true)
            (`KismetSystemLibrary.Delay` 2.0) ; パターンAへ移行
            (set `self.bRun` false)
            (set `self.bTurn1` false)
            (set `self.bTurn2` true)
            (`self.K2_SetActorRotation` (struct :`Yaw` 110.0))
            (`self.K2_SetActorLocation` (-1469.0 -693.0 10.0))
            (goto _label_2 :!via `Reset`)))))
    (:`then_2`
      (if (`self.bRun`)
        (`self.K2_SetActorLocation` (+ (`self.K2_GetActorLocation`) (* (`self.GetActorForwardVector`) (* (`self.DeltaSec`) 450.0))))))))

(fn `InitBodyMID`
  (bind _mesh_garnet (`self.Mesh_Garnet`))
  (bind _returnvalue (`PrimitiveComponent.CreateDynamicMaterialInstance` _mesh_garnet 0 (`PrimitiveComponent.GetMaterial` _mesh_garnet 0) "None")) ; 本体用MID
  (bind _output_get (set `self.MID_Body` _returnvalue))
  (`MaterialInstanceDynamic.SetScalarParameterValue` _output_get "Face" 0.0) ; 表情初期化
  (`MaterialInstanceDynamic.SetScalarParameterValue` _output_get "MaskMode" 2.0) ; プレイヤー隠し機能初期化
)

(fn `InitFlaskMID`
  (bind _mesh_garnet (`self.Mesh_Garnet`))
  (`|ExecutionSequence`
    (:`then_0`
      (bind _returnvalue (`PrimitiveComponent.CreateDynamicMaterialInstance` _mesh_garnet 2 (`PrimitiveComponent.GetMaterial` _mesh_garnet 2) "None")) ; フラスコ容量表示MID
      (bind _output_get (set `self.MID_Flask` _returnvalue))
      (`MaterialInstanceDynamic.SetScalarParameterValue` _output_get "TankCapacity" 0.0) ; フラスコ容量初期化
      (`MaterialInstanceDynamic.SetScalarParameterValue` _output_get "BottomFlask" (`self.FlaskRefPos`)) ; フラスコ参照位置更新
      (`MaterialInstanceDynamic.SetScalarParameterValue` _output_get "WaveStrength" 0.5) ; フラスコ揺れ具合更新
      (`MaterialInstanceDynamic.SetScalarParameterValue` _output_get "MaskMode" 1.0) ; プレイヤー隠し機能初期化
    )
    (:`then_1`
      (`|ExecutionSequence`
        (:`then_0`
          (bind _returnvalue_2 (`PrimitiveComponent.CreateDynamicMaterialInstance` _mesh_garnet 4 (`PrimitiveComponent.GetMaterial` _mesh_garnet 4) "None")) ; フラスコガラス用MID
          (bind _output_get_2 (set `self.MID_FlaskGlass` _returnvalue_2))
          (`MaterialInstanceDynamic.SetScalarParameterValue` _output_get_2 "TankCapacity" 0.0) ; フラスコ容量初期化
          (`MaterialInstanceDynamic.SetScalarParameterValue` _output_get_2 "BottomFlask" (`self.FlaskRefPos`)) ; フラスコ参照位置更新
          (`MaterialInstanceDynamic.SetScalarParameterValue` _output_get_2 "WaveStrength" 0.5) ; フラスコ揺れ具合更新
          (`MaterialInstanceDynamic.SetScalarParameterValue` _output_get_2 "MaskMode" 1.0) ; プレイヤー隠し機能初期化
        )
        (:`then_1`
          (bind _returnvalue_3 (`PrimitiveComponent.CreateDynamicMaterialInstance` _mesh_garnet 1 (`PrimitiveComponent.GetMaterial` _mesh_garnet 1) "None")) ; フラスコガラス（外側）用MID
          (bind _output_get_3 (set `self.MID_FlaskGlassOut` _returnvalue_3))
          (`MaterialInstanceDynamic.SetScalarParameterValue` _output_get_3 "MaskMode" 1.0) ; プレイヤー隠し機能初期化
        )))))

(fn `InitPipeMID`
  (bind _mesh_garnet (`self.Mesh_Garnet`))
  (bind _returnvalue (`PrimitiveComponent.CreateDynamicMaterialInstance` _mesh_garnet 3 (`PrimitiveComponent.GetMaterial` _mesh_garnet 3) "None")) ; パイプ用MID
  (bind _output_get (set `self.MID_Pipe` _returnvalue))
  (`MaterialInstanceDynamic.SetScalarParameterValue` _output_get "MaskMode" 1.0) ; プレイヤー隠し機能初期化
  (`self.UpdatePipeMID` false))

(fn `UpdateFlaskMID_BottomFlask`
  (bind _output_get (set `self.FlaskRefPos` (- (* (.z (`SceneComponent.GetSocketLocation` (`self.Mesh_Garnet`) "JNT_flaskbottom_C0")) 1.0) 150.0)))
  (`MaterialInstanceDynamic.SetScalarParameterValue` (`self.MID_Flask`) "BottomFlask" _output_get) ; フラスコ参照位置更新
  (`MaterialInstanceDynamic.SetScalarParameterValue` (`self.MID_FlaskGlass`) "BottomFlask" _output_get) ; フラスコ参照位置更新
)

(fn `UpdatePipeMID`
  (params (UsePipe :type Boolean) (SuckMode :type Boolean))
  (bind _mid_pipe (`self.MID_Pipe`))
  (bind _mid_pipe_2 (`self.MID_Pipe`))
  (if UsePipe
    (`MaterialInstanceDynamic.SetScalarParameterValue` _mid_pipe_2 "PipeFlow" 0.0)
    (if SuckMode
      (`MaterialInstanceDynamic.SetScalarParameterValue` _mid_pipe "Reverse" 1.0)
      (else
        (`MaterialInstanceDynamic.SetScalarParameterValue` _mid_pipe "Reverse" 0.0)))
    (else
      (`MaterialInstanceDynamic.SetScalarParameterValue` _mid_pipe_2 "PipeFlow" 1.0))))

(fn `UserConstructionScript`)