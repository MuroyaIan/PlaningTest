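; Sign actor that shows a paged hint screen for stages 1-3 or the Stage 1 controls tutorial, selected by StageNum.
; BeginPlay enables input, creates the matching widget and creates, but does not display, a button prompt widget.
; Confirm opens the screen and Back closes it, with sound and animation-busy checks.
; Left/Right turn pages, as does the stick past a threshold through 0.5-second Delays that throttle repeats.
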(event `self.ReceiveBeginPlay`
  (bind _asbp_player_controller (cast `/Game/Blueprints/Player/BP_PlayerController` (`GameplayStatics.GetPlayerController` 0)))
  (`self.EnableInput` _asbp_player_controller) ; 入力有効化
  (`self.Init`)
  (bind _returnvalue (`|CreateWidget` "/Game/Maps/TestMap/Kitayama/UI_Kitayama/Widget_UI/TutorialWidget/UMG_SingButton.UMG_SingButton_C")) ; ふよふよ浮かぶボタンUI
  (set `self.ButtonUI` _returnvalue))

(event `self.ReceiveTick`
  (params (DeltaSeconds :type "Float (single-precision)")))

(event `InputAction|UI_Confirm` :consume false
  (params (Key :type "Key Structure"))
  (:`Pressed`
    (`self.UMGAdd Toview`)))

(event `InputAction|UI_Back` :consume false
  (params (Key :type "Key Structure"))
  (:`Pressed`
    (if (`self.bIsDisp`)
      (switch `int` (- (`self.StageNum`) 1)
        (:`0`
          (bind _isplaying (`/Game/Maps/TestMap/Kitayama/UI_Kitayama/Widget_UI/TutorialWidget/UMG_SignStage1.IsPlayingAnimCheck` (`self.Stage1`)))
          (if (not _isplaying)
            (`/Game/Maps/TestMap/Kitayama/UI_Kitayama/Widget_UI/TutorialWidget/UMG_SignStage1.PlayUnDisp` (`self.Stage1`))
            (set `self.bIsDisp` false :!label _label)
            (`GameplayStatics.PlaySound2D` "/Game/Resource/SO/SE/UI/UI/SO_SE_UI_Back_Cue.SO_SE_UI_Back_Cue" 1.0 1.0 0.0 null null) ; 効果音再生
          ))
        (:`1`
          (bind _isplaying_2 (`/Game/Maps/TestMap/Kitayama/UI_Kitayama/Widget_UI/TutorialWidget/UMG_SignStage2.IsPlayingAnimCheck` (`self.Stage2`)))
          (if (not _isplaying_2)
            (`/Game/Maps/TestMap/Kitayama/UI_Kitayama/Widget_UI/TutorialWidget/UMG_SignStage2.PlayUnDisp` (`self.Stage2`))
            (goto _label)))
        (:`2`
          (bind _isplaying_3 (`/Game/Maps/TestMap/Kitayama/UI_Kitayama/Widget_UI/TutorialWidget/UMG_SignStage3.IsPlayingAnimCheck` (`self.Stage3`)))
          (if (not _isplaying_3)
            (`/Game/Maps/TestMap/Kitayama/UI_Kitayama/Widget_UI/TutorialWidget/UMG_SignStage3.PlayUnDisp` (`self.Stage3`))
            (goto _label)))
        (:`3`
          (bind _isplaying_4 (`/Game/Maps/TestMap/Kitayama/UI_Kitayama/Widget_UI/TutorialWidget/UMG_SignStage1_Tutorial.IsPlayingAnimCheck` (`self.Tutorial`)))
          (if (not _isplaying_4)
            (`/Game/Maps/TestMap/Kitayama/UI_Kitayama/Widget_UI/TutorialWidget/UMG_SignStage1_Tutorial.PlayUnDisp` (`self.Tutorial`))
            (goto _label)))))))

(event `InputAction|UI_Right` :consume false
  (params (Key :type "Key Structure"))
  (:`Pressed`
    (if (`self.bIsDisp`)
      (switch `int` (- (`self.StageNum`) 1)
        (:`0`
          (`/Game/Maps/TestMap/Kitayama/UI_Kitayama/Widget_UI/TutorialWidget/UMG_SignStage1.ChangePage` (`self.Stage1`) true))
        (:`1`
          (`/Game/Maps/TestMap/Kitayama/UI_Kitayama/Widget_UI/TutorialWidget/UMG_SignStage2.ChangePage` (`self.Stage2`) true))
        (:`2`
          (`/Game/Maps/TestMap/Kitayama/UI_Kitayama/Widget_UI/TutorialWidget/UMG_SignStage3.ChangePage` (`self.Stage3`) true))
        (:`3`
          (`/Game/Maps/TestMap/Kitayama/UI_Kitayama/Widget_UI/TutorialWidget/UMG_SignStage1_Tutorial.ChangePage` (`self.Tutorial`) true))))))

(event `InputAxis|UI_Stick_X` :consume false
  (params (AxisValue :type "Float (single-precision)"))
  (if (> AxisValue (`self.StickX`))
    (`KismetSystemLibrary.Delay` 0.5)
    (if (`self.bIsDisp`)
      (switch `int` (- (`self.StageNum`) 1)
        (:`0`
          (`/Game/Maps/TestMap/Kitayama/UI_Kitayama/Widget_UI/TutorialWidget/UMG_SignStage1.ChangePage` (`self.Stage1`) true))
        (:`1`
          (`/Game/Maps/TestMap/Kitayama/UI_Kitayama/Widget_UI/TutorialWidget/UMG_SignStage2.ChangePage` (`self.Stage2`) true))
        (:`2`
          (`/Game/Maps/TestMap/Kitayama/UI_Kitayama/Widget_UI/TutorialWidget/UMG_SignStage3.ChangePage` (`self.Stage3`) true))
        (:`3`
          (`/Game/Maps/TestMap/Kitayama/UI_Kitayama/Widget_UI/TutorialWidget/UMG_SignStage1_Tutorial.ChangePage` (`self.Tutorial`) true))))
    (elif (< AxisValue (* (`self.StickX`) -1.0))
      (`KismetSystemLibrary.Delay` 0.5)
      (if (`self.bIsDisp`)
        (switch `int` (- (`self.StageNum`) 1)
          (:`0`
            (`/Game/Maps/TestMap/Kitayama/UI_Kitayama/Widget_UI/TutorialWidget/UMG_SignStage1.ChangePage` (`self.Stage1`) false))
          (:`1`
            (`/Game/Maps/TestMap/Kitayama/UI_Kitayama/Widget_UI/TutorialWidget/UMG_SignStage2.ChangePage` (`self.Stage2`) false))
          (:`2`
            (`/Game/Maps/TestMap/Kitayama/UI_Kitayama/Widget_UI/TutorialWidget/UMG_SignStage3.ChangePage` (`self.Stage3`) false))
          (:`3`
            (`/Game/Maps/TestMap/Kitayama/UI_Kitayama/Widget_UI/TutorialWidget/UMG_SignStage1_Tutorial.ChangePage` (`self.Tutorial`) false)))))))

(event `InputAction|UI_Left` :consume false
  (params (Key :type "Key Structure"))
  (:`Pressed`
    (if (`self.bIsDisp`)
      (switch `int` (- (`self.StageNum`) 1)
        (:`0`
          (`/Game/Maps/TestMap/Kitayama/UI_Kitayama/Widget_UI/TutorialWidget/UMG_SignStage1.ChangePage` (`self.Stage1`) false))
        (:`1`
          (`/Game/Maps/TestMap/Kitayama/UI_Kitayama/Widget_UI/TutorialWidget/UMG_SignStage2.ChangePage` (`self.Stage2`) false))
        (:`2`
          (`/Game/Maps/TestMap/Kitayama/UI_Kitayama/Widget_UI/TutorialWidget/UMG_SignStage3.ChangePage` (`self.Stage3`) false))
        (:`3`
          (`/Game/Maps/TestMap/Kitayama/UI_Kitayama/Widget_UI/TutorialWidget/UMG_SignStage1_Tutorial.ChangePage` (`self.Tutorial`) false))))))

(fn `Init`
  (switch `int` (- (`self.StageNum`) 1)
    (:`0`
      (bind _returnvalue (`|CreateWidget` "/Game/Maps/TestMap/Kitayama/UI_Kitayama/Widget_UI/TutorialWidget/UMG_SignStage1.UMG_SignStage1_C")) ; Stage1のヒントUI
      (set `self.Stage1` _returnvalue))
    (:`1`
      (bind _returnvalue_2 (`|CreateWidget` "/Game/Maps/TestMap/Kitayama/UI_Kitayama/Widget_UI/TutorialWidget/UMG_SignStage2.UMG_SignStage2_C")) ; Stage2のヒントUI
      (set `self.Stage2` _returnvalue_2))
    (:`2`
      (bind _returnvalue_3 (`|CreateWidget` "/Game/Maps/TestMap/Kitayama/UI_Kitayama/Widget_UI/TutorialWidget/UMG_SignStage3.UMG_SignStage3_C")) ; Stage3のヒントUI
      (set `self.Stage3` _returnvalue_3))
    (:`3`
      (bind _returnvalue_4 (`|CreateWidget` "/Game/Maps/TestMap/Kitayama/UI_Kitayama/Widget_UI/TutorialWidget/UMG_SignStage1_Tutorial.UMG_SignStage1_Tutorial_C")) ; Stage1の操作方法UI
      (set `self.Tutorial` _returnvalue_4))))

(fn `UMGAdd Toview`
  (if (not (`self.bIsDisp`))
    (switch `int` (- (`self.StageNum`) 1)
      (:`0`
        (if (not (`Widget.IsInViewport` (`self.Stage1`)))
          (bind _isplaying (`/Game/Maps/TestMap/Kitayama/UI_Kitayama/Widget_UI/TutorialWidget/UMG_SignStage1.IsPlayingAnimCheck` (`self.Stage1`)))
          (if (not _isplaying)
            (`UserWidget.AddToViewport` (`self.Stage1`) 0)
            (set `self.bIsDisp` true :!label _label)
            (`GameplayStatics.PlaySound2D` "/Game/Resource/SO/SE/UI/Pause/SO_SE_Pause_Start_Cue.SO_SE_Pause_Start_Cue" 1.0 1.0 0.0 null null) ; 効果音再生
          )))
      (:`1`
        (if (not (`Widget.IsInViewport` (`self.Stage2`)))
          (bind _isplaying_2 (`/Game/Maps/TestMap/Kitayama/UI_Kitayama/Widget_UI/TutorialWidget/UMG_SignStage2.IsPlayingAnimCheck` (`self.Stage2`)))
          (if (not _isplaying_2)
            (`UserWidget.AddToViewport` (`self.Stage2`) 0)
            (goto _label))))
      (:`2`
        (if (not (`Widget.IsInViewport` (`self.Stage3`)))
          (bind _isplaying_3 (`/Game/Maps/TestMap/Kitayama/UI_Kitayama/Widget_UI/TutorialWidget/UMG_SignStage3.IsPlayingAnimCheck` (`self.Stage3`)))
          (if (not _isplaying_3)
            (`UserWidget.AddToViewport` (`self.Stage3`) 0)
            (goto _label))))
      (:`3`
        (if (not (`Widget.IsInViewport` (`self.Tutorial`)))
          (bind _isplaying_4 (`/Game/Maps/TestMap/Kitayama/UI_Kitayama/Widget_UI/TutorialWidget/UMG_SignStage1_Tutorial.IsPlayingAnimCheck` (`self.Tutorial`)))
          (if (not _isplaying_4)
            (`UserWidget.AddToViewport` (`self.Tutorial`) 0)
            (goto _label)))))))

(fn `UserConstructionScript`)