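; Player controller for BP_Player, handling camera-relative movement, camera look, suck/fire weapon input and saving on quit.
; Tick rotates the pawn, locking it to camera yaw while aiming or easing it toward stick direction otherwise, then applies movement, slowed when aiming.
; Look input is scaled by separate normal and aim sensitivity levels, while being hurt blocks movement and weapon starts.
; Includes debug keys and an on-screen pad readout.
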(event `self.ReceiveBeginPlay`)

(event `self.ReceiveTick`
  (params (DeltaSeconds :type "Float (single-precision)"))
  (`self.SetRotation`)
  (`self.UpdateMovement`)
  (`self.PrintPadInfo`))

(event `InputAxis|LookRight`
  (params (AxisValue :type "Float (single-precision)"))
  ;[1 1 1] カメラ回転
  (bind _output_get (set `self.ValueAxisRX` AxisValue))
  (`self.UpdateSensitivity` _output_get true) ; 感度更新
  (`/Game/Blueprints/Player/BP_PlayerCameraManager.AddYawInput` (`self.GetCameraManager`) _output_get))

(event `InputAxis|LookUp`
  (params (AxisValue :type "Float (single-precision)"))
  ;[1 1 1] カメラ回転
  (bind _output_get (set `self.ValueAxisRY` AxisValue))
  (`self.UpdateSensitivity` _output_get)
  (`/Game/Blueprints/Player/BP_PlayerCameraManager.AddPitchInput` (`self.GetCameraManager`) _output_get))

(event `InputAxis|MoveForward`
  (params (AxisValue :type "Float (single-precision)"))
  ;[0.5 1 1] キャラクター移動
  (bind _bhurt (`self.CheckIfNotHurt`))
  (if _bhurt
    (if (`KismetMathLibrary.NearlyEqual_FloatFloat` AxisValue 0.0 (`self.InputTolerance`))
      (set `self.ValueAxisLY` 0.0 :!label _label)
      (else
        (set `self.ValueAxisLY` AxisValue)))
    (else
      (goto _label))))

(event `InputAxis|MoveRight`
  (params (AxisValue :type "Float (single-precision)"))
  ;[0.5 1 1] キャラクター移動
  (bind _bhurt (`self.CheckIfNotHurt`))
  (if _bhurt
    (if (`KismetMathLibrary.NearlyEqual_FloatFloat` AxisValue 0.0 (`self.InputTolerance`))
      (set `self.ValueAxisLX` 0.0 :!label _label_2)
      (else
        (set `self.ValueAxisLX` AxisValue)))
    (else
      (goto _label_2))))

(event `UpdateMovement`
  ;[0.5 1 1] キャラクター移動
  (bind _revspeed (`self.UpdateMoveSpeed`)) ; 速度更新
  (bind _rotation (`/Game/Blueprints/Player/BP_PlayerCameraManager.GetCameraRotationEx` (`self.GetCameraManager`) false false true)) ; カメラの向き取得
  (`Pawn.AddMovementInput` (`self.GetPlayerPawn`) (`KismetMathLibrary.GreaterGreater_VectorRotator` (`/Game/Blueprints/BP_FuncLibrary.Vector to 2D(NormalizeXY)` (`KismetMathLibrary.MakeVector` (`self.ValueAxisLY`) (`self.ValueAxisLX`))) _rotation) _revspeed false))

(event `AimOn`
  ;[1 0.5 0.7544] 照準&武器使用
  (set `self.AimMode` true)
  (`/Game/Blueprints/Player/BP_Player.UpdateFlaskMID_WaveStrength` (`self.GetPlayerPawn`) true))

(event `AimOff`
  (bind _playerpawn (`self.GetPlayerPawn`))
  ;[1 0.5 0.7544] 照準&武器使用
  (set `self.AimMode` false)
  (if (<= (`KismetMathLibrary.VSize` (`self.GetVelocity` _playerpawn)) 0.0)
    (`/Game/Blueprints/Player/BP_Player.UpdateFlaskMID_WaveStrength` _playerpawn false)))

(event `InputAction|Weapon_Suck` :consume false
  (params (Key :type "Key Structure"))
  ;[1 0.5 0.7544] 照準&武器使用
  (:`Pressed`
    (set `self.bHold_Suck` true)
    (bind _bhurt (`self.CheckIfNotHurt`))
    (if _bhurt
      (`self.SuckOn`)))
  (:`Released`
    (set `self.bHold_Suck` false)
    (`self.SuckOff`)))

(event `CheckWeapon`
  ;[1 0.5 0.7544] 照準&武器使用
  (if (`self.bHold_Suck`)
    (`self.SuckOn`)
    (elif (`self.bHold_Fire`)
      (`self.FireOn`))))

(event `InputAction|Weapon_Fire` :consume false
  (params (Key :type "Key Structure"))
  ;[1 0.5 0.7544] 照準&武器使用
  (:`Pressed`
    (set `self.bHold_Fire` true)
    (bind _bhurt (`self.CheckIfNotHurt`))
    (if _bhurt
      (`self.FireOn`)))
  (:`Released`
    (set `self.bHold_Fire` false)
    (`self.FireOff`)))

(event `InputAction|DebugLog_Print`
  (params (Key :type "Key Structure"))
  ;[1 1 1] デバッグログ出力
  (:`Pressed`
    (bind _asbp_global_data (cast `/Game/Blueprints/System/BP_GlobalData` (`GameplayStatics.GetGameInstance`)))
    (set `/Game/Blueprints/System/BP_GlobalData.bDebugLog` (not (`/Game/Blueprints/System/BP_GlobalData.bDebugLog` _asbp_global_data)) _asbp_global_data) ; 出力切替
  ))

(event `InputAction|QuitGame`
  (params (Key :type "Key Structure"))
  ;[1 1 1] ゲーム終了
  (:`Pressed`
    (bind _asbp_game_mode (cast `/Game/Blueprints/System/BP_GameMode` (`GameplayStatics.GetGameMode`)))
    (`/Game/Blueprints/System/BP_GameMode.SaveGame` _asbp_game_mode) ; 保存＆ゲーム終了
  ))

(event `Key|R`
  (params (Key :type "Key Structure"))
  (:`Pressed`
    (bind _asbp_global_data (cast `/Game/Blueprints/System/BP_GlobalData` (`GameplayStatics.GetGameInstance`)))
    (bind _output_get (set `/Game/Blueprints/System/BP_GlobalData.TestVal` (+ (`/Game/Blueprints/System/BP_GlobalData.TestVal` _asbp_global_data) 1) _asbp_global_data))
    (`KismetSystemLibrary.PrintString` (`KismetStringLibrary.Concat_StrStr` "TestVal:" (`KismetStringLibrary.Conv_IntToString` _output_get)))))

(event `Key|T`
  (params (Key :type "Key Structure"))
  (:`Pressed`
    (bind _asbp_game_mode (cast `/Game/Blueprints/System/BP_GameMode` (`GameplayStatics.GetGameMode`)))
    (`AudioComponent.Play` (`/Game/Blueprints/System/BP_GameMode.BGM_Player` _asbp_game_mode) 0.0)))

(event `Key|F`
  (params (Key :type "Key Structure"))
  (:`Pressed`
    (`GameplayStatics.ApplyDamage` (`self.GetPlayerPawn`) 1.0 null null "/Script/Engine.DamageType")))

(event `Key|R`
  (params (Key :type "Key Structure"))
  (:`Pressed`
    (`GameplayStatics.ApplyDamage` (`self.GetPlayerPawn`) 2.0 null null "/Script/Engine.DamageType")))

(fn `CalcSensitivity`
  (params (SensitivityLevel :type Integer) (InputValue :type "Float (double-precision) (by ref)"))
  (returns (OutputValue :type "Float (double-precision)"))
  (bind _returnvalue (- SensitivityLevel 5))
  (if (>= _returnvalue 0)
    (return (+ (* (* _returnvalue 0.4) InputValue) InputValue))
    (else
      (return (+ (* (* _returnvalue 0.1) InputValue) InputValue)))))

(fn `CheckIfNotHurt`
  (returns (bHurt :type Boolean))
  (return (not (`/Game/Blueprints/Player/BP_Player.bHurt` (`self.GetPlayerPawn`)))))

(fn `GetCameraManager`
  (returns (CameraManager :type "/Game/Blueprints/Player/BP_PlayerCameraManager Object Reference"))
  (bind _asbp_player_camera_manager (cast `/Game/Blueprints/Player/BP_PlayerCameraManager` (`self.PlayerCameraManager`)))
  (return _asbp_player_camera_manager))

(fn `GetPlayerPawn`
  (returns (PlayerPawn :type "/Game/Blueprints/Player/BP_Player Object Reference"))
  (bind _asbp_player (cast `/Game/Blueprints/Player/BP_Player` (`self.K2_GetPawn`)))
  (return _asbp_player))

(fn `PrintPadInfo`
  (bind _bdebug (`/Game/Blueprints/BP_FuncLibrary.CheckDebugPrint`))
  (if _bdebug
    (`KismetSystemLibrary.PrintString` (`KismetStringLibrary.Concat_StrStr` "[PadInfo]" " \nStickLX:" (`KismetTextLibrary.Conv_TextToString` (`KismetTextLibrary.Conv_DoubleToText` (`self.ValueAxisLX`) "HalfFromZero" false false 1 1 1 1)) " \nStickLY:" (`KismetTextLibrary.Conv_TextToString` (`KismetTextLibrary.Conv_DoubleToText` (`self.ValueAxisLY`) "HalfFromZero" false false 1 1 1 1)) " \nStickRX:" (`KismetTextLibrary.Conv_TextToString` (`KismetTextLibrary.Conv_DoubleToText` (`self.ValueAxisRX`) "HalfFromZero" false false 1 1 1 1)) " \nStickRY:" (`KismetTextLibrary.Conv_TextToString` (`KismetTextLibrary.Conv_DoubleToText` (`self.ValueAxisRY`) "HalfFromZero" false false 1 1 1 1)) " \nSuck:" (`KismetStringLibrary.Conv_BoolToString` (`self.bHold_Suck`)) " \nFire:" (`KismetStringLibrary.Conv_BoolToString` (`self.bHold_Fire`))) true false (struct :`G` 1.0 :`B` 0.087113 :`A` 1.0) 0.0)))

(fn `SetRotation`
  (if (`self.AimMode`)
    (bind _rotation (`/Game/Blueprints/Player/BP_PlayerCameraManager.GetCameraRotationEx` (`self.GetCameraManager`) false false true)) ; カメラ正面の向き（Z軸回転取得）
    (bind _output_get (set `self.Rotation` _rotation)) ; 回転情報を同期
    (bind _output_get_2 (set `self.TargetRotation` _output_get))
    (`self.K2_SetActorRotation` (`self.GetPlayerPawn`) _output_get_2 false) ; 常にカメラと同じ向き
    (else
      (if (not (and (== (`self.ValueAxisLY`) 0.0) (== (`self.ValueAxisLX`) 0.0)))
        (`self.SetTargetRotation`))
      (bind _output_get_3 (set `self.Rotation` (`KismetMathLibrary.RLerp` (`self.Rotation`) (`self.TargetRotation`) 0.25 true)))
      (`self.K2_SetActorRotation` (`self.GetPlayerPawn`) _output_get_3 false) ; 目標値へ補間しながら向きを合わせる
    )))

(fn `SetTargetRotation`
  (bind _rotation (`/Game/Blueprints/Player/BP_PlayerCameraManager.GetCameraRotationEx` (`self.GetCameraManager`) false false true)) ; カメラ正面の向き（Z軸回転取得）
  (set `self.TargetRotation` (`KismetMathLibrary.ComposeRotators` _rotation (`KismetMathLibrary.Conv_VectorToRotator` (`/Game/Blueprints/BP_FuncLibrary.Vector to 2D(NormalizeXY)` (`KismetMathLibrary.MakeVector` (`self.ValueAxisLY`) (`self.ValueAxisLX`)))))))

(fn `UpdateMoveSpeed`
  (returns (RevSpeed :type "Float (double-precision)"))
  (bind _bhurt (`self.CheckIfNotHurt`))
  (if _bhurt
    (if (`self.AimMode`)
      (return 0.05) ; 構え歩き
      (else
        (return 1.0) ; 走り
      ))
    (else
      (return 0.0) ; 被ダメージ状態
    )))

(fn `UpdateSensitivity`
  (params (Value :type "Float (double-precision) (by ref)") (Horizontal :type Boolean))
  (if Horizontal
    (if (`self.AimMode`)
      (bind _outputvalue (`self.CalcSensitivity` (`self.Sensitivity_Aim`) Value))
      (set `self.ValueAxisRX` _outputvalue)
      (else
        (bind _outputvalue_2 (`self.CalcSensitivity` (`self.Sensitivity`) Value))
        (set `self.ValueAxisRX` _outputvalue_2)))
    (elif (`self.AimMode`)
      (bind _outputvalue_3 (`self.CalcSensitivity` (`self.Sensitivity_Aim`) Value))
      (set `self.ValueAxisRY` _outputvalue_3)
      (else
        (bind _outputvalue_4 (`self.CalcSensitivity` (`self.Sensitivity`) Value))
        (set `self.ValueAxisRY` _outputvalue_4)))))

(fn `UserConstructionScript`)