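; Title-screen game mode that spawns the audio and title UI actors and handles saving and loading of stage-clear progress.
; BeginPlay ensures BP_GlobalData holds a save object and, when its OpenGame flag is set, starts an async load copying StageClear into that game instance.
; SaveGame writes StageClear back asynchronously, then quits the game on completion.
; A PlayBGM helper swaps and restarts the track on BGMPlayer.
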(event `self.ReceiveBeginPlay`
  ;[1 1 1] セーブデータ初期化
  (bind _asbp_global_data (cast `/Game/Blueprints/System/BP_GlobalData` (`GameplayStatics.GetGameInstance`)))
  (bind _savedata (`/Game/Blueprints/System/BP_GlobalData.SaveData` _asbp_global_data))
  (if (not (`KismetSystemLibrary.IsValid` _savedata))
    (bind _returnvalue (`GameplayStatics.CreateSaveGameObject` "/Game/Blueprints/System/BP_SaveGame.BP_SaveGame_C"))
    (set `/Game/Blueprints/System/BP_GlobalData.SaveData` _returnvalue _asbp_global_data))
  (set `self.SaveGameObject` (`|ConvertAsset` _savedata)) ; データ入出力処理初期化
  (if (`/Game/Blueprints/System/BP_GlobalData.OpenGame` _asbp_global_data)
    (`self.LoadGame`) ; データ読込み
  )
  (bind _returnvalue_2 (`|SpawnActorFromClass` "/Game/Blueprints/System/BP_Audio.BP_Audio_C" (`KismetMathLibrary.MakeTransform` (0.0 0.0 0.0)) "Undefined" "OverrideRootScale" null null))
  (set `self.Actor_Audio` (`|ConvertAsset` _returnvalue_2))
  (`self.InitTitleUI`))

(event `LoadGame`
  ;[1 1 1] セーブ＆ロード
  (bind (_slotname _userindex) (`/Game/Blueprints/System/BP_SaveGame.GetSaveID` (`|ConvertAsset` (`self.SaveGameObject`))))
  (bind (_savegame _bsuccess) (`AsyncActionHandleSaveGame.AsyncLoadGameFromSlot` _slotname _userindex) ; データ読込み
    (:`Completed`
      (if _bsuccess
        (bind _asbp_save_game (cast `/Game/Blueprints/System/BP_SaveGame` _savegame))
        (bind _asbp_global_data (cast `/Game/Blueprints/System/BP_GlobalData` (`GameplayStatics.GetGameInstance`)))
        (set `/Game/Blueprints/System/BP_GlobalData.bStageClear` (`/Game/Blueprints/System/BP_SaveGame.bStageClear` _asbp_save_game) _asbp_global_data) ; データ更新
      ))))

(event `SaveGame`
  (bind _output (`|ConvertAsset` (`self.SaveGameObject`)))
  ;[1 1 1] セーブ＆ロード
  (bind _asbp_global_data (cast `/Game/Blueprints/System/BP_GlobalData` (`GameplayStatics.GetGameInstance`)))
  (set `/Game/Blueprints/System/BP_SaveGame.bStageClear` (`/Game/Blueprints/System/BP_GlobalData.bStageClear` _asbp_global_data) _output) ; データ保存
  (bind (_slotname _userindex) (`/Game/Blueprints/System/BP_SaveGame.GetSaveID` _output)) ; データ書出し
  (`AsyncActionHandleSaveGame.AsyncSaveGameToSlot` _output _slotname _userindex
    (:`Completed`
      (`KismetSystemLibrary.QuitGame` null "Quit") ; ゲーム終了
    )))

(fn `InitTitleUI`
  (bind _returnvalue (`|SpawnActorFromClass` "/Game/Blueprints/System/BP_UI/BP_TitleUI.BP_TitleUI_C" (`KismetMathLibrary.MakeTransform` (0.0 0.0 0.0)) "Undefined" "OverrideRootScale" null null))
  (set `self.Actor_TitleUI` (`|ConvertAsset` _returnvalue)))

(fn `PlayBGM`
  (params (BGM_Cue :type "SoundCue Object Reference"))
  (returns (BGM_Player :type "AudioComponent Object Reference"))
  (bind _bgm_player (`self.BGM_Player`))
  (if (`AudioComponent.IsPlaying` _bgm_player)
    (`AudioComponent.Stop` _bgm_player) ; BGM停止
  )
  (`AudioComponent.SetSound` _bgm_player BGM_Cue) ; BGM変更
  (`AudioComponent.Play` _bgm_player 0.0) ; BGM開始
  (return _bgm_player))

(fn `UserConstructionScript`)