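; Slime enemy that rushes the player and can be sucked into the player's weapon.
; Entering its trigger sphere starts timed charges along a flattened direction locked at each start, repeating while the player stays in range, with material swaps.
; BeginSuck disables physics and character movement, then Tick's swept offset, which also drives charges, homes on the weapon.
; Overlapping the weapon while being sucked destroys the slime.
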(event `self.ReceiveActorBeginOverlap`
  (params (OtherActor :type "Actor Object Reference")))

(event `self.ReceiveBeginPlay`
  (`SphereComponent.SetSphereRadius` (`self.Rush Trigger`) (`self.Radius`) true))

(event `self.ReceiveTick`
  (params (DeltaSeconds :type "Float (single-precision)"))
  ;[1 1 1] 移動
  (if (or (`self.IsChasing`) (`self.IsSucking`))
    (`self.K2_AddActorWorldOffset` (* (`self.PlayerDirection`) (* DeltaSeconds (`self.Speed`))) true)
    (if (`self.IsSucking`)
      (set `self.PlayerDirection` (`self.CalcWeaponDirection`)) ; プレイヤーの位置更新
    )))

(event `self.Rush Trigger.OnComponentBeginOverlap`
  (params (OverlappedComponent :type "PrimitiveComponent Object Reference") (OtherActor :type "Actor Object Reference") (OtherComp :type "PrimitiveComponent Object Reference") (OtherBodyIndex :type Integer) (bFromSweep :type Boolean) (SweepResult :type "HitResult Structure (by ref)"))
  ;[1 1 1] プレイヤー発見
  (if (and (`.bSuccess` (cast `/Game/Blueprints/Player/BP_Player` OtherActor :!pure true)) (not (`self.IsSucking`)))
    (`PrimitiveComponent.SetMaterial` (`self.Mesh`) 0 "/Engine/MapTemplates/Materials/BasicAsset01.BasicAsset01")
    (`KismetSystemLibrary.K2_SetTimerDelegate` (delegate `BeginChase`) 2.0)))

(event `BeginChase`
  ;[1 1 1] 追いかけ開始
  (set `self.IsChasing` true)
  (set `self.PlayerDirection` (`self.CalcPlayerDirectionFlat`))
  (set `self.Speed` (`self.ChaseSpeed`))
  (`PrimitiveComponent.SetMaterial` (`self.Mesh`) 0 "/Engine/MapTemplates/Materials/BasicAsset01.BasicAsset01")
  (`KismetSystemLibrary.K2_SetTimerDelegate` (delegate `EndChase`) 2.0))

(event `EndChase`
  ;[1 1 1] 追いかけ終了
  (if (and (>= (`self.Radius`) (`self.CalcPlayerDistance`)) (not (`self.IsSucking`)))
    (`KismetSystemLibrary.K2_SetTimerDelegate` (delegate `BeginChase`) 2.0))
  (`PrimitiveComponent.SetMaterial` (`self.Mesh`) 0 "/Engine/MapTemplates/Materials/BasicAsset02.BasicAsset02")
  (set `self.IsChasing` false))

(event `Begin Suck`
  ;[1 1 1] 吸い込まれ開始
  (set `self.IsSucking` true)
  (set `self.Speed` (`self.SuckSpeed`))
  (set `self.PlayerDirection` (`self.CalcWeaponDirection`))
  (`PrimitiveComponent.SetSimulatePhysics` (`self.Mesh`) false)
  (`ActorComponent.Deactivate` (`self.CharacterMovement`)))

(event `self.StaticMesh.OnComponentBeginOverlap`
  (params (OverlappedComponent :type "PrimitiveComponent Object Reference") (OtherActor :type "Actor Object Reference") (OtherComp :type "PrimitiveComponent Object Reference") (OtherBodyIndex :type Integer) (bFromSweep :type Boolean) (SweepResult :type "HitResult Structure (by ref)"))
  ;[1 1 1] 吸い込まれ終了
  (if (and (`.bSuccess` (cast `/Game/Blueprints/Weapon/BP_Weapon` OtherActor :!pure true)) (`self.IsSucking`))
    (`self.K2_DestroyActor`)))

(fn `CalcPlayerDirectionFlat`
  (returns (Directon :type "Vector Structure"))
  (return (`KismetMathLibrary.Normal` (`KismetMathLibrary.MakeVector` (.x (- (`self.K2_GetActorLocation` (`GameplayStatics.GetPlayerPawn` 0)) (`self.K2_GetActorLocation`))) (.y (- (`self.K2_GetActorLocation` (`GameplayStatics.GetPlayerPawn` 0)) (`self.K2_GetActorLocation`)))))))

(fn `CalcPlayerDistance`
  (returns (Distance :type "Float (double-precision)"))
  (return (`KismetMathLibrary.VSize` (- (`self.K2_GetActorLocation` (`GameplayStatics.GetPlayerPawn` 0)) (`self.K2_GetActorLocation`)))))

(fn `CalcWeaponDirection`
  (returns (Direction :type "Vector Structure"))
  (return (`KismetMathLibrary.Normal` (- (`self.CalcWeaponLocation`) (`self.K2_GetActorLocation`)))))

(fn `CalcWeaponLocation`
  (returns (Location :type "Vector Structure"))
  (bind _asbp_player (cast `/Game/Blueprints/Player/BP_Player` (`GameplayStatics.GetPlayerPawn` 0)))
  (return (`self.K2_GetActorLocation` (`|ConvertAsset` (`/Game/Blueprints/Player/BP_Player.GetWeapon` _asbp_player)))))

(fn `UserConstructionScript`)