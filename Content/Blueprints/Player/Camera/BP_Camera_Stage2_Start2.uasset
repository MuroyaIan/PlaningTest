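; Intro camera actor for the start of Stage 2 that flies a camera along a spline around the player.
; While Start is set, Tick snaps the actor to the player and turns the camera toward them, keeping it level.
; It also advances the camera along SplineStageStart at MoveSpeed.
; At the spline's end it blends the view to the player pawn and updates BP_GlobalData to begin the stage and end cinema mode.
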(event `self.ReceiveTick`
  (params (DeltaSeconds :type "Float (single-precision)"))
  (bind _cameracomponent (`self.CameraComponent`))
  (bind _returnvalue (`self.K2_GetActorLocation` (`GameplayStatics.GetPlayerPawn` 0)))
  (if (and (`self.bStart`) (not (`self.bFin`)))
    (`|ExecutionSequence`
      (:`then_0`
        (`self.K2_SetActorLocation` _returnvalue) ; プレイヤーの位置と同期
        (`SceneComponent.K2_SetWorldRotation` _cameracomponent (`KismetMathLibrary.FindLookAtRotation` (`KismetMathLibrary.MakeVector` (.x (`SceneComponent.K2_GetComponentLocation` _cameracomponent)) (.y (`SceneComponent.K2_GetComponentLocation` _cameracomponent)) (.z _returnvalue)) _returnvalue) false false) ; プレイヤーへ向かわせる
      )
      (:`then_1`
        (set `self.CurrentDistance` (+ (`self.CurrentDistance`) (* (`self.MoveSpeed`) DeltaSeconds)))
        (`SceneComponent.K2_SetWorldLocation` (`self.CameraComponent`) (`SplineComponent.GetLocationAtDistanceAlongSpline` (`self.Spline_StageStart`) (`self.CurrentDistance`) "World") false false)
        (if (>= (`self.CurrentDistance`) (`SplineComponent.GetSplineLength` (`self.Spline_StageStart`)))
          (set `self.bFin` true)
          (`PlayerController.SetViewTargetWithBlend` (`GameplayStatics.GetPlayerController` 0) (`GameplayStatics.GetPlayerPawn` 0) 1.0 "VTBlend_Linear" 0.0 false)
          (bind _asbp_global_data (cast `/Game/Blueprints/System/BP_GlobalData` (`GameplayStatics.GetGameInstance`)))
          (set `/Game/Blueprints/System/BP_GlobalData.bStageStart` true _asbp_global_data)
          (set `/Game/Blueprints/System/BP_GlobalData.bCinema` false _asbp_global_data))))))

(fn `UserConstructionScript`)