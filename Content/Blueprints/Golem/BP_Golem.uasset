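; Golem boss character whose overlap volumes start the battle and flag trample, punch, sweep and rush attacks.
; Limb and hip-drop hitboxes apply fixed damage, while CheckAction toggles the trigger volumes and CheckPunchLR picks the fist nearer the player.
; On BeginPlay it spawns slime cover actors and assigns arm socket names to some.
; It binds to the player's weapon detector for suck events and offers debug hitbox and speed display.
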(event `self.ReceiveBeginPlay`
  (set `CharacterMovementComponent.MaxWalkSpeed` (`self.MoveSpeed`) (`self.CharacterMovement`)) ; 移動速度初期化
  (`self.Debug_DrawCollision`)
  (`self.InitSlimeCover`))

(event `self.ReceiveTick`
  (params (DeltaSeconds :type "Float (single-precision)"))
  (`self.InitBind`)
  (`self.PrintInfo`))

(event `self.StartBattle.OnComponentBeginOverlap`
  (params (OverlappedComponent :type "PrimitiveComponent Object Reference") (OtherActor :type "Actor Object Reference") (OtherComp :type "PrimitiveComponent Object Reference") (OtherBodyIndex :type Integer) (bFromSweep :type Boolean) (SweepResult :type "HitResult Structure (by ref)"))
  (`/Engine/EditorBlueprintResources/StandardMacros.DoOnce` false
    (:`Completed`
      (set `self.bBattle` true) ; 戦闘開始
    )))

(event `PlayerSuckOn`
  (set `self.bPlayerSuck` true))

(event `PlayerSuckOff`
  (set `self.bPlayerSuck` false))

(event `self.StartTrampling.OnComponentBeginOverlap`
  (params (OverlappedComponent :type "PrimitiveComponent Object Reference") (OtherActor :type "Actor Object Reference") (OtherComp :type "PrimitiveComponent Object Reference") (OtherBodyIndex :type Integer) (bFromSweep :type Boolean) (SweepResult :type "HitResult Structure (by ref)"))
  (set `self.bTrampling` true))

(event `self.TramplingR.OnComponentBeginOverlap`
  (params (OverlappedComponent :type "PrimitiveComponent Object Reference") (OtherActor :type "Actor Object Reference") (OtherComp :type "PrimitiveComponent Object Reference") (OtherBodyIndex :type Integer) (bFromSweep :type Boolean) (SweepResult :type "HitResult Structure (by ref)"))
  (`GameplayStatics.ApplyDamage` OtherActor 2.0 null null "/Script/Engine.DamageType"))

(event `self.TramplingL.OnComponentBeginOverlap`
  (params (OverlappedComponent :type "PrimitiveComponent Object Reference") (OtherActor :type "Actor Object Reference") (OtherComp :type "PrimitiveComponent Object Reference") (OtherBodyIndex :type Integer) (bFromSweep :type Boolean) (SweepResult :type "HitResult Structure (by ref)"))
  (`GameplayStatics.ApplyDamage` OtherActor 2.0 null null "/Script/Engine.DamageType"))

(event `self.HipDrop.OnComponentBeginOverlap`
  (params (OverlappedComponent :type "PrimitiveComponent Object Reference") (OtherActor :type "Actor Object Reference") (OtherComp :type "PrimitiveComponent Object Reference") (OtherBodyIndex :type Integer) (bFromSweep :type Boolean) (SweepResult :type "HitResult Structure (by ref)"))
  (`GameplayStatics.ApplyDamage` OtherActor 8.0 null null "/Script/Engine.DamageType"))

(event `self.StartPunch.OnComponentBeginOverlap`
  (params (OverlappedComponent :type "PrimitiveComponent Object Reference") (OtherActor :type "Actor Object Reference") (OtherComp :type "PrimitiveComponent Object Reference") (OtherBodyIndex :type Integer) (bFromSweep :type Boolean) (SweepResult :type "HitResult Structure (by ref)"))
  (set `self.bPunch` true)
  (set `self.bTriPunch` true))

(event `self.PunchR.OnComponentBeginOverlap`
  (params (OverlappedComponent :type "PrimitiveComponent Object Reference") (OtherActor :type "Actor Object Reference") (OtherComp :type "PrimitiveComponent Object Reference") (OtherBodyIndex :type Integer) (bFromSweep :type Boolean) (SweepResult :type "HitResult Structure (by ref)"))
  (`GameplayStatics.ApplyDamage` OtherActor 2.0 null null "/Script/Engine.DamageType"))

(event `self.PunchL.OnComponentBeginOverlap`
  (params (OverlappedComponent :type "PrimitiveComponent Object Reference") (OtherActor :type "Actor Object Reference") (OtherComp :type "PrimitiveComponent Object Reference") (OtherBodyIndex :type Integer) (bFromSweep :type Boolean) (SweepResult :type "HitResult Structure (by ref)"))
  (`GameplayStatics.ApplyDamage` OtherActor 2.0 null null "/Script/Engine.DamageType"))

(event `self.StartGetRidOfL.OnComponentBeginOverlap`
  (params (OverlappedComponent :type "PrimitiveComponent Object Reference") (OtherActor :type "Actor Object Reference") (OtherComp :type "PrimitiveComponent Object Reference") (OtherBodyIndex :type Integer) (bFromSweep :type Boolean) (SweepResult :type "HitResult Structure (by ref)"))
  (set `self.bGetRidOf_L` true))

(event `self.StartGetRidOfR.OnComponentBeginOverlap`
  (params (OverlappedComponent :type "PrimitiveComponent Object Reference") (OtherActor :type "Actor Object Reference") (OtherComp :type "PrimitiveComponent Object Reference") (OtherBodyIndex :type Integer) (bFromSweep :type Boolean) (SweepResult :type "HitResult Structure (by ref)"))
  (set `self.bGetRidOf_R` true))

(event `self.GetRidOfL.OnComponentBeginOverlap`
  (params (OverlappedComponent :type "PrimitiveComponent Object Reference") (OtherActor :type "Actor Object Reference") (OtherComp :type "PrimitiveComponent Object Reference") (OtherBodyIndex :type Integer) (bFromSweep :type Boolean) (SweepResult :type "HitResult Structure (by ref)"))
  (`GameplayStatics.ApplyDamage` OtherActor 4.0 null null "/Script/Engine.DamageType"))

(event `self.GetRidOfR.OnComponentBeginOverlap`
  (params (OverlappedComponent :type "PrimitiveComponent Object Reference") (OtherActor :type "Actor Object Reference") (OtherComp :type "PrimitiveComponent Object Reference") (OtherBodyIndex :type Integer) (bFromSweep :type Boolean) (SweepResult :type "HitResult Structure (by ref)"))
  (`GameplayStatics.ApplyDamage` OtherActor 4.0 null null "/Script/Engine.DamageType"))

(event `self.StartRushTrampling.OnComponentBeginOverlap`
  (params (OverlappedComponent :type "PrimitiveComponent Object Reference") (OtherActor :type "Actor Object Reference") (OtherComp :type "PrimitiveComponent Object Reference") (OtherBodyIndex :type Integer) (bFromSweep :type Boolean) (SweepResult :type "HitResult Structure (by ref)"))
  ;[1 1 1] ダメージコリジョンは踏み潰しと共有！
  (set `self.bRushTrampling` true))

(event `self.MoveL.OnComponentBeginOverlap`
  (params (OverlappedComponent :type "PrimitiveComponent Object Reference") (OtherActor :type "Actor Object Reference") (OtherComp :type "PrimitiveComponent Object Reference") (OtherBodyIndex :type Integer) (bFromSweep :type Boolean) (SweepResult :type "HitResult Structure (by ref)"))
  (`GameplayStatics.ApplyDamage` OtherActor 1.0 null null "/Script/Engine.DamageType"))

(event `self.MoveR.OnComponentBeginOverlap`
  (params (OverlappedComponent :type "PrimitiveComponent Object Reference") (OtherActor :type "Actor Object Reference") (OtherComp :type "PrimitiveComponent Object Reference") (OtherBodyIndex :type Integer) (bFromSweep :type Boolean) (SweepResult :type "HitResult Structure (by ref)"))
  (`GameplayStatics.ApplyDamage` OtherActor 1.0 null null "/Script/Engine.DamageType"))

(fn `Check Punch LR`
  (bind _returnvalue (`self.K2_GetActorLocation` (`GameplayStatics.GetPlayerPawn` 0)))
  (if (< (`KismetMathLibrary.Vector_Distance` (`SceneComponent.K2_GetComponentLocation` (`self.PunchL`)) _returnvalue) (`KismetMathLibrary.Vector_Distance` _returnvalue (`SceneComponent.K2_GetComponentLocation` (`self.PunchR`))))
    (set `self.bPunch_L` true)
    (else
      (set `self.bPunch_R` true))))

(fn `CheckAction`
  (if (`self.bAction`)
    (`PrimitiveComponent.SetCollisionEnabled` (`self.StartTrampling`) "NoCollision")
    (`PrimitiveComponent.SetCollisionEnabled` (`self.StartPunch`) "NoCollision")
    (`PrimitiveComponent.SetCollisionEnabled` (`self.StartGetRidOfL`) "NoCollision")
    (`PrimitiveComponent.SetCollisionEnabled` (`self.StartGetRidOfR`) "NoCollision")
    (`PrimitiveComponent.SetCollisionEnabled` (`self.StartRushTrampling`) "NoCollision")
    (else
      (`PrimitiveComponent.SetCollisionEnabled` (`self.StartTrampling`) "QueryAndPhysics")
      (`PrimitiveComponent.SetCollisionEnabled` (`self.StartPunch`) "QueryAndPhysics")
      (`PrimitiveComponent.SetCollisionEnabled` (`self.StartGetRidOfL`) "QueryAndPhysics")
      (`PrimitiveComponent.SetCollisionEnabled` (`self.StartGetRidOfR`) "QueryAndPhysics")
      (`PrimitiveComponent.SetCollisionEnabled` (`self.StartRushTrampling`) "QueryAndPhysics"))))

(fn `Debug_DrawCollision`
  (if (`self.bDebugDraw`)
    (`|ExecutionSequence`
      (:`then_0`
        (`/Engine/EditorBlueprintResources/StandardMacros.DoOnce` false
          (:`Completed`
            (`SceneComponent.SetHiddenInGame` (`self.StartBattle`) false false)
            (`SceneComponent.SetHiddenInGame` (`self.StartTrampling`) false false)
            (`SceneComponent.SetHiddenInGame` (`self.StartPunch`) false false)
            (`SceneComponent.SetHiddenInGame` (`self.StartGetRidOfR`) true false)
            (`SceneComponent.SetHiddenInGame` (`self.StartGetRidOfL`) false false)
            (`SceneComponent.SetHiddenInGame` (`self.StartRushTrampling`) false false))))
      (:`then_1`
        (`|ExecutionSequence`
          (:`then_0`
            (if (or (`self.bTrampling`) (`self.bRushTrampling`))
              (`SceneComponent.SetHiddenInGame` (`self.TramplingL`) false false)
              (`SceneComponent.SetHiddenInGame` (`self.TramplingR`) false false)
              (else
                (`SceneComponent.SetHiddenInGame` (`self.TramplingL`) true false)
                (`SceneComponent.SetHiddenInGame` (`self.TramplingR`) true false))))
          (:`then_1`
            (if (`self.bHipDrop`)
              (`SceneComponent.SetHiddenInGame` (`self.HipDrop`) false false)
              (else
                (`SceneComponent.SetHiddenInGame` (`self.HipDrop`) true false))))
          (:`then_2`
            (if (or (`self.bPunch`) (`self.bTriPunch`))
              (`SceneComponent.SetHiddenInGame` (`self.PunchL`) false false)
              (`SceneComponent.SetHiddenInGame` (`self.PunchR`) false false)
              (else
                (`SceneComponent.SetHiddenInGame` (`self.PunchL`) true false)
                (`SceneComponent.SetHiddenInGame` (`self.PunchR`) true false))))
          (:`then_3`
            (if (or (`self.bGetRidOf_L`) (`self.bGetRidOf_R`))
              (`SceneComponent.SetHiddenInGame` (`self.GetRidOfL`) false false)
              (`SceneComponent.SetHiddenInGame` (`self.GetRidOfR`) false false)
              (else
                (`SceneComponent.SetHiddenInGame` (`self.GetRidOfL`) true false)
                (`SceneComponent.SetHiddenInGame` (`self.GetRidOfR`) true false)))))))))

(fn `InitBind`
  (`/Engine/EditorBlueprintResources/StandardMacros.DoOnce` false
    (:`Completed`
      (bind _asbp_player (cast `/Game/Blueprints/Player/BP_Player` (`GameplayStatics.GetPlayerPawn` 0)))
      (add `/Game/Blueprints/Weapon/BP_Detector.SuckBoss` (`/Game/Blueprints/Weapon/BP_Weapon.GetDetector` (`/Game/Blueprints/Player/BP_Player.GetWeapon` _asbp_player)) (`|CreateDelegate` :!event `PlayerSuckOn`)) ; 武器スキャン機と紐づけ
    )))

(fn `InitSlimeCover`
  (bind _slime_cover (`self.Slime_Cover`))
  (`|ExecutionSequence`
    (:`then_0`
      (for _ (range 27)
        (bind _returnvalue (`|SpawnActorFromClass` "/Game/Blueprints/Slime/BP_Slime_Cover.BP_Slime_Cover_C" (`self.GetTransform`) "Undefined" "OverrideRootScale" null (`|ConvertAsset` self) null))
        (`KismetArrayLibrary.Array_Add` (`self.Slime_Cover`) (`|ConvertAsset` _returnvalue))))
    (:`then_1`
      (`|ExecutionSequence`
        (:`then_0`
          (set `/Game/Blueprints/Slime/BP_Slime_Cover.SocketName` "JNT_RightArmSlimeA" (`|ConvertAsset` (`|GetArrayItem` _slime_cover)))
          (set `/Game/Blueprints/Slime/BP_Slime_Cover.SocketName` "JNT_RightArmSlimeB" (`|ConvertAsset` (`|GetArrayItem` _slime_cover 1)))
          (set `/Game/Blueprints/Slime/BP_Slime_Cover.SocketName` "JNT_RightArmSlimeC" (`|ConvertAsset` (`|GetArrayItem` _slime_cover 2)))
          (set `/Game/Blueprints/Slime/BP_Slime_Cover.SocketName` "JNT_RightArmSlimeD" (`|ConvertAsset` (`|GetArrayItem` _slime_cover 3)))
          (set `/Game/Blueprints/Slime/BP_Slime_Cover.SocketName` "JNT_RightArmSlimeE" (`|ConvertAsset` (`|GetArrayItem` _slime_cover 4)))
          (set `/Game/Blueprints/Slime/BP_Slime_Cover.SocketName` "JNT_RightArmSlimeF" (`|ConvertAsset` (`|GetArrayItem` _slime_cover 5)))
          (set `/Game/Blueprints/Slime/BP_Slime_Cover.SocketName` "JNT_RightArmSlimeG" (`|ConvertAsset` (`|GetArrayItem` _slime_cover 6)))
          (set `/Game/Blueprints/Slime/BP_Slime_Cover.SocketName` "JNT_RightArmSlimeH" (`|ConvertAsset` (`|GetArrayItem` _slime_cover 7))))
        (:`then_1`
          (set `/Game/Blueprints/Slime/BP_Slime_Cover.SocketName` "JNT_LeftArmSlimeA" (`|ConvertAsset` (`|GetArrayItem` _slime_cover 8))))))))

(fn `PrintInfo`
  (bind _bdebug (`/Game/Blueprints/BP_FuncLibrary.CheckDebugPrint`))
  (if _bdebug
    (`KismetSystemLibrary.PrintString` (`KismetStringLibrary.Concat_StrStr` "[GolemInfo] \nSpeed:" (`KismetStringLibrary.Conv_IntToString` (`KismetMathLibrary.Round` (`KismetMathLibrary.VSize` (`self.GetVelocity`))))) true false (struct :`R` 1.0 :`G` 0.892819 :`A` 1.0) 0.0)))

(fn `ResetActionFlag`
  (set `self.bTrampling` false)
  (set `self.bHipDrop` false)
  (set `self.bSuckReady` false)
  (set `self.bPunch` false)
  (set `self.bTriPunch` false)
  (set `self.bPunch_L` false)
  (set `self.bPunch_R` false)
  (set `self.bGetRidOf_L` false)
  (set `self.bGetRidOf_R` false)
  (set `self.bRushTrampling` false)
  ;[1 1 1] 体幹耐え初期化
  (set `self.bTrunkEndurance` false)
  (`self.PlayerSuckOff`))

(fn `UserConstructionScript`)