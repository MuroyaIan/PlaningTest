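; Player camera manager for an orbiting third-person camera offset to the target's right.
; BlueprintUpdateCamera looks at a cached chest-height gaze point, shifted along camera right, from a rotated relative offset.
; Pitch and yaw inputs, gated by a Control flag, adjust the target rotation, with pitch clamped.
; Tick eases offset, rotation and FOV toward targets by a fixed, frame-rate-dependent lerp and prints camera debug info on screen.
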(event `self.ReceiveBeginPlay`
  (set `self.Location` (`self.TargetLocation`)) ; 位置修正初期化
  (set `self.Rotation` (`self.TargetRotation`)) ; 回転値初期化
  (set `self.FOV` (`self.TargetFOV`)) ; 視野角初期化
)

(event `self.ReceiveTick`
  (params (DeltaSeconds :type "Float (single-precision)"))
  (`|ExecutionSequence`
    (:`then_0`
      (if (`KismetMathLibrary.NotEqualExactly_VectorVector` (`self.Location`) (`self.TargetLocation`))
        (set `self.Location` (`KismetMathLibrary.VLerp` (`self.Location`) (`self.TargetLocation`) 0.25)) ; 位置修正更新
      ))
    (:`then_1`
      (if (!= (`self.Rotation`) (`self.TargetRotation`) :`ErrorTolerance` 0.0)
        (set `self.Rotation` (`KismetMathLibrary.RLerp` (`self.Rotation`) (`self.TargetRotation`) 0.25 true)) ; 回転値更新
      ))
    (:`then_2`
      (if (!= (`self.FOV`) (`self.TargetFOV`))
        (set `self.FOV` (`KismetMathLibrary.Lerp` (`self.FOV`) (`self.TargetFOV`) 0.25)) ; 視野角更新
      ))
    (:`then_3`
      (`self.PrintCameraInfo` (`self.Rotation`) (`self.Location`) (`self.FOV`)))))

(fn `AddPitchInput`
  (params (Value :type "Float (double-precision) (by ref)"))
  (if (`self.Control`)
    (if (!= 0.0 Value)
      (set `self.TargetRotation` (`KismetMathLibrary.MakeRotator` (.roll (`self.TargetRotation`)) (`KismetMathLibrary.ClampAngle` (+ (.pitch (`self.TargetRotation`)) Value) (`self.ViewPitchMin`) (`self.ViewPitchMax`)) (.yaw (`self.TargetRotation`)))))))

(fn `AddYawInput`
  (params (Value :type "Float (double-precision) (by ref)"))
  (if (`self.Control`)
    (if (!= 0.0 Value)
      (set `self.TargetRotation` (`KismetMathLibrary.MakeRotator` (.roll (`self.TargetRotation`)) (.pitch (`self.TargetRotation`)) (+ (.yaw (`self.TargetRotation`)) Value))))))

(fn `BlueprintUpdateCamera`
  (params (CameraTarget :type "Actor Object Reference"))
  (returns (NewCameraLocation :type "Vector Structure") (NewCameraRotation :type "Rotator Structure") (NewCameraFOV :type "Float (double-precision)") (ReturnValue :type Boolean))
  (bind _gazepoint (`self.SetGazePoint` (`self.K2_GetActorLocation` CameraTarget))) ; 注視点位置（アクタ）
  (bind _pov (`self.SetPOV` _gazepoint)) ; 視点位置（カメラ）
  (return _pov (`KismetMathLibrary.FindLookAtRotation` _pov _gazepoint) (`self.FOV`) true))

(fn `GetCameraRotationEx`
  (params (RotX :type Boolean :default true) (RotY :type Boolean :default true) (RotZ :type Boolean :default true))
  (returns (Rotation :type "Rotator Structure"))
  (locals (CameraRotation :type "Rotator Structure" :default (struct)))
  (bind _returnvalue (`self.GetCameraRotation`))
  (if RotX
    (set `local.CameraRotation` (`KismetMathLibrary.MakeRotator` (+ (.roll (`local.CameraRotation`)) (.roll _returnvalue)) (.pitch (`local.CameraRotation`)) (.yaw (`local.CameraRotation`)))))
  (if RotY
    (set `local.CameraRotation` (`KismetMathLibrary.MakeRotator` (.roll (`local.CameraRotation`)) (+ (.pitch (`local.CameraRotation`)) (.pitch _returnvalue)) (.yaw (`local.CameraRotation`)))))
  (if RotZ
    (bind _output_get (set `local.CameraRotation` (`KismetMathLibrary.MakeRotator` (.roll (`local.CameraRotation`)) (.pitch (`local.CameraRotation`)) (+ (.yaw (`local.CameraRotation`)) (.yaw _returnvalue))))))
  (return _output_get))

(fn `GetForwardVector`
  (returns (Value :type "Vector Structure"))
  (return (`KismetMathLibrary.GetForwardVector` (`self.GetCameraRotation`))))

(fn `GetForwardVector_XY`
  (returns (Value :type "Vector Structure"))
  (return (`/Game/Blueprints/BP_FuncLibrary.Vector to 2D(NormalizeXY)` (`KismetMathLibrary.GetForwardVector` (`self.GetCameraRotation`)))))

(fn `GetRightVector`
  (returns (Value :type "Vector Structure"))
  (return (`KismetMathLibrary.GetRightVector` (`self.GetCameraRotation`))))

(fn `GetRightVector_XY`
  (returns (Value :type "Vector Structure"))
  (return (`/Game/Blueprints/BP_FuncLibrary.Vector to 2D(NormalizeXY)` (`KismetMathLibrary.GetRightVector` (`self.GetCameraRotation`)))))

(fn `GetUpVector`
  (returns (Value :type "Vector Structure"))
  (return (`KismetMathLibrary.GetUpVector` (`self.GetCameraRotation`))))

(fn `GetUpVector_XY`
  (returns (Value :type "Vector Structure"))
  (return (`/Game/Blueprints/BP_FuncLibrary.Vector to 2D(NormalizeXY)` (`KismetMathLibrary.GetUpVector` (`self.GetCameraRotation`)))))

(fn `PrintCameraInfo`
  (params (Rotation :type "Rotator Structure (by ref)") (Location :type "Vector Structure (by ref)") (FOV :type "Float (double-precision) (by ref)"))
  (`KismetSystemLibrary.PrintString` (`KismetStringLibrary.Concat_StrStr` "[CameraInfo] \nAngleRoll:" (`KismetStringLibrary.Conv_IntToString` (`KismetMathLibrary.Round` (.roll Rotation))) " \nAnglePitch:" (`KismetStringLibrary.Conv_IntToString` (`KismetMathLibrary.Round` (.pitch Rotation))) " \nAngleYaw:" (`KismetStringLibrary.Conv_IntToString` (`KismetMathLibrary.Round` (.yaw Rotation))) " \nDistance:" (`KismetStringLibrary.Conv_IntToString` (`KismetMathLibrary.Round` (`KismetMathLibrary.VSize` Location))) " \nFOV:" (`KismetStringLibrary.Conv_IntToString` (`KismetMathLibrary.Round` FOV))) true false (struct :`R` 1.0 :`A` 1.0) 0.0))

(fn `SetGazePoint`
  (params (Vector :type "Vector Structure (by ref)"))
  (returns (GazePoint :type "Vector Structure"))
  (bind _value (`self.GetRightVector_XY`))
  (if (`KismetMathLibrary.EqualExactly_VectorVector` Vector (`self.ActorLoaction_Backup`))
    (if (not (`KismetMathLibrary.EqualExactly_VectorVector` (`self.CameraRightVector`) _value))
      (set `self.ActorLoaction_Backup` Vector :!label _label) ; アクタ位置更新
      (set `self.CameraRightVector` _value) ; カメラ向き更新
      (bind _output_get (set `self.GazePoint` (+ (`KismetMathLibrary.MakeVector` (.x (`self.ActorLoaction_Backup`)) (.y (`self.ActorLoaction_Backup`)) (+ (.z (`self.ActorLoaction_Backup`)) (`self.ChestOffset`))) (* (`self.CameraRightVector`) 100)))) ; 注視点位置更新
    )
    (else
      (goto _label)))
  (return _output_get))

(fn `SetPOV`
  (params (GazePoint :type "Vector Structure (by ref)"))
  (returns (POV :type "Vector Structure"))
  (return (+ GazePoint (`KismetMathLibrary.GreaterGreater_VectorRotator` (`self.Location`) (`self.Rotation`)))) ; カメラと注視点の相対位置を決める
)

(fn `UserConstructionScript`)