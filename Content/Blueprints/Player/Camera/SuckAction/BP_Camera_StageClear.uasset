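; BP_Camera_StageClear is a camera Blueprint, named for the stage-clear moment, that frames the player from the front-right and slightly above.
; Each Tick it casts the player pawn to BP_Player and snaps itself to a fixed offset along that player's forward, right and up vectors.
; It then rotates to look at the player's location, with no interpolation or sweep.
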(event `self.ReceiveBeginPlay`)

(event `self.ReceiveTick`
  (params (DeltaSeconds :type "Float (single-precision)"))
  (bind _asbp_player (cast `/Game/Blueprints/Player/BP_Player` (`GameplayStatics.GetPlayerPawn` 0)))
  (bind _returnvalue (`self.K2_GetActorLocation` _asbp_player))
  (`self.K2_SetActorLocation` (+ (+ (+ (* (`self.GetActorForwardVector` _asbp_player) 200.0) (* (`self.GetActorRightVector` _asbp_player) 100.0)) (* (`self.GetActorUpVector` _asbp_player) 50.0)) _returnvalue)) ; 位置更新
  (`self.K2_SetActorRotation` (`KismetMathLibrary.FindLookAtRotation` (`self.K2_GetActorLocation`) _returnvalue)) ; 回転更新
)

(fn `UserConstructionScript`)