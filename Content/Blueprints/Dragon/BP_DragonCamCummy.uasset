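; Dragon camera helper actor, judging by its name, that follows the dragon during the player's boss-kill sequence.
; While the player's BossSucked and KillBoss flags are set, Tick copies the dragon's rotation and spine socket XY.
; Its Z lerps from the socket's starting height toward just below the player's weapon, using an unclamped, time-accumulated alpha.
; ZHeight also interpolates each tick but feeds nothing in this graph.
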(event `self.ReceiveBeginPlay`
  (bind (_returnvalue_x _returnvalue_y _returnvalue_z) (`KismetMathLibrary.BreakVector` (`SceneComponent.GetSocketLocation` (`Character.Mesh` (`self.DragonRef`)) "JNT_spine_C0_2")))
  (bind _asbp_player (cast `/Game/Blueprints/Player/BP_Player` (`GameplayStatics.GetPlayerPawn` 0)))
  (set `self.PlayerRef` _asbp_player)
  (set `self.BaseZ` _returnvalue_z))

(event `self.ReceiveTick`
  (params (DeltaSeconds :type "Float (single-precision)"))
  (bind _dragonref (`self.DragonRef`))
  (bind _playerref (`self.PlayerRef`))
  (bind (_returnvalue_x _returnvalue_y) (`KismetMathLibrary.BreakVector` (`SceneComponent.GetSocketLocation` (`Character.Mesh` _dragonref) "JNT_spine_C0_2")))
  (bind (_returnvalue_x_2 _returnvalue_y_2 _returnvalue_z) (`KismetMathLibrary.BreakVector` (+ (`self.K2_GetActorLocation` (`/Game/Blueprints/Player/BP_Player.GetWeapon` (`self.PlayerRef`))) (0.0 0.0 -10.0))))
  (if (and (`/Game/Blueprints/Player/BP_Player.bBossSucked` _playerref) (`/Game/Blueprints/Player/BP_Player.bKillBoss` _playerref))
    (set `self.Alpha` (+ (`self.Alpha`) (* DeltaSeconds 4.0)))
    (`self.K2_SetActorRotation` (`self.K2_GetActorRotation` _dragonref))
    (`self.K2_SetActorLocation` (`KismetMathLibrary.MakeVector` _returnvalue_x _returnvalue_y (`KismetMathLibrary.Lerp` (`self.BaseZ`) _returnvalue_z (`self.Alpha`))))
    (set `self.ZHeight` (`KismetMathLibrary.FInterpTo_Constant` (`self.ZHeight`) 10.0 (`GameplayStatics.GetWorldDeltaSeconds`) 80.0))))

(fn `UserConstructionScript`)