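; BP_LoseUI is an actor that manages the lose-screen menu, creating a UMG_Lose widget and enabling input from BP_PlayerController on BeginPlay.
; ChangeDisp sets a display flag that Tick polls to add or remove the widget from the viewport.
; While displayed, up, down and confirm input actions forward selection and decision to the widget.
; DispOff removes the widget, clears the flag and unpauses the game.
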(event `self.ReceiveBeginPlay`
  (bind _asbp_player_controller (cast `/Game/Blueprints/Player/BP_PlayerController` (`GameplayStatics.GetPlayerController` 0)))
  (`self.EnableInput` _asbp_player_controller) ; 入力有効化
  (bind _returnvalue (`|CreateWidget` "/Game/Maps/TestMap/Kitayama/UI_Kitayama/Widget_UI/PauseWidget/UMG_Lose.UMG_Lose_C"))
  (set `self.Widget_LoseUI` _returnvalue))

(event `self.ReceiveTick`
  (params (DeltaSeconds :type "Float (single-precision)"))
  (bind _returnvalue (`Widget.IsInViewport` (`self.Widget_LoseUI`)))
  (if (`self.isDispUI`)
    (if (not _returnvalue)
      (`UserWidget.AddToViewport` (`self.Widget_LoseUI`) 0))
    (elif _returnvalue
      (`Widget.RemoveFromParent` (`self.Widget_LoseUI`)))))

(event `ChangeDisp`
  (params (Disp :type Boolean))
  (set `self.isDispUI` Disp))

(event `InputAction|UI_Confirm` :consume false :paused true
  (params (Key :type "Key Structure"))
  (:`Pressed`
    (if (`self.isDispUI`)
      (`/Game/Maps/TestMap/Kitayama/UI_Kitayama/Widget_UI/PauseWidget/UMG_Lose.DecidedMenu` (`self.Widget_LoseUI`)))))

(event `InputAction|UI_Up` :consume false :paused true
  (params (Key :type "Key Structure"))
  (:`Pressed`
    (if (`self.isDispUI`)
      (`/Game/Maps/TestMap/Kitayama/UI_Kitayama/Widget_UI/PauseWidget/UMG_Lose.SelectMenu` (`self.Widget_LoseUI`) false))))

(event `InputAction|UI_Down` :consume false :paused true
  (params (Key :type "Key Structure"))
  (:`Pressed`
    (if (`self.isDispUI`)
      (`/Game/Maps/TestMap/Kitayama/UI_Kitayama/Widget_UI/PauseWidget/UMG_Lose.SelectMenu` (`self.Widget_LoseUI`) true))))

(fn `DispOff`
  (`Widget.RemoveFromParent` (`self.Widget_LoseUI`)) ; UIを非表示
  (bind _output_get (set `self.isDispUI` false)) ; 入力制御更新
  (`GameplayStatics.SetGamePaused` _output_get) ; ポーズ処理
)

(fn `UserConstructionScript`)