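; BP_SlimeDefault is an AI-controlled enemy slime that the player wears down by suction.
; Suction hits after the first flag the Blackboard, then spawn a BP_Slime_Small child after a delay and subtract HP.
; Tick destroys it below zero HP, otherwise sets scale and walk speed in five HP steps, and fades escaping slimes out before destroying them.
; A damage overlap flags the Blackboard and gates SlimeAttack damage on the player.
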(event `self.ReceiveBeginPlay`
  (bind _mesh (`self.Mesh`))
  (set `self.HitpointBase` (`self.SlimeHitpoint`)) ; 一応初期化
  ;[0.5 1 1] フェード用に動的にマテリアルを作成
  (`PrimitiveComponent.CreateDynamicMaterialInstance` _mesh 0 "/Game/Maps/TestMap/Nishino/Enemy_SlimeDefault/M_SlimeDefault.M_SlimeDefault" "None")
  (`PrimitiveComponent.CreateDynamicMaterialInstance` _mesh 1 "/Game/Maps/TestMap/Nishino/Enemy_SlimeDefault/M_SlimeDefault.M_SlimeDefault" "None"))

(event `self.ReceiveTick`
  (params (DeltaSeconds :type "Float (single-precision)"))
  (bind _isdelete (`self.Chack_HitPoint` DeltaSeconds)) ; 体力の確認
  (if (not _isdelete)
    (`self.SetSlimeState`) ; 大きさの変更
    ;[0.5 0.5 1] 逃げスライムをいい感じに消す処理
    (if (`self.EscapeFlg`)
      (bind (_direction `_オパシティ`) (`Timeline|EscapeDestroy_TimeLine` :`NewTime` 3.0)
        (:`Update`
          (`MeshComponent.SetScalarParameterValueOnMaterials` (`self.Mesh`) "Opacity" `_オパシティ`))
        (:`Finished`
          (`self.K2_DestroyActor`) ; スライムを消す
        )))))

(event `HitSuck`
  ;[1 0.5 0.5] 吸引に当たっているときの処理
  (if (`self.HitFlg`)
    (set `self.HitFlg` false) ; 当たり判定フラグのリセット
    (if (`self.BindFlg`)
      (`BlackboardComponent.SetValueAsBool` (`AIBlueprintHelperLibrary.GetBlackboard` (`self.GetController`)) "Suck_Flg" true) ; ブラックボードの情報を設定
      (`KismetSystemLibrary.Delay` (`self.Spawn_Time`)) ; 生成頻度
      (`self.Spone_Small`) ; 中神スライムを発生させる
      (set `self.SlimeHitpoint` (- (`self.SlimeHitpoint`) (`self.SlimeDamage`))) ; 体力を減らす
      (else
        (set `self.BindFlg` true) ; 反応のフラグを設定
      ))))

(event `Spone_Small`
  ;[1 1 0.5] 中神スライムを生成
  (bind _returnvalue (`|SpawnActorFromClass` "/Game/Blueprints/Slime/BP_Slime_Small.BP_Slime_Small_C" (`self.MakeTransform`) "Undefined" "OverrideRootScale" null null))
  (set `/Game/Blueprints/Slime/BP_Slime_Small.ParentSlime` (`|ConvertAsset` self) _returnvalue) ; 産まれた奴に情報を書き込む
)

(event `self.Damage.OnComponentBeginOverlap`
  (params (OverlappedComponent :type "PrimitiveComponent Object Reference") (OtherActor :type "Actor Object Reference") (OtherComp :type "PrimitiveComponent Object Reference") (OtherBodyIndex :type Integer) (bFromSweep :type Boolean) (SweepResult :type "HitResult Structure (by ref)"))
  (bind _returnvalue (`AIBlueprintHelperLibrary.GetBlackboard` (`self.GetController`)))
  ;[0.5 1 0.5] ダメージ判定に触った時
  (if (== OtherActor (`GameplayStatics.GetPlayerPawn` 0))
    (`/Engine/EditorBlueprintResources/StandardMacros.IsValid` _returnvalue
      (:`Is Valid`
        (`BlackboardComponent.SetValueAsBool` _returnvalue "DamageCollision_Flg" true)
        (set `self.AttackFlg` true)))))

(event `self.Damage.OnComponentEndOverlap`
  (params (OverlappedComponent :type "PrimitiveComponent Object Reference") (OtherActor :type "Actor Object Reference") (OtherComp :type "PrimitiveComponent Object Reference") (OtherBodyIndex :type Integer))
  (bind _returnvalue (`AIBlueprintHelperLibrary.GetBlackboard` (`self.GetController`)))
  ;[0.5 1 0.5] ダメージ判定に触った時
  (if (== OtherActor (`GameplayStatics.GetPlayerPawn` 0))
    (`/Engine/EditorBlueprintResources/StandardMacros.IsValid` _returnvalue
      (:`Is Valid`
        (`BlackboardComponent.SetValueAsBool` _returnvalue "DamageCollision_Flg" false)
        (set `self.AttackFlg` false)))))

(event `SlimeAttack`
  ;[1 0.5 1] ダメージを与える処理
  (if (`self.AttackFlg`)
    (`GameplayStatics.ApplyDamage` (`GameplayStatics.GetPlayerPawn` 0) 1.0 (`self.GetController`) self) ; スライムからプレイヤーに１ダメージ！
  ))

(fn `Chack_HitPoint`
  (params (Secons :type "Float (double-precision)"))
  (returns (IsDelete :type Boolean))
  ;[1 0.5 1] とりあえずHP<0なら消す
  (if (< (`self.SlimeHitpoint`) 0.0)
    (`self.K2_DestroyActor`) ; スライムを消す
    (return true)
    (else
      (return false))))

(fn `Check_Bind`
  (returns (IfBind :type Boolean))
  (return (not (`self.BindFlg`))))

(fn `Check_Hit`
  (params (`if hit` :type Boolean))
  (set `self.HitFlg` `if hit`))

(fn `SetSlimeState`
  (bind _returnvalue (`KismetMathLibrary.FTrunc` (/ (`self.HitpointBase`) 5.0)))
  ;[0.5 1 1] HPの数値をいい感じに計算して、スライムの大きさを変更する
  (bind _output_get (set `self.SlimeSize` (* (+ (/ (`KismetMathLibrary.FTrunc` (`self.SlimeHitpoint`)) _returnvalue) 1) _returnvalue))) ; サイズの保存
  (bind _returnvalue_2 (`KismetMathLibrary.Conv_IntToDouble` _output_get))
  ;[1 0.5 1] 大きさの変更
  (`SceneComponent.SetWorldScale3D` (`self.Mesh`) (`KismetMathLibrary.MakeVector` _returnvalue_2 _returnvalue_2 _returnvalue_2))
  ;[1 0.5 1] 速度の変更
  (set `CharacterMovementComponent.MaxWalkSpeed` (`|GetArrayItem` (`self.SlimeSpeed`) (- (/ (`self.SlimeSize`) (`KismetMathLibrary.FTrunc` (/ (`self.HitpointBase`) 5.0))) 1)) (`self.CharacterMovement`)))

(fn `SetStatus`
  (params (Hitpoint :type "Float (double-precision)") (Damage :type "Float (double-precision)") (SpawnTime :type "Float (double-precision)") (SlimeSize :type Integer) (SlimeSpeed :type "Array of Float (double-precision)"))
  (set `self.SlimeDamage` Damage) ; 受けるダメージ
  (set `self.Spawn_Time` SpawnTime) ; 出現頻度
  (bind _output_get (set `self.HitpointBase` Hitpoint)) ; 計算用初期体力
  (set `self.SlimeHitpoint` (- (* SlimeSize (/ _output_get 5.0)) 0.0001)) ; スライムの体力
  (set `self.SlimeSpeed` SlimeSpeed) ; スライムの速度
)

(fn `UserConstructionScript`)