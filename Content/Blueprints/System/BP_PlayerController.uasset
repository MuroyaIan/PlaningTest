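; Player controller that routes look and movement axis input to the camera manager and the controlled pawn.
; On BeginPlay it caches the player camera manager as BP_PlayerCameraManager.
; Look axes feed yaw and pitch input into that manager.
; Move axes push the pawn along the camera's forward and right vectors, flattened and normalized in XY, giving camera-relative movement.
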(event `self.ReceiveBeginPlay`
  (bind _asbp_player_camera_manager (cast `/Game/Blueprints/System/BP_PlayerCameraManager` (`self.PlayerCameraManager`)))
  (set `self.CameraManager` _asbp_player_camera_manager) ; 初期化
)

(event `InputAxis|LookRight`
  (params (AxisValue :type "Float (single-precision)"))
  ;[1 1 1] カメラ回転
  (`/Game/Blueprints/System/BP_PlayerCameraManager.AddYawInput` (`self.CameraManager`) AxisValue))

(event `InputAxis|LookUp`
  (params (AxisValue :type "Float (single-precision)"))
  ;[1 1 1] カメラ回転
  (`/Game/Blueprints/System/BP_PlayerCameraManager.AddPitchInput` (`self.CameraManager`) AxisValue))

(event `InputAxis|MoveForward`
  (params (AxisValue :type "Float (single-precision)"))
  ;[1 1 1] キャラクター移動
  (`Pawn.AddMovementInput` (`self.K2_GetPawn`) (`/Game/Blueprints/BP_FuncLibrary.Vector to 2D(NormalizeXY)` (`/Game/Blueprints/System/BP_PlayerCameraManager.GetForwardVector` (`self.CameraManager`))) AxisValue false))

(event `InputAxis|MoveRight`
  (params (AxisValue :type "Float (single-precision)"))
  ;[1 1 1] キャラクター移動
  (`Pawn.AddMovementInput` (`self.K2_GetPawn`) (`/Game/Blueprints/BP_FuncLibrary.Vector to 2D(NormalizeXY)` (`/Game/Blueprints/System/BP_PlayerCameraManager.GetRightVector` (`self.CameraManager`))) AxisValue false))

(fn `UserConstructionScript`)