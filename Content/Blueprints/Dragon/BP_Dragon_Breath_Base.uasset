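; Base projectile Blueprint for dragon breath attacks that damages the player on overlap.
; BeginPlay launches it forward without gravity, sets a lifespan, and enables gravity after a timer unless that timer is negative.
; Overlapping BP_Player stores the damage position, applies damage and calls OnCollisionPlayer, an empty hook presumably for child classes.
; Any overlap with the player collision component that skips or completes this shortens the lifespan to half a second.
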(event `self.ReceiveBeginPlay`
  (bind _projectilemovement (`self.ProjectileMovement`))
  (set `ProjectileMovementComponent.ProjectileGravityScale` 0.0 _projectilemovement)
  (set `ProjectileMovementComponent.InitialSpeed` (`self.InitialSpeed`) _projectilemovement)
  (set `MovementComponent.Velocity` (* (`self.GetActorForwardVector`) (`self.InitialSpeed`)) _projectilemovement)
  (`self.SetLifeSpan` (`self.LifeSpan`))
  (if (>= (`self.GravityTimer`) 0.0)
    (`KismetSystemLibrary.K2_SetTimerDelegate` (delegate `EnableGravity`) (`self.GravityTimer`))))

(event `EnableGravity`
  ;[0.4115 0.4115 0.4115] 重力有効化
  (set `ProjectileMovementComponent.ProjectileGravityScale` 1.0 (`self.ProjectileMovement`)))

(event `self.PlayerCollsion.OnComponentBeginOverlap`
  (params (OverlappedComponent :type "PrimitiveComponent Object Reference") (OtherActor :type "Actor Object Reference") (OtherComp :type "PrimitiveComponent Object Reference") (OtherBodyIndex :type Integer) (bFromSweep :type Boolean) (SweepResult :type "HitResult Structure (by ref)"))
  (`|ExecutionSequence`
    (:`then_0`
      ;[0.2651 0.6924 0.9427] プレイヤーとの当たり判定の処理
      (bind _asbp_player (cast `/Game/Blueprints/Player/BP_Player` OtherActor))
      (set `/Game/Blueprints/Player/BP_Player.DamagePos` (`SceneComponent.K2_GetComponentLocation` OverlappedComponent) _asbp_player)
      (`GameplayStatics.ApplyDamage` _asbp_player (`self.Damage`))
      (`self.OnCollisionPlayer` _asbp_player))
    (:`then_1`
      (`self.SetLifeSpan` 0.5))))

(fn `OnCollisionPlayer`
  (params (Player :type "/Game/Blueprints/Player/BP_Player Object Reference")))

(fn `UserConstructionScript`)