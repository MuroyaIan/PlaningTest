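; Second camera in the boss suck-in cutscene, active when Start is set and the player's weapon reports SuckBoss.
; Each Tick it orbits the player at a fixed radius and slight height, easing yaw at constant speed toward a target angle while looking at the player.
; A DoOnce starts a delay, then blends the view to NextCamera, starts BP_Camera_SuckBoss03, and resets its own state for reuse.
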(event `self.ReceiveBeginPlay`)

(event `self.ReceiveTick`
  (params (DeltaSeconds :type "Float (single-precision)"))
  (bind _nextcamera (`self.NextCamera`))
  (set `self.DeltaSec` DeltaSeconds)
  (if (`self.bStart`)
    (bind _asbp_player (cast `/Game/Blueprints/Player/BP_Player` (`GameplayStatics.GetPlayerPawn` 0)))
    (if (`/Game/Blueprints/Weapon/BP_Weapon.bSuckBoss` (`/Game/Blueprints/Player/BP_Player.GetWeapon` _asbp_player))
      (`|ExecutionSequence`
        (:`then_0`
          (`/Engine/EditorBlueprintResources/StandardMacros.DoOnce` false :!label _label
            (:`Completed`
              (`KismetSystemLibrary.Delay` 3.0) ; カメラ切替
              (`PlayerController.SetViewTargetWithBlend` (`GameplayStatics.GetPlayerController` 0) _nextcamera 1.0 "VTBlend_EaseOut" 0.5 false) ; カメラ切替
              (bind _asbp_camera_suck_boss_03 (cast `/Game/Blueprints/Player/Camera/SuckAction/BP_Camera_SuckBoss03` _nextcamera))
              (set `/Game/Blueprints/Player/Camera/SuckAction/BP_Camera_SuckBoss03.bStart` true _asbp_camera_suck_boss_03)
              (set `self.bStart` false)
              (set `self.Rot` (struct :`Yaw` -135.0))
              (goto _label :!via `Reset`))))
        (:`then_1`
          (bind _returnvalue (`self.K2_GetActorLocation` _asbp_player))
          (bind _returnvalue_2 (+ (`KismetMathLibrary.GreaterGreater_VectorRotator` (* (`self.GetActorForwardVector` _asbp_player) 300.0) (`self.Rot`)) (* (`self.GetActorUpVector` _asbp_player) 30.0) _returnvalue))
          (`self.K2_SetActorLocation` _returnvalue_2) ; カメラ更新
          (`self.K2_SetActorRotation` (`KismetMathLibrary.FindLookAtRotation` _returnvalue_2 _returnvalue))
          (set `self.Rot` (`KismetMathLibrary.MakeRotator` 0.0 0.0 (`KismetMathLibrary.FInterpTo_Constant` (.yaw (`self.Rot`)) -270.0 (`self.DeltaSec`) 20.0))) ; 回転角更新
        )))))

(fn `UserConstructionScript`)