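; Title slime actor, apparently for the title screen, that endlessly alternates two scripted passes: walking, getting sucked away, then respawning facing the other way.
; Turn flags checked on Tick gate delay-timed sequences that toggle the Run and Die states driving per-frame movement and shrinking.
; While shrinking, a dynamic material's MoveVector pulls the body backward and upward, and a looping timer spawns small slimes.
; Each pass ends by resetting scale, material and transform.
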(event `self.ReceiveBeginPlay`
  (bind _mesh_slime (`self.Mesh_Slime`))
  (bind _returnvalue (`PrimitiveComponent.CreateDynamicMaterialInstance` _mesh_slime 0 (`PrimitiveComponent.GetMaterial` _mesh_slime 0) "None"))
  (set `self.MID_Body` _returnvalue) ; 吸われ状態用
)

(event `self.ReceiveTick`
  (params (DeltaSeconds :type "Float (single-precision)"))
  (set `self.DeltaSec` DeltaSeconds)
  (`|ExecutionSequence`
    (:`then_0`
      (if (`self.bTurn1`)
        (`/Engine/EditorBlueprintResources/StandardMacros.DoOnce` false :!label _label
          (:`Completed`
            (`SkeletalMeshComponent.PlayAnimation` (`self.Mesh_Slime`) "/Game/Resource/CH/Slime/Anim/CH_MO_Slime_Walk.CH_MO_Slime_Walk" true) ; 走り出す
            (set `self.bRun` true)
            (`KismetSystemLibrary.Delay` 15.0)
            (set `self.bRun` false)
            (`SkeletalMeshComponent.PlayAnimation` (`self.Mesh_Slime`) "/Game/Resource/CH/Slime/Anim/CH_MO_Slime_Idle.CH_MO_Slime_Idle" true) ; 吸われ開始
            (`MaterialInstanceDynamic.SetVectorParameterValue` (`self.MID_Body`) "MoveVector" (`KismetMathLibrary.MakeColor` (.x (* (`self.GetActorForwardVector`) -1.0)) (.y (* (`self.GetActorForwardVector`) -1.0)) (+ (.z (* (`self.GetActorForwardVector`) -1.0)) 0.5)))
            (`KismetSystemLibrary.K2_SetTimer` null "SpawnSmallSlime_L" 0.2 true)
            (set `self.bDie` true)
            (`KismetSystemLibrary.Delay` 4.5)
            (`KismetSystemLibrary.K2_ClearTimer` null "SpawnSmallSlime_L")
            (`KismetSystemLibrary.Delay` 0.5) ; パターンBへ移行
            (set `self.bDie` false)
            (`KismetSystemLibrary.Delay` 4.0) ; パターンB開始
            (`MaterialInstanceDynamic.SetVectorParameterValue` :`self` (`self.MID_Body`) :`ParameterName` "MoveVector")
            (bind _output_get (set `self.BodyScale` 1.0))
            (`self.SetActorScale3D` (`KismetMathLibrary.MakeVector` _output_get _output_get _output_get))
            (set `self.bTurn1` false)
            (set `self.bTurn2` true)
            (`self.K2_SetActorRotation` (struct :`Yaw` 290.0))
            (`self.K2_SetActorLocation` (-1901.0 515.0 10.0))
            (goto _label :!via `Reset`)))))
    (:`then_1`
      (if (`self.bTurn2`)
        (`/Engine/EditorBlueprintResources/StandardMacros.DoOnce` false :!label _label_2
          (:`Completed`
            (`SkeletalMeshComponent.PlayAnimation` (`self.Mesh_Slime`) "/Game/Resource/CH/Slime/Anim/CH_MO_Slime_Walk.CH_MO_Slime_Walk" true) ; 走り出す
            (set `self.bRun` true)
            (`KismetSystemLibrary.Delay` 15.0)
            (set `self.bRun` false)
            (`SkeletalMeshComponent.PlayAnimation` (`self.Mesh_Slime`) "/Game/Resource/CH/Slime/Anim/CH_MO_Slime_Idle.CH_MO_Slime_Idle" true) ; 吸われ開始
            (`MaterialInstanceDynamic.SetVectorParameterValue` (`self.MID_Body`) "MoveVector" (`KismetMathLibrary.MakeColor` (.x (* (`self.GetActorForwardVector`) -1.0)) (.y (* (`self.GetActorForwardVector`) -1.0)) (+ (.z (* (`self.GetActorForwardVector`) -1.0)) 0.5)))
            (`KismetSystemLibrary.K2_SetTimer` null "SpawnSmallSlime_R" 0.2 true)
            (set `self.bDie` true)
            (`KismetSystemLibrary.Delay` 4.5)
            (`KismetSystemLibrary.K2_ClearTimer` null "SpawnSmallSlime_R")
            (`KismetSystemLibrary.Delay` 0.5) ; パターンBへ移行
            (set `self.bDie` false)
            (`KismetSystemLibrary.Delay` 4.0) ; パターンB開始
            (`MaterialInstanceDynamic.SetVectorParameterValue` :`self` (`self.MID_Body`) :`ParameterName` "MoveVector")
            (bind _output_get_2 (set `self.BodyScale` 1.0))
            (`self.SetActorScale3D` (`KismetMathLibrary.MakeVector` _output_get_2 _output_get_2 _output_get_2))
            (set `self.bTurn1` true)
            (set `self.bTurn2` false)
            (`self.K2_SetActorRotation` (struct :`Yaw` 110.0))
            (`self.K2_SetActorLocation` (-1469.0 -693.0 10.0))
            (goto _label_2 :!via `Reset`)))))
    (:`then_2`
      (if (`self.bRun`)
        (`self.K2_SetActorLocation` (+ (`self.K2_GetActorLocation`) (* (`self.GetActorForwardVector`) (* (`self.DeltaSec`) 50.0))))))
    (:`then_3`
      (if (`self.bDie`)
        (bind _output_get_3 (set `self.BodyScale` (- (`self.BodyScale`) (* (`self.DeltaSec`) 0.2))))
        (`self.SetActorScale3D` (`KismetMathLibrary.MakeVector` _output_get_3 _output_get_3 _output_get_3))))))

(fn `SpawnSmallSlime_L`
  (`|SpawnActorFromClass` "/Game/Blueprints/Slime/BP_TitleSlime_Small.BP_TitleSlime_Small_C" (`KismetMathLibrary.MakeTransform` (`self.K2_GetActorLocation`) (struct :`Pitch` 22.0 :`Yaw` 290.0)) "Undefined" "OverrideRootScale" null null))

(fn `SpawnSmallSlime_R`
  (`|SpawnActorFromClass` "/Game/Blueprints/Slime/BP_TitleSlime_Small.BP_TitleSlime_Small_C" (`KismetMathLibrary.MakeTransform` (`self.K2_GetActorLocation`) (struct :`Pitch` 22.0 :`Yaw` 110.0)) "Undefined" "OverrideRootScale" null null))

(fn `UserConstructionScript`)