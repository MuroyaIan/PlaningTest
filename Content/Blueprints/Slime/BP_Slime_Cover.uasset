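; A slime cover patch that follows a socket on the Golem and builds up as tagged slime bullets hit its sphere, which is enlarged for head patches.
; Hits first raise wetness; once fully wet, the patch spawns slime that further hits grow until hidden.
; Tick eases both values toward targets, writing wetness to the Golem's body material and size to its per-index bone scale array.
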(event `self.ReceiveBeginPlay`
  (`self.UpdateTransForm`)
  (`self.CheckIfSlimeInHead`)
  (set `self.TargetWetValue` 0.0) ; 濡れ具合初期化
  (set `self.TargetSlimeSize` 0.0) ; スライムサイズ初期化
  (add `/Game/Blueprints/Golem/BP_Golem.ResetSlimeCover` (`|ConvertAsset` (`self.Golem`)) (`|CreateDelegate` :!event `ResetSize`)))

(event `self.ReceiveTick`
  (params (DeltaSeconds :type "Float (single-precision)"))
  (set `self.DeltaSec` DeltaSeconds)
  (`self.UpdateTransForm`)
  (`self.UpdateWetFX`)
  (`self.UpdateSlimeSize`))

(event `self.BulletHit.OnComponentBeginOverlap`
  (params (OverlappedComponent :type "PrimitiveComponent Object Reference") (OtherActor :type "Actor Object Reference") (OtherComp :type "PrimitiveComponent Object Reference") (OtherBodyIndex :type Integer) (bFromSweep :type Boolean) (SweepResult :type "HitResult Structure (by ref)"))
  (bind _targetslimesize (`self.TargetSlimeSize`))
  (if (`ActorComponent.ComponentHasTag` OtherComp "BossHit")
    (if (not (`self.bHide`))
      (if (`self.bWet`)
        (if (< _targetslimesize 1.0)
          (set `self.TargetSlimeSize` (+ _targetslimesize 0.2)) ; サイズ増加
        )
        (else
          (set `self.TargetWetValue` (+ (`self.TargetWetValue`) 0.5)) ; 濡れ具合更新
          (if (>= (`self.WetValue`) 1.0)
            (set `self.bWet` true) ; 付着スライム発生
            (set `self.TargetSlimeSize` 0.6) ; スライムサイズ更新
          ))))))

(event `ResetSize`
  (bind _slimesize (`self.SlimeSize`))
  (if (> _slimesize 0.6)
    (set `self.SlimeSize` (`KismetMathLibrary.FInterpTo_Constant` _slimesize 0.8 (`self.DeltaSec`) 1.0)) ; サイズを縮小
    (set `self.TargetSlimeSize` 0.8)))

(fn `CheckIfSlimeInHead`
  (bind _slimeindex (`self.SlimeIndex`))
  (if (and (>= _slimeindex 14) (<= _slimeindex 18))
    (`SphereComponent.SetSphereRadius` (`self.BulletHit`) 225.0 true)))

(fn `HideSlime`
  (set `self.SlimeSize` 0.1)
  (set `self.TargetSlimeSize` 0.0)
  (set `self.bHide` true))

(fn `UpdateSlimeSize`
  (bind _slimesize (`self.SlimeSize`))
  (if (not (`KismetMathLibrary.NearlyEqual_FloatFloat` (`self.SlimeSize`) (`self.TargetSlimeSize`) 0.01))
    (set `self.SlimeSize` (`KismetMathLibrary.FInterpTo_Constant` (`self.SlimeSize`) (`self.TargetSlimeSize`) (`self.DeltaSec`) 1.0)) ; スライムサイズ更新
    (`KismetArrayLibrary.Array_Set` (`/Game/Blueprints/Golem/BP_Golem.SlimeScale` (`|ConvertAsset` (`self.Golem`))) (`self.SlimeIndex`) (`KismetMathLibrary.MakeVector` _slimesize _slimesize _slimesize)) ; ボーンサイズ更新
  ))

(fn `UpdateTransForm`
  (bind _golem (`self.Golem`))
  (if (`KismetSystemLibrary.IsValidSoftObjectReference` _golem)
    (`self.K2_SetActorLocation` (`SceneComponent.GetSocketLocation` (`Character.Mesh` (`|ConvertAsset` _golem)) (`self.SocketName`)))))

(fn `UpdateWetFX`
  (bind _output (`|ConvertAsset` (`self.Golem`)))
  (if (not (`KismetMathLibrary.NearlyEqual_FloatFloat` (`self.WetValue`) (`self.TargetWetValue`) 0.01))
    (set `self.WetValue` (`KismetMathLibrary.FInterpTo_Constant` (`self.WetValue`) (`self.TargetWetValue`) (`self.DeltaSec`) 1.0)) ; 濡れ具合更新
    (`/Game/Blueprints/Golem/BP_Golem.UpdateBodyMID` _output (`BlueprintMapLibrary.Map_Find` (`/Game/Blueprints/Golem/BP_Golem.Map_WetFX` _output) (`self.SlimeIndex`)) (`self.WetValue`)) ; マテリアル更新
  ))

(fn `UserConstructionScript`)