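; Destructible wall actor that shatters when an actor tagged "Golem" overlaps any of its three box triggers.
; CreateDestMesh removes the static mesh and boxes, then adds a destructible component and applies damage with an impulse along the golem's forward vector.
; After a delay, Tick fades the debris through a dynamic material's Opacity Mask parameter and destroys the actor once it reaches zero.
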(event `self.ReceiveBeginPlay`)

(event `self.ReceiveTick`
  (params (DeltaSeconds :type "Float (single-precision)"))
  (set `self.DeltaSec` DeltaSeconds)
  (if (`self.bStartDestroy`)
    (bind _output_get (set `self.MID_Opacity` (- (`self.MID_Opacity`) (* (`self.DeltaSec`) 0.25)))) ; 4秒で消える
    (`MaterialInstanceDynamic.SetScalarParameterValue` (`self.MID_DestMesh`) "Opacity Mask" _output_get) ; 透明度更新
    (if (<= (`self.MID_Opacity`) 0.0)
      (`self.K2_DestroyActor`))))

(event `self.Box_Origin.OnComponentBeginOverlap`
  (params (OverlappedComponent :type "PrimitiveComponent Object Reference") (OtherActor :type "Actor Object Reference") (OtherComp :type "PrimitiveComponent Object Reference") (OtherBodyIndex :type Integer) (bFromSweep :type Boolean) (SweepResult :type "HitResult Structure (by ref)"))
  (bind _actorisgolem (`self.CreateDestMesh` OtherActor))
  (if _actorisgolem
    (`KismetSystemLibrary.Delay` 5.0 :!label _label) ; 消滅処理
    (set `self.bStartDestroy` true)))

(event `self.Box_1.OnComponentBeginOverlap`
  (params (OverlappedComponent :type "PrimitiveComponent Object Reference") (OtherActor :type "Actor Object Reference") (OtherComp :type "PrimitiveComponent Object Reference") (OtherBodyIndex :type Integer) (bFromSweep :type Boolean) (SweepResult :type "HitResult Structure (by ref)"))
  (bind _actorisgolem (`self.CreateDestMesh` OtherActor))
  (if _actorisgolem
    (goto _label)))

(event `self.Box_2.OnComponentBeginOverlap`
  (params (OverlappedComponent :type "PrimitiveComponent Object Reference") (OtherActor :type "Actor Object Reference") (OtherComp :type "PrimitiveComponent Object Reference") (OtherBodyIndex :type Integer) (bFromSweep :type Boolean) (SweepResult :type "HitResult Structure (by ref)"))
  (bind _actorisgolem (`self.CreateDestMesh` OtherActor))
  (if _actorisgolem
    (goto _label)))

(fn `CreateDestMesh`
  (params (ActorRef :type "Actor Object Reference (by ref)"))
  (returns (ActorIsGolem :type Boolean))
  (bind _destpower (`self.DestPower`))
  (if (`self.ActorHasTag` ActorRef "Golem")
    (`ActorComponent.K2_DestroyComponent` (`self.StaticMesh`))
    (`self.DestroyBoxCollision`)
    (bind _returnvalue (`AddComponent|NODE_AddDestructibleComponent-0` :`RelativeTransform` (`KismetMathLibrary.MakeTransform` (0.0 0.0 -432.0)))) ; 破壊メッシュ置換
    (`DestructibleComponent.SetDestructibleMesh` _returnvalue (`self.DestMeshSlot`))
    (bind _returnvalue_2 (`PrimitiveComponent.CreateDynamicMaterialInstance` _returnvalue 0 (`PrimitiveComponent.GetMaterial` _returnvalue 0) "None"))
    (bind _output_get (set `self.MID_DestMesh` _returnvalue_2))
    (`MaterialInstanceDynamic.SetScalarParameterValue` _output_get "Opacity Mask" (`self.MID_Opacity`)) ; 透明度設定
    (`DestructibleComponent.ApplyDamage` _returnvalue _destpower (`KismetMathLibrary.MakeVector` (.x (`SceneComponent.K2_GetComponentLocation` _returnvalue)) (.y (`SceneComponent.K2_GetComponentLocation` _returnvalue)) (+ (.z (`SceneComponent.K2_GetComponentLocation` _returnvalue)) 82.0)) (`self.GetActorForwardVector` ActorRef) _destpower) ; ダメージ設定
    (return true)
    (else
      (return false))))

(fn `DestroyBoxCollision`
  (`ActorComponent.K2_DestroyComponent` (`self.Box_Origin`))
  (`ActorComponent.K2_DestroyComponent` (`self.Box_1`))
  (`ActorComponent.K2_DestroyComponent` (`self.Box_2`)))

(fn `UserConstructionScript`)