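; Blueprint function library of shared helpers for flattening vectors onto the XY plane and querying a debug-logging flag.
; Two vector functions zero out Z, one keeping the XY values and the other normalizing them.
; CheckDebugPrint casts the game instance to BP_GlobalData and returns its DebugLog flag, or false if the cast fails.
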(fn `CheckDebugPrint`
  (returns (bDebug :type Boolean))
  (bind _asbp_global_data (cast `/Game/Blueprints/System/BP_GlobalData` (`GameplayStatics.GetGameInstance` null))
    (:`then`
      (return (`/Game/Blueprints/System/BP_GlobalData.bDebugLog` _asbp_global_data)))
    (:`CastFailed`
      (return false))))

(fn `Vector to 2D(NormalizeXY)`
  (params (Vector :type "Vector Structure"))
  (returns (`Vector(XY)` :type "Vector Structure"))
  (return (`KismetMathLibrary.Conv_Vector2DToVector` (`KismetMathLibrary.Normal2D` (`KismetMathLibrary.Conv_VectorToVector2D` Vector)))))

(fn `Vector to 2D(XY)`
  (params (Vector :type "Vector Structure"))
  (returns (`Vector(XY)` :type "Vector Structure"))
  (return (`KismetMathLibrary.Conv_Vector2DToVector` (`KismetMathLibrary.Conv_VectorToVector2D` Vector))))