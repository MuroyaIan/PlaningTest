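; Title screen controller actor that sequences the startup logo, fade and title menu widgets and handles menu input.
; BeginPlay creates the widgets, adding the logo only when BP_GlobalData's OpenGame flag marks a fresh launch.
; Tick shows the fade, starts title BGM, then displays the title after a timer and enables input after its intro animation time.
; Button and stick events, gated by CanInput, drive selection, value changes, confirm and back.
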(event `self.ReceiveBeginPlay`
  (`self.EnableInput` (`GameplayStatics.GetPlayerController` 0)) ; 入力有効化
  (bind _returnvalue (`|CreateWidget` "/Game/Maps/TestMap/Kitayama/UI_Kitayama/Widget_UI/Title_Widget/UMG_Title.UMG_Title_C")) ; タイトルUI
  (set `self.TitleWidget` _returnvalue)
  (bind _returnvalue_2 (`|CreateWidget` "/Game/Blueprints/System/BP_UI/UMG_FadeOnly.UMG_FadeOnly_C")) ; フェードUI
  (set `self.FadeWidget` _returnvalue_2)
  (bind _asbp_global_data (cast `/Game/Blueprints/System/BP_GlobalData` (`GameplayStatics.GetGameInstance`)))
  (if (`/Game/Blueprints/System/BP_GlobalData.OpenGame` _asbp_global_data)
    (set `self.First` true)
    (bind _returnvalue_3 (`|CreateWidget` "/Game/Maps/TestMap/Kitayama/UI_Kitayama/Widget_UI/Title_Widget/UMG_StartLogo.UMG_StartLogo_C")) ; ロゴUI
    (bind _output_get (set `self.LogoWidget` _returnvalue_3))
    (`UserWidget.AddToViewport` _output_get 2)
    (else
      (set `self.First` false))))

(event `self.ReceiveTick`
  (params (DeltaSeconds :type "Float (single-precision)"))
  (`|ExecutionSequence`
    (:`then_0`
      (if (`self.First`)
        (if (`/Game/Maps/TestMap/Kitayama/UI_Kitayama/Widget_UI/Title_Widget/UMG_StartLogo.LogoAnimationEnd` (`self.LogoWidget`))
          (`/Engine/EditorBlueprintResources/StandardMacros.DoOnce` false
            (:`Completed`
              (`Widget.RemoveFromParent` (`self.LogoWidget`))
              (`UserWidget.AddToViewport` (`self.FadeWidget`) 1)
              (bind _asbp_global_data (cast `/Game/Blueprints/System/BP_GlobalData` (`GameplayStatics.GetGameInstance`)))
              (set `/Game/Blueprints/System/BP_GlobalData.OpenGame` false _asbp_global_data) ; ロゴ演出は一度だけ
              (set `self.FadeTimerOn` true)
              ;[1 1 1] BGM再生
              (bind _asbp_game_mode_title (cast `/Game/Blueprints/System/BP_GameMode_Title` (`GameplayStatics.GetGameMode`) :!label _label))
              (`/Game/Blueprints/System/BP_Audio.PlayBGM_Title` (`|ConvertAsset` (`/Game/Blueprints/System/BP_GameMode_Title.Actor_Audio` _asbp_game_mode_title))))))
        (else
          (`/Engine/EditorBlueprintResources/StandardMacros.DoOnce` false
            (:`Completed`
              (`UserWidget.AddToViewport` (`self.FadeWidget`) 1)
              (set `self.FadeTimerOn` true)
              (goto _label))))))
    (:`then_1`
      (if (`self.FadeTimerOn`)
        (bind _output_get (set `self.Timer` (+ (`self.Timer`) DeltaSeconds)))
        (if (>= _output_get (`self.FadeTime`))
          (set `self.FadeTimerOn` false)
          (set `self.Timer` 0.0)
          (set `self.TitleIn` true))))
    (:`then_2`
      (if (`self.TitleIn`)
        (`/Engine/EditorBlueprintResources/StandardMacros.DoOnce` false
          (:`Completed`
            (`UserWidget.AddToViewport` (`self.TitleWidget`) 0)
            (set `self.TitleIn` false)
            (set `self.TitleInEnd` true)))))
    (:`then_3`
      (if (`self.TitleInEnd`)
        (`KismetSystemLibrary.Delay` (`/Game/Maps/TestMap/Kitayama/UI_Kitayama/Widget_UI/Title_Widget/UMG_Title.InAnimTime` (`self.TitleWidget`)))
        (set `self.CanInput` true)))))

(event `InputAction|UI_Up`
  (params (Key :type "Key Structure"))
  (:`Pressed`
    (if (`self.CanInput`)
      (if (`self.First`)
        (if (`/Game/Maps/TestMap/Kitayama/UI_Kitayama/Widget_UI/Title_Widget/UMG_StartLogo.LogoAnimationEnd` (`self.LogoWidget`))
          (`/Game/Maps/TestMap/Kitayama/UI_Kitayama/Widget_UI/Title_Widget/UMG_Title.Select` (`self.TitleWidget`) false :!label _label))
        (else
          (goto _label))))))

(event `InputAction|Pause_Back`
  (params (Key :type "Key Structure"))
  (:`Pressed`
    (if (`self.CanInput`)
      (if (`self.First`)
        (if (`/Game/Maps/TestMap/Kitayama/UI_Kitayama/Widget_UI/Title_Widget/UMG_StartLogo.LogoAnimationEnd` (`self.LogoWidget`))
          (`/Game/Maps/TestMap/Kitayama/UI_Kitayama/Widget_UI/Title_Widget/UMG_Title.OptionBack` (`self.TitleWidget`) :!label _label_2)
          (`GameplayStatics.PlaySound2D` "/Game/Resource/SO/SE/UI/SO_SE_UI_Back_Cue.SO_SE_UI_Back_Cue" 1.0 1.0 0.0 null null) ; 効果音再生
        )
        (else
          (goto _label_2))))))

(event `InputAction|UI_Down`
  (params (Key :type "Key Structure"))
  (:`Pressed`
    (if (`self.CanInput`)
      (if (`self.First`)
        (if (`/Game/Maps/TestMap/Kitayama/UI_Kitayama/Widget_UI/Title_Widget/UMG_StartLogo.LogoAnimationEnd` (`self.LogoWidget`))
          (`/Game/Maps/TestMap/Kitayama/UI_Kitayama/Widget_UI/Title_Widget/UMG_Title.Select` (`self.TitleWidget`) true :!label _label_3))
        (else
          (goto _label_3))))))

(event `InputAction|UI_Confirm`
  (params (Key :type "Key Structure"))
  (:`Pressed`
    (if (`self.CanInput`)
      (if (`self.First`)
        (if (`/Game/Maps/TestMap/Kitayama/UI_Kitayama/Widget_UI/Title_Widget/UMG_StartLogo.LogoAnimationEnd` (`self.LogoWidget`))
          (`/Game/Maps/TestMap/Kitayama/UI_Kitayama/Widget_UI/Title_Widget/UMG_Title.ConfirmAction` (`self.TitleWidget`) :!label _label_4))
        (else
          (goto _label_4))))))

(event `InputAxis|UI_Stick_Y` :consume false :paused true
  (params (AxisValue :type "Float (single-precision)"))
  (bind _caninput (`self.CanInput`))
  (bind _titlewidget (`self.TitleWidget`))
  (bind _sticky (`self.StickY`))
  (bind _first (`self.First`))
  (bind _logoanimationend (`/Game/Maps/TestMap/Kitayama/UI_Kitayama/Widget_UI/Title_Widget/UMG_StartLogo.LogoAnimationEnd` (`self.LogoWidget`)))
  (if (> AxisValue _sticky)
    (`KismetSystemLibrary.Delay` 0.1)
    (if _caninput
      (if _first
        (if _logoanimationend
          (`/Game/Maps/TestMap/Kitayama/UI_Kitayama/Widget_UI/Title_Widget/UMG_Title.Select` _titlewidget false :!label _label_5))
        (else
          (goto _label_5))))
    (elif (< AxisValue (* _sticky -1.0))
      (`KismetSystemLibrary.Delay` 0.1)
      (if _caninput
        (if _first
          (if _logoanimationend
            (`/Game/Maps/TestMap/Kitayama/UI_Kitayama/Widget_UI/Title_Widget/UMG_Title.Select` _titlewidget true :!label _label_6))
          (else
            (goto _label_6)))))))

(event `InputAction|UI_Left`
  (params (Key :type "Key Structure"))
  (:`Pressed`
    (if (`self.CanInput`)
      (if (`self.First`)
        (if (`/Game/Maps/TestMap/Kitayama/UI_Kitayama/Widget_UI/Title_Widget/UMG_StartLogo.LogoAnimationEnd` (`self.LogoWidget`))
          (`/Game/Maps/TestMap/Kitayama/UI_Kitayama/Widget_UI/Title_Widget/UMG_Title.SetVal` (`self.TitleWidget`) false :!label _label_7))
        (else
          (goto _label_7))))))

(event `InputAction|UI_Right`
  (params (Key :type "Key Structure"))
  (:`Pressed`
    (if (`self.CanInput`)
      (if (`self.First`)
        (if (`/Game/Maps/TestMap/Kitayama/UI_Kitayama/Widget_UI/Title_Widget/UMG_StartLogo.LogoAnimationEnd` (`self.LogoWidget`))
          (`/Game/Maps/TestMap/Kitayama/UI_Kitayama/Widget_UI/Title_Widget/UMG_Title.SetVal` (`self.TitleWidget`) true :!label _label_8))
        (else
          (goto _label_8))))))

(event `InputAxis|UI_Stick_X` :consume false :paused true
  (params (AxisValue :type "Float (single-precision)"))
  (bind _first (`self.First`))
  (bind _titlewidget (`self.TitleWidget`))
  (bind _logoanimationend (`/Game/Maps/TestMap/Kitayama/UI_Kitayama/Widget_UI/Title_Widget/UMG_StartLogo.LogoAnimationEnd` (`self.LogoWidget`)))
  (if (> AxisValue (`self.StickX`))
    (`KismetSystemLibrary.Delay` 0.2)
    (if (`self.CanInput`)
      (if _first
        (if _logoanimationend
          (`/Game/Maps/TestMap/Kitayama/UI_Kitayama/Widget_UI/Title_Widget/UMG_Title.SetVal` _titlewidget true :!label _label_9))
        (else
          (goto _label_9))))
    (elif (< AxisValue (* (`self.StickX`) -1.0))
      (`KismetSystemLibrary.Delay` 0.2)
      (if (`self.CanInput`)
        (if _first
          (if _logoanimationend
            (`/Game/Maps/TestMap/Kitayama/UI_Kitayama/Widget_UI/Title_Widget/UMG_Title.SetVal` _titlewidget false :!label _label_10))
          (else
            (goto _label_10)))))))

(fn `UserConstructionScript`)