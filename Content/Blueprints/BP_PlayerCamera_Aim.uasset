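; BP_PlayerCamera_Aim is an actor that keeps itself just in front of the player in the camera's horizontal facing direction, apparently as an aim camera reference point.
; On BeginPlay and every Tick, SetLoaction adds a fixed-distance offset to the BP_Player location, built from the BP_PlayerCameraManager forward vector passed through VectorTo2DNormalizeXY.
; The move is a direct SetActorLocation without sweep, and rotation is left untouched.
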(event `self.ReceiveBeginPlay`
  (`self.SetLoaction`))

(event `self.ReceiveTick`
  (params (DeltaSeconds :type "Float (single-precision)"))
  (`self.SetLoaction`))

(fn `SetLoaction`
  (`self.K2_SetActorLocation` (+ (`self.K2_GetActorLocation` (cast `/Game/Blueprints/BP_Player` (`GameplayStatics.GetPlayerPawn` 0) :!pure true)) (* (`/Game/Blueprints/BP_FuncLibrary.Vector to 2D(NormalizeXY)` (`/Game/Blueprints/System/BP_PlayerCameraManager.GetForwardVector` (cast `/Game/Blueprints/System/BP_PlayerCameraManager` (`GameplayStatics.GetPlayerCameraManager` 0) :!pure true))) 100))))

(fn `UserConstructionScript`)