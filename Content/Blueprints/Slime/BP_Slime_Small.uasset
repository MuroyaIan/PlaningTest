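; Small slime actor that is either sucked into the player's weapon or fired as a projectile.
; By default it spawns offset by parent slime size, drifts toward the weapon nozzle, then fires a sucked event and destroys itself on overlap.
; Bullet mode launches it forward with delayed gravity; near-zero velocity counts as landing, triggering hit VFX, BossHit collision and timed removal.
; Actor rotation follows movement, feeding a dynamic material's direction parameter.
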(event `self.ReceiveBeginPlay`
  (bind _staticmesh (`self.StaticMesh`))
  (`|ExecutionSequence`
    (:`then_0`
      ;[0.2708 0.2708 0.2708] 初期化Part1
      ;;[0.4166 0.9901 1] プレイヤーの参照取得
      (bind _asbp_player_controller (cast `/Game/Blueprints/Player/BP_PlayerController` (`GameplayStatics.GetPlayerController` 0)))
      (set `self.PlayerRef` (`|ConvertAsset` (`/Game/Blueprints/Player/BP_PlayerController.GetPlayerPawn` _asbp_player_controller))))
    (:`then_1`
      ;;[1 1 1] 重力無効化(もっといい方法知りたい)
      (`ActorComponent.Deactivate` (`self.CharacterMovement`))
      (`ActorComponent.Deactivate` (`self.ProjectileMovement`)))
    (:`then_2`
      ;;[0.2471 0.9059 0.2] マテリアルインスタンス生成
      (bind _returnvalue (`PrimitiveComponent.CreateDynamicMaterialInstance` _staticmesh 0 (`PrimitiveComponent.GetMaterial` _staticmesh 0) "None"))
      (bind _output_get (set `self.MID` _returnvalue))
      ;;[0.2471 0.9059 0.2] パラメータの初期化
      (`MaterialInstanceDynamic.SetVectorParameterValue` _output_get "Step" (make `LinearColor` -1.0 0.0 0.0 1.0))
      (`MaterialInstanceDynamic.SetScalarParameterValue` _output_get "Extend" 50.0)
      ;;[1 1 1] 向き調整用
      (set `self.Pos_Backup` (`self.K2_GetActorLocation`)) ; 自分の位置を記憶
    )
    (:`then_3`
      ;;[0.1314 0.9203 1] 付着処理用コリジョン初期化
      (`PrimitiveComponent.SetCollisionEnabled` (`self.BossHit`) "NoCollision"))))

(event `self.ReceiveTick`
  (params (DeltaSeconds :type "Float (single-precision)"))
  (`|ExecutionSequence`
    (:`then_0`
      ;[0.3125 0.3125 0.3125] 初期化Part2
      (`/Engine/EditorBlueprintResources/StandardMacros.DoOnce` false
        (:`Completed`
          (`|ExecutionSequence`
            (:`then_0`
              ;;[0.3955 0.9801 1] 武器の参照取得
              (set `self.WeaponRef` (`|ConvertAsset` (`/Game/Blueprints/Player/BP_Player.GetWeapon` (`|ConvertAsset` (`self.PlayerRef`)))))
              ;;[0.2599 0.2366 1] イベントバインド
              (add `self.ED_Sucked` (`|CreateDelegate` (`/Game/Blueprints/Player/BP_Player.GetWeapon` (`|ConvertAsset` (`self.PlayerRef`))) :!event `AddSlime`)))
            (:`then_1`
              ;;[0.2507 0.3647 1] スポーン位置のオフセット
              (if (not (`self.IsBullet`))
                (`self.K2_AddActorWorldOffset` (`KismetMathLibrary.MakeVector` 0.0 0.0 (`self.GetSpawnOffset`)))))))))
    (:`then_1`
      ;[0.349 0.349 0.349] 更新
      (if (not (`self.IsBullet`))
        ;;[0.3969 1 0.3036] 武器の方に近づく
        (bind _output_get (set `self.PlayerDir` (`self.Get Wpeapon Direction Normalized`)))
        (`self.K2_AddActorWorldOffset` (* _output_get (* (`self.Speed`) DeltaSeconds)))
        (`self.K2_AddActorWorldOffset` (`KismetMathLibrary.MakeVector` 0.0 0.0 (* (`self.ZIncrementValue`) DeltaSeconds)))
        ;;[0.2471 0.9059 0.2] マテリアルインスタンスのパラメータ更新
        (`self.SetDirection`)
        (`self.MIDSetVectorParameterNegatived` (`self.GetActorForwardVector`))
        (else
          ;;[0.2471 0.9059 0.2] マテリアルインスタンスのパラメータ更新
          (`self.SetDirection`)
          (`self.MIDSetVectorParameterNegatived` (`self.GetActorForwardVector`))
          ;;[1 0.4695 0.8533] 接地したか?(速度が小さい==接地したとみなす)
          (if (< (`KismetMathLibrary.VSize` (`MovementComponent.Velocity` (`self.ProjectileMovement`))) 5.0)
            (`/Engine/EditorBlueprintResources/StandardMacros.DoOnce` false
              (:`Completed`
                (`self.SetLifeSpan` 1.0) ; 3秒後に消す
                (`SceneComponent.SetHiddenInGame` (`self.StaticMesh`) true false)
                (`ActorComponent.Activate` (`self.FX_VFX_PlayerHit`) false) ; ヒットエフェクト再生
                (`PrimitiveComponent.SetCollisionEnabled` (`self.BossHit`) "QueryAndPhysics") ; 付着処理用コリジョン起動
              ))))))))

(event `self.StaticMesh.OnComponentBeginOverlap`
  (params (OverlappedComponent :type "PrimitiveComponent Object Reference") (OtherActor :type "Actor Object Reference") (OtherComp :type "PrimitiveComponent Object Reference") (OtherBodyIndex :type Integer) (bFromSweep :type Boolean) (SweepResult :type "HitResult Structure (by ref)"))
  ;[1 0.8884 0.25] 武器に吸い込まれた(完全に)
  (if (`self.IsBullet`)
    _
    (elif (`self.ActorHasTag` OtherActor "Weapon")
      (`self.ED_Sucked`)
      (`self.K2_DestroyActor`))))

(event `SetToBullet`
  (bind _projectilemovement (`self.ProjectileMovement`))
  ;[1 0.4819 0.4121] 弾モードにする
  (set `self.IsBullet` true)
  (`ActorComponent.Activate` _projectilemovement true)
  (set `ProjectileMovementComponent.ProjectileGravityScale` 0.0 _projectilemovement)
  (bind _output_get (set `MovementComponent.Velocity` (* (`self.GetActorForwardVector`) (`self.Bullet Initial Speed`)) _projectilemovement))
  (`self.K2_SetActorLocation` (- (`self.K2_GetActorLocation`) (* _output_get (`GameplayStatics.GetWorldDeltaSeconds`)))) ; 変な位置にスポーンするのでわざとずらす
  (`KismetSystemLibrary.K2_SetTimerDelegate` (delegate `EnableProjectileGravity`) (`self.TimeEnableGravity`))
  ;;[0.2471 0.9059 0.2] マテリアルインスタンスのパラメータ初期化
  (`self.MIDSetVectorParameterNegatived` (`self.GetActorForwardVector`)))

(event `EnableProjectileGravity`
  ;[1 1 1] 重力をかける
  (set `ProjectileMovementComponent.ProjectileGravityScale` 1.0 (`self.ProjectileMovement`)))

(fn `Get Wpeapon Direction Normalized`
  (returns (`Dir Normalized` :type "Vector Structure"))
  (return (`KismetMathLibrary.Normal` (- (`SceneComponent.K2_GetComponentLocation` (`|GetArrayItem` (`self.K2_GetComponentsByClass` (`|ConvertAsset` (`self.WeaponRef`)) "/Script/Engine.StaticMeshComponent") 1)) (`self.K2_GetActorLocation`)))))

(fn `GetSlimeSize`
  (returns (SlimeSize :type Integer))
  (return (`/Game/Maps/TestMap/Nishino/Enemy_SlimeDefault/BP_SlimeDefault.SlimeSize` (`|ConvertAsset` (`self.ParentSlime`)))))

(fn `GetSpawnOffset`
  (returns (`Return Value` :type "Float (double-precision)"))
  (return (`|GetArrayItem` (`self.SpawnZOffset`) (- (/ (`self.GetSlimeSize`) 2) 1))))

(fn `MIDSetVectorParameterNegatived`
  (params (VectorParameter :type "Vector Structure"))
  (`MaterialInstanceDynamic.SetVectorParameterValue` (`self.MID`) "MoveDir" (make `LinearColor` (.x (* VectorParameter -1.0)) (.y (* VectorParameter -1.0)) (.z (* VectorParameter -1.0)) 1.0)))

(fn `SetDirection`
  (bind _returnvalue (`self.K2_GetActorLocation`))
  (bind _pos_backup (`self.Pos_Backup`))
  (if (`KismetMathLibrary.NotEqualExactly_VectorVector` _pos_backup _returnvalue)
    (`self.K2_SetActorRotation` (`KismetMathLibrary.FindLookAtRotation` _pos_backup _returnvalue)) ; 向き修正
    (set `self.Pos_Backup` _returnvalue) ; バックアップ更新
  ))

(fn `UserConstructionScript`)