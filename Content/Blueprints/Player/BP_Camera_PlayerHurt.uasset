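; Hurt-reaction camera actor that registers itself as CameraHurt on BP_Player at BeginPlay.
; While TargetHurtOffset is non-zero, each tick places it at the camera manager's POV, shifted along the player's forward vector by HurtOffset.
; Its rotation follows the line from the unshifted POV to the gaze point derived from the player's location.
; HurtOffset moves toward its target at constant CameraSpeed every tick.
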(event `self.ReceiveBeginPlay`
  (bind _asbp_player (cast `/Game/Blueprints/Player/BP_Player` (`GameplayStatics.GetPlayerPawn` 0)))
  (set `/Game/Blueprints/Player/BP_Player.Camera_Hurt` (`|ConvertAsset` self) _asbp_player) ; 参照を格納
)

(event `self.ReceiveTick`
  (params (DeltaSeconds :type "Float (single-precision)"))
  (set `self.DeltaSec` DeltaSeconds)
  (`self.UpdateLocation`)
  (`self.UpdateCamera`))

(event `UpdateCamera`
  (set `self.HurtOffset` (`KismetMathLibrary.FInterpTo_Constant` (`self.HurtOffset`) (`self.TargetHurtOffset`) (`self.DeltaSec`) (`self.CameraSpeed`))))

(fn `UpdateLocation`
  (if (!= (`self.TargetHurtOffset`) 0.0)
    (bind _asbp_player_controller (cast `/Game/Blueprints/Player/BP_PlayerController` (`GameplayStatics.GetPlayerController` 0)))
    (bind _cameramanager (`/Game/Blueprints/Player/BP_PlayerController.GetCameraManager` _asbp_player_controller))
    (bind _playerpawn (`/Game/Blueprints/Player/BP_PlayerController.GetPlayerPawn` _asbp_player_controller))
    (bind _gazepoint (`/Game/Blueprints/Player/BP_PlayerCameraManager.SetGazePoint` _cameramanager (`self.K2_GetActorLocation` _playerpawn)))
    (bind _pov (`/Game/Blueprints/Player/BP_PlayerCameraManager.SetPOV` _cameramanager _gazepoint))
    (`self.K2_SetActorLocation` (+ _pov (* (`self.GetActorForwardVector` _playerpawn) (`self.HurtOffset`))))
    (`self.K2_SetActorRotation` (`KismetMathLibrary.FindLookAtRotation` _pov _gazepoint))))

(fn `UserConstructionScript`)