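; BP_Camera_KillBoss02 is one shot in the boss-kill camera sequence, idle until its Start flag is set.
; It fixes a camera position and gaze point once from the player's transform.
; Each tick it applies that framing, eases FOV toward a target and triggers camera shake.
; After a delay it switches the view to NextCamera, starts BP_Camera_KillBoss03 and stops itself and the shake.
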(event `self.ReceiveBeginPlay`)

(event `self.ReceiveTick`
  (params (DeltaSeconds :type "Float (single-precision)"))
  (bind _campos (`self.CamPos`))
  (bind _nextcamera (`self.NextCamera`))
  (set `self.DeltaSec` DeltaSeconds)
  (if (`self.bStart`)
    (bind _asbp_player (cast `/Game/Blueprints/Player/BP_Player` (`GameplayStatics.GetPlayerPawn` 0)))
    (`|ExecutionSequence`
      (:`then_0`
        (`/Engine/EditorBlueprintResources/StandardMacros.DoOnce` false
          (:`Completed`
            (bind _returnvalue (`self.GetActorForwardVector` _asbp_player))
            (bind _returnvalue_2 (`self.GetActorUpVector` _asbp_player))
            (bind _returnvalue_3 (`self.K2_GetActorLocation` _asbp_player))
            (set `self.CamPos` (+ (`KismetMathLibrary.GreaterGreater_VectorRotator` (* _returnvalue 550.0) (struct :`Yaw` 120.0)) (* _returnvalue_2 30.0) _returnvalue_3)) ; 視点初期化
            (set `self.GazePoint` (+ (+ (* _returnvalue_2 270.0) _returnvalue_3) (* _returnvalue 500.0))) ; 注視点初期化
            (`KismetSystemLibrary.Delay` 4.2) ; カメラ切替
            (`PlayerController.SetViewTargetWithBlend` (`GameplayStatics.GetPlayerController` 0) _nextcamera 0.0 "VTBlend_Linear" 0.0 false) ; メインカメラ切替
            (bind _asbp_camera_kill_boss_03 (cast `/Game/Blueprints/Player/Camera/SuckAction/BP_Camera_KillBoss03` _nextcamera))
            (set `/Game/Blueprints/Player/Camera/SuckAction/BP_Camera_KillBoss03.bStart` true _asbp_camera_kill_boss_03)
            (set `self.bStart` false)
            (`PlayerController.ClientStopCameraShake` (`GameplayStatics.GetPlayerController` 0) "/Game/Blueprints/Player/Camera/Shake/BP_Shake_KillBoss2.BP_Shake_KillBoss2_C" true))))
      (:`then_1`
        (`self.K2_SetActorLocation` _campos) ; カメラ更新
        (`self.K2_SetActorRotation` (`KismetMathLibrary.FindLookAtRotation` _campos (`self.GazePoint`)))
        (bind _output_get (set `self.FOV` (`KismetMathLibrary.FInterpTo_Constant` (`self.FOV`) 90.0 (`self.DeltaSec`) 2.0)))
        (`CameraComponent.SetFieldOfView` (`self.CameraComponent`) _output_get) ; ズームイン
        (`PlayerController.ClientStartCameraShake` :`self` (`GameplayStatics.GetPlayerController` 0) :`Shake` "/Game/Blueprints/Player/Camera/Shake/BP_Shake_KillBoss2.BP_Shake_KillBoss2_C")))))

(fn `UserConstructionScript`)