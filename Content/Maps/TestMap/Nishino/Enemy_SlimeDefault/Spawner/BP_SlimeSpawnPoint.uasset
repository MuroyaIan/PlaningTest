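; Slime enemy spawn point that creates and tracks a capped number of BP_SlimeDefault actors.
; IsActive checks player distance band, cooldown and cap, while SlimeSpawn, not called within this Blueprint, spawns a slime, applies stats with random size and starts the cooldown.
; Tick prunes destroyed slimes, clears the cooldown through a Delay and recolors a cone to show player distance or cooldown state.
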(event `カスタムイベント_0`
  (bind _cone (`self.Cone`))
  (bind _returnvalue (`self.GetDistanceTo` (`GameplayStatics.GetPlayerPawn` 0) self))
  (if (< (`self.NearDistance`) _returnvalue)
    (if (< _returnvalue (`self.FarDistance`))
      (`PrimitiveComponent.SetMaterial` _cone 0 "/AnimationSharing/AnimSharingGreen.AnimSharingGreen") ; ちょうどいい
      (else
        (`PrimitiveComponent.SetMaterial` _cone 0 "/AnimationSharing/AnimSharingBlue.AnimSharingBlue") ; とおい
      ))
    (else
      (`PrimitiveComponent.SetMaterial` (`self.Cone`) 0 "/AnimationSharing/AnimSharingRed.AnimSharingRed") ; 近い
    ))
  (if (`self.SpawnCooltimeFlg`)
    (`PrimitiveComponent.SetMaterial` (`self.Cone`) 0 "/DatasmithContent/Materials/AliasMaster.AliasMaster") ; じかん
    (if true
      _)))

(event `self.ReceiveTick`
  (params (DeltaSeconds :type "Float (single-precision)"))
  ;[1 0 0] tick
  (`self.Chack_Slime`)
  (`self.Chack_Cooltime`)
  (`self.カスタムイベント_0`))

(event `Chack_Slime`
  (bind _slime (`self.Slime`))
  ;[0 1 0] スライムの状態確認
  (for _array_element _slime
    (`/Engine/EditorBlueprintResources/StandardMacros.IsValid` _array_element
      (:`Is Not Valid`
        (`KismetArrayLibrary.Array_RemoveItem` _slime _array_element)))))

(event `Chack_Cooltime`
  ;[1 1 0] クールタイムの確認
  (if (`self.SpawnCooltimeFlg`)
    (`KismetSystemLibrary.Delay` (`self.SpawnCooltime`))
    (set `self.SpawnCooltimeFlg` false)))

(fn `Is Active`
  (returns (Active :type Boolean))
  (bind _returnvalue (`self.GetDistanceTo` (`GameplayStatics.GetPlayerPawn` 0) self))
  (return (and (< (`self.NearDistance`) _returnvalue) (< _returnvalue (`self.FarDistance`)) (not (`self.SpawnCooltimeFlg`)) (< (`KismetArrayLibrary.Array_Length` (`self.Slime`)) (`self.SpawnMaxNum`)))))

(fn `Slime Spawn`
  (returns (Success :type Boolean) (Slime :type "/Game/Maps/TestMap/Nishino/Enemy_SlimeDefault/BP_SlimeDefault Object Reference"))
  (if (< (`KismetArrayLibrary.Array_Length` (`self.Slime`)) (`self.SpawnMaxNum`))
    (bind _returnvalue (`|SpawnActorFromClass` "/Game/Maps/TestMap/Nishino/Enemy_SlimeDefault/BP_SlimeDefault.BP_SlimeDefault_C" (`self.MakeTransform`) "Undefined" "OverrideRootScale" null null)) ; スライム作成
    (`/Engine/EditorBlueprintResources/StandardMacros.IsValid` _returnvalue ; 使用可能か確認
      (:`Is Valid`
        (`Pawn.SpawnDefaultController` _returnvalue) ; 一応設定
        (`/Game/Maps/TestMap/Nishino/Enemy_SlimeDefault/BP_SlimeDefault.SetStatus` _returnvalue (`self.Hitpoint`) (`self.Damage`) (`self.SpawnTime`) (`KismetMathLibrary.RandomIntegerInRange` 3 5) (`self.SlimeDestroyDistance`)) ; ステータス設定
        (`KismetArrayLibrary.Array_Add` (`self.Slime`) _returnvalue)
        (set `self.SpawnCooltimeFlg` true)
        (return true _returnvalue) ; 出現成功
      )
      (:`Is Not Valid`
        (return false null) ; 出現失敗
      ))
    (else
      (return false null) ; 出現上限
    )))

(fn `UserConstructionScript`)