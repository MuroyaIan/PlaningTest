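; Short-lived small slime actor, named for the title screen, that flies straight along its forward vector and then destroys itself.
; BeginPlay creates a dynamic material on the slime mesh and sets its Step and Extend parameters.
; Tick moves the actor at constant speed without sweep, while a one-time branch feeds the reversed forward vector to the material's MoveDir, briefly delays unhiding the mesh, then destroys the actor shortly afterward.
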(event `self.ReceiveBeginPlay`
  (bind _sm_slimesmall (`self.SM_SlimeSmall`))
  (bind _returnvalue (`PrimitiveComponent.CreateDynamicMaterialInstance` _sm_slimesmall 0 (`PrimitiveComponent.GetMaterial` _sm_slimesmall 0) "None"))
  (bind _output_get (set `self.MID` _returnvalue))
  (`MaterialInstanceDynamic.SetVectorParameterValue` _output_get "Step" (make `LinearColor` -1.0 0.0 0.0 1.0))
  (`MaterialInstanceDynamic.SetScalarParameterValue` _output_get "Extend" 50.0))

(event `self.ReceiveTick`
  (params (DeltaSeconds :type "Float (single-precision)"))
  (set `self.DeltaSec` DeltaSeconds)
  (`|ExecutionSequence`
    (:`then_0`
      (`/Engine/EditorBlueprintResources/StandardMacros.DoOnce` false
        (:`Completed`
          (`MaterialInstanceDynamic.SetVectorParameterValue` (`self.MID`) "MoveDir" (make `LinearColor` (.x (* (`self.GetActorForwardVector`) -1.0)) (.y (* (`self.GetActorForwardVector`) -1.0)) (.z (* (`self.GetActorForwardVector`) -1.0)) 1.0))
          (`KismetSystemLibrary.Delay` 0.1)
          (`SceneComponent.SetHiddenInGame` (`self.SM_SlimeSmall`) false false)
          (`KismetSystemLibrary.Delay` 0.3)
          (`self.K2_DestroyActor`))))
    (:`then_1`
      (`self.K2_SetActorLocation` (+ (`self.K2_GetActorLocation`) (* (`self.GetActorForwardVector`) (* (`self.DeltaSec`) 500.0)))))))

(fn `UserConstructionScript`)