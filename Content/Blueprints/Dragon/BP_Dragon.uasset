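; BP_Dragon is a three-form dragon enemy that attacks the player with bite, tackle and breath.
; A named flag map records the current form and attacks requested by trigger overlaps, while separate hitboxes, disabled at BeginPlay, apply damage.
; BeginPlay spawns slime cover actors assigned to joint names, with a scale map used to check first-stage slime completion.
; Dynamic body and crystal materials take parameter updates according to form.
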(event `self.ReceiveBeginPlay`
  (`self.Initialize Collider`)
  (`self.InitializeSlime`)
  (`self.InitializeMaterial`))

(event `self.ReceiveTick`
  (params (DeltaSeconds :type "Float (single-precision)"))
  (if (`self.DebugFlag`)
    (`self.PrintDebugInfo`)
    (bind _1ststagedone (`self.Check1stSlime`))
    (if _1ststagedone
      (`KismetSystemLibrary.PrintString` "1stFormEnded" true true (struct :`G` 0.66 :`B` 1.0 :`A` 1.0) 0.0))))

(event `SwitchTo2ndForm`
  ;[1 0.3535 0.3125] 2段階目に移行
  (`self.SetFlag` "secondform" true)
  (`self.SetFlag` "firstform")
  (`self.SetFlag` "thirdform")
  (`SceneComponent.K2_SetRelativeLocation` (`self.Mesh`) (0.0 0.0 140.0) false false))

(event `SwitchTo3rdForm`
  ;[0.133 1 0.2084] 3段階目に移行
  (`self.SetFlag` "thirdform" true)
  (`self.SetFlag` "firstform")
  (`self.SetFlag` "secondform"))

(event `DoBreathA`
  (`|SpawnActorFromClass` "/Game/Blueprints/Dragon/BP_Dragon_BreathA.BP_Dragon_BreathA_C" (`KismetMathLibrary.MakeTransform` (`SceneComponent.GetSocketLocation` (`self.Mesh`) "JNT_mouth_C0_teethlow") (`self.K2_GetActorRotation`)) "Undefined" "OverrideRootScale" null 3000.0 -1.0 null))

(event `self.BiteTrigger.OnComponentBeginOverlap`
  (params (OverlappedComponent :type "PrimitiveComponent Object Reference") (OtherActor :type "Actor Object Reference") (OtherComp :type "PrimitiveComponent Object Reference") (OtherBodyIndex :type Integer) (bFromSweep :type Boolean) (SweepResult :type "HitResult Structure (by ref)"))
  (cast `/Game/Blueprints/Player/BP_Player` OtherActor)
  (`self.SetFlag` "bite" true))

(event `self.BiteAtk.OnComponentBeginOverlap`
  (params (OverlappedComponent :type "PrimitiveComponent Object Reference") (OtherActor :type "Actor Object Reference") (OtherComp :type "PrimitiveComponent Object Reference") (OtherBodyIndex :type Integer) (bFromSweep :type Boolean) (SweepResult :type "HitResult Structure (by ref)"))
  (bind _asbp_player (cast `/Game/Blueprints/Player/BP_Player` OtherActor))
  (`GameplayStatics.ApplyDamage` _asbp_player 2.0))

(event `self.TackleTriggerR.OnComponentBeginOverlap`
  (params (OverlappedComponent :type "PrimitiveComponent Object Reference") (OtherActor :type "Actor Object Reference") (OtherComp :type "PrimitiveComponent Object Reference") (OtherBodyIndex :type Integer) (bFromSweep :type Boolean) (SweepResult :type "HitResult Structure (by ref)"))
  (cast `/Game/Blueprints/Player/BP_Player` OtherActor)
  (`self.SetFlag` "tackleAR" true))

(event `self.TackleTriggerL.OnComponentBeginOverlap`
  (params (OverlappedComponent :type "PrimitiveComponent Object Reference") (OtherActor :type "Actor Object Reference") (OtherComp :type "PrimitiveComponent Object Reference") (OtherBodyIndex :type Integer) (bFromSweep :type Boolean) (SweepResult :type "HitResult Structure (by ref)"))
  (cast `/Game/Blueprints/Player/BP_Player` OtherActor)
  (`self.SetFlag` "tackleAL" true))

(event `self.TackleAtkL.OnComponentBeginOverlap`
  (params (OverlappedComponent :type "PrimitiveComponent Object Reference") (OtherActor :type "Actor Object Reference") (OtherComp :type "PrimitiveComponent Object Reference") (OtherBodyIndex :type Integer) (bFromSweep :type Boolean) (SweepResult :type "HitResult Structure (by ref)"))
  (bind _asbp_player (cast `/Game/Blueprints/Player/BP_Player` OtherActor))
  (`GameplayStatics.ApplyDamage` _asbp_player 1.0))

(event `self.TackleAtkR.OnComponentBeginOverlap`
  (params (OverlappedComponent :type "PrimitiveComponent Object Reference") (OtherActor :type "Actor Object Reference") (OtherComp :type "PrimitiveComponent Object Reference") (OtherBodyIndex :type Integer) (bFromSweep :type Boolean) (SweepResult :type "HitResult Structure (by ref)"))
  (bind _asbp_player (cast `/Game/Blueprints/Player/BP_Player` OtherActor))
  (`GameplayStatics.ApplyDamage` _asbp_player 1.0))

(fn `Check1stSlime`
  (returns (`1stStageDone` :type Boolean))
  (locals (Success :type "Array of Boolean"))
  (bind _values (`BlueprintMapLibrary.Map_Values` (`self.SlimeScale`)))
  (for (_array_element _array_index) _values
    (if (>= _array_index (`self.NumOf1stSlime`))
      (break)
      (elif (>= (.x _array_element) 1.0)
        (`KismetArrayLibrary.Array_Add` (`local.Success`) true)
        (else
          (break)))))
  (return (== (`KismetArrayLibrary.Array_Length` (`local.Success`)) (`self.NumOf1stSlime`))))

(fn `Decl1stSlimeScale`
  (for _array_element (`self.SlimeCover`)
    (if (== (`/Game/Blueprints/Dragon/BP_Dragon_SlimeCover.form` _array_element) 1)
      (set `/Game/Blueprints/Dragon/BP_Dragon_SlimeCover.TargetSlimeSize` 0.4 _array_element))))

(fn `GetFlag`
  (params (Name :type Name))
  (returns (`return flag` :type Boolean))
  (bind (_value _returnvalue) (`BlueprintMapLibrary.Map_Find` (`self.Flags`) Name))
  (if _returnvalue
    (return _value)
    (else
      (return false))))

(fn `Initialize Collider`
  (bind _returnvalue (not (`self.DebugFlag`)))
  (`|ExecutionSequence`
    (:`then_0`
      ;[0.4323 0.12 0.1148] デバッグ表示
      (`SceneComponent.SetHiddenInGame` (`self.TackleTriggerR`) _returnvalue false)
      (`SceneComponent.SetHiddenInGame` (`self.TackleTriggerL`) _returnvalue false)
      (`SceneComponent.SetHiddenInGame` (`self.BiteTrigger`) _returnvalue false)
      (`SceneComponent.SetHiddenInGame` (`self.BiteAtk`) _returnvalue false)
      (`SceneComponent.SetHiddenInGame` (`self.TackleAtkR`) _returnvalue false)
      (`SceneComponent.SetHiddenInGame` (`self.TackleAtkL`) _returnvalue false))
    (:`then_1`
      ;[0.3854 1 0.6929] 攻撃判定無効化
      (`PrimitiveComponent.SetCollisionEnabled` (`self.BiteAtk`) "NoCollision")
      (`PrimitiveComponent.SetCollisionEnabled` (`self.TackleAtkR`) "NoCollision")
      (`PrimitiveComponent.SetCollisionEnabled` (`self.TackleAtkL`) "NoCollision"))))

(fn `InitializeMaterial`
  (bind _mesh (`self.Mesh`))
  (bind _returnvalue (`PrimitiveComponent.CreateDynamicMaterialInstance` _mesh 3 "/Game/Resource/CH/Dragon/IM/CH_IM_DragonBody2nd.CH_IM_DragonBody2nd" "None"))
  (set `self.IM_Body2nd` _returnvalue)
  (`PrimitiveComponent.CreateDynamicMaterialInstance` _mesh 3 "/Game/Resource/CH/Dragon/IM/CH_IM_DragonBody1st.CH_IM_DragonBody1st" "None")
  (bind _returnvalue_2 (`PrimitiveComponent.CreateDynamicMaterialInstance` _mesh 9 "/Game/Resource/CH/Dragon/IM/CH_IM_DragonCrystal.CH_IM_DragonCrystal" "None"))
  (set `self.IM_Crystal` _returnvalue_2))

(fn `InitializeSlime`
  (`|ExecutionSequence`
    (:`then_0`
      (bind _keys (`BlueprintMapLibrary.Map_Keys` (`self.SlimeScale`)))
      (for _index (range 23)
        (bind _returnvalue (`|SpawnActorFromClass` "/Game/Blueprints/Dragon/BP_Dragon_SlimeCover.BP_Dragon_SlimeCover_C" (`self.GetTransform`) "Undefined" "OverrideRootScale" null (`|GetArrayItem` _keys _index) self (`self.SlimeCoverRadius`) null))
        (`KismetArrayLibrary.Array_Add` (`self.SlimeCover`) _returnvalue)))
    (:`then_1`
      (for (_array_element _array_index) (`self.SlimeCover`)
        (`/Game/Blueprints/Dragon/BP_Dragon_SlimeCover.SetInfomation` _array_element (`|GetArrayItem` (`|MakeArray` "JNT_SlimeA" "JNT_SlimeA1" "JNT_SlimeA2" "JNT_SlimeA3" "JNT_SlimeA4" "JNT_SlimeA5" "JNT_SlimeA6" "JNT_SlimeB" "JNT_SlimeB1" "JNT_SlimeB2" "JNT_SlimeB3" "JNT_SlimeB4" "JNT_SlimeB5" "JNT_SlimeB6" "JNT_SlimeB7" "JNT_SlimeB8" "JNT_SlimeB9" "JNT_SlimeB10" "JNT_SlimeB11" "JNT_SlimeB12" "JNT_SlimeB13" "JNT_SlimeB14" "JNT_SlimeB15" :!type "Name") _array_index))))))

(fn `PrintDebugInfo`
  (locals (FormArray :type "Array of String"))
  (`KismetSystemLibrary.PrintString` (`KismetStringLibrary.Concat_StrStr` "Distance : " (`KismetStringLibrary.Conv_DoubleToString` (`KismetMathLibrary.Vector_Distance` (`self.K2_GetActorLocation` (`GameplayStatics.GetPlayerPawn` 0)) (`self.K2_GetActorLocation`)))) true false (struct :`G` 0.66 :`B` 1.0 :`A` 1.0) 0.0))

(fn `Reset1stSlimeScale`
  (bind _keys (`BlueprintMapLibrary.Map_Keys` (`self.SlimeScale`)))
  (for _index (range (`self.NumOf1stSlime`))
    (`self.SetSlimeScale` (`|GetArrayItem` _keys _index))))

(fn `ResetFlags`
  (bind _flags (`self.Flags`))
  (bind _keys (`BlueprintMapLibrary.Map_Keys` _flags))
  (for _array_element _keys
    (`BlueprintMapLibrary.Map_Add` _flags _array_element)))

(fn `SetFlag`
  (params (Name :type Name) (Flag :type Boolean))
  (bind _flags (`self.Flags`))
  (if (`.ReturnValue` (`BlueprintMapLibrary.Map_Find` _flags Name))
    (`BlueprintMapLibrary.Map_Add` _flags Name Flag)))

(fn `SetSlimeScale`
  (params (Name :type Name) (NewScale :type "Float (double-precision)"))
  (bind _slimescale (`self.SlimeScale`))
  (if (`BlueprintMapLibrary.Map_Contains` _slimescale Name)
    (`BlueprintMapLibrary.Map_Add` _slimescale Name (`KismetMathLibrary.MakeVector` NewScale NewScale NewScale))))

(fn `UpdateMaterialParameter`
  (params (ParamName :type Name) (`New Value` :type "Float (double-precision)"))
  (if (`self.GetFlag` "firstform")
    (`MaterialInstanceDynamic.SetScalarParameterValue` (`self.IM_Crystal`) ParamName `New Value`)
    (elif (`self.GetFlag` "secondform")
      (`MaterialInstanceDynamic.SetScalarParameterValue` (`self.IM_Body2nd`) ParamName `New Value`))))

(fn `UserConstructionScript`)