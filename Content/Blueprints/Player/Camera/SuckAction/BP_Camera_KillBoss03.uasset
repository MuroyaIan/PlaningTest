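; Camera actor for a boss-kill cutscene (third variant, by name), run from Tick in two stages once Start is set.
; Stage one shakes and moves along ActorPos's forward axis, ramping slow motion up through CustomTimeDilation on itself, player and target.
; After a 2.2-second delay it restores time, hides the target, swaps shakes, then pushes toward the player for a frame-counted duration.
; The FOV zoom logic is disconnected.
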(event `self.ReceiveBeginPlay`)

(event `self.ReceiveTick`
  (params (DeltaSeconds :type "Float (single-precision)"))
  (bind _returnvalue (`self.K2_GetActorLocation`))
  (bind _returnvalue_2 (`GameplayStatics.GetPlayerPawn` 0))
  (bind _returnvalue_3 (`GameplayStatics.GetPlayerController` 0))
  (bind _campos (`self.CamPos`))
  (bind _actorpos (`self.ActorPos`))
  (bind _timeratio (`self.TimeRatio`))
  (bind _actorpos_2 (`self.ActorPos`))
  (bind _returnvalue_4 (`self.K2_GetActorLocation` _actorpos_2))
  (bind _returnvalue_5 (`self.K2_GetActorLocation` _actorpos_2))
  (bind _returnvalue_6 (* (`self.GetActorUpVector` _actorpos_2) (`self.CameraDist_Z`)))
  (bind _returnvalue_7 (* (`self.GetActorUpVector` _actorpos_2) (`self.CameraDist_Z`)))
  (bind _returnvalue_8 (`KismetMathLibrary.MakeVector` (.x (+ _returnvalue (* (`/Game/Blueprints/BP_FuncLibrary.Vector to 2D(NormalizeXY)` (- (`self.K2_GetActorLocation` _returnvalue_2) _returnvalue)) (`self.CamPush_X`)))) (.y (+ _returnvalue (* (`/Game/Blueprints/BP_FuncLibrary.Vector to 2D(NormalizeXY)` (- (`self.K2_GetActorLocation` _returnvalue_2) _returnvalue)) (`self.CamPush_X`)))) (+ (.z (+ _returnvalue (* (`/Game/Blueprints/BP_FuncLibrary.Vector to 2D(NormalizeXY)` (- (`self.K2_GetActorLocation` _returnvalue_2) _returnvalue)) (`self.CamPush_X`)))) (`self.CamPush_Z`))))
  (set `self.DeltaSec` DeltaSeconds)
  (if (`self.bStart`)
    (if (`KismetSystemLibrary.IsValid` _actorpos_2)
      (`|ExecutionSequence`
        (:`then_0`
          (`/Engine/EditorBlueprintResources/StandardMacros.DoOnce` false
            (:`Completed`
              (set `self.CamPos` (+ (* (`self.GetActorForwardVector` _actorpos_2) (`self.CameraDist_X`)) _returnvalue_6 _returnvalue_4)) ; 視点初期化
              (set `self.GazePoint` (+ _returnvalue_6 _returnvalue_4)) ; 注視点初期化
              (`KismetSystemLibrary.Delay` 2.2) ; 第一段階終了
              (bind _output_get (set `self.CustomTimeDilation` 1.0)) ; スローモーション終了
              (bind _output_get_2 (set `Actor.CustomTimeDilation` _output_get (`GameplayStatics.GetPlayerPawn` 0)))
              (set `Actor.CustomTimeDilation` _output_get_2 _actorpos)
              (`self.SetActorHiddenInGame` _actorpos true)
              (set `self.bStepFin1` true)
              (`PlayerController.ClientStopCameraShake` _returnvalue_3 "/Game/Blueprints/Player/Camera/Shake/BP_Shake_KillBoss3.BP_Shake_KillBoss3_C" true)
              (`PlayerController.ClientStartCameraShake` :`self` _returnvalue_3 :`Shake` "/Game/Blueprints/Player/Camera/Shake/BP_Shake_KillBoss4.BP_Shake_KillBoss4_C"))))
        (:`then_1`
          (`|ExecutionSequence`
            (:`then_0`
              (if (not (`self.bStepFin1`))
                (`self.K2_SetActorLocation` _campos) ; カメラ更新
                (`self.K2_SetActorRotation` (`KismetMathLibrary.FindLookAtRotation` _campos (`self.GazePoint`)))
                (set `self.CamPos` (+ (* (`self.GetActorForwardVector` _actorpos_2) (* (`self.CamRatio`) (`self.CameraDist_X`))) _returnvalue_7 _returnvalue_5)) ; 視点初期化
                (set `self.GazePoint` (+ _returnvalue_7 _returnvalue_5)) ; 注視点初期化
                (`PlayerController.ClientStartCameraShake` :`self` (`GameplayStatics.GetPlayerController` 0) :`Shake` "/Game/Blueprints/Player/Camera/Shake/BP_Shake_KillBoss3.BP_Shake_KillBoss3_C")
                (set `self.CamRatio` (`KismetMathLibrary.FInterpTo_Constant` (`self.CamRatio`) 0.0 (`self.DeltaSec`) (`self.TargetMoveSpeed`)))
                (bind _output_get_3 (set `self.CustomTimeDilation` (`self.TimeRatio`))) ; スローモーション
                (bind _output_get_4 (set `Actor.CustomTimeDilation` _output_get_3 (`GameplayStatics.GetPlayerPawn` 0)))
                (set `Actor.CustomTimeDilation` _output_get_4 (`self.ActorPos`))
                (if (< _timeratio 0.03)
                  (set `self.TimeRatio` (+ _timeratio 0.0002))
                  (elif (< _timeratio 1.0)
                    (set `self.TimeRatio` (+ (`self.TimeRatio`) 0.01))
                    (else
                      (set `self.TimeRatio` 1.0))))))
            (:`then_1`
              (`|ExecutionSequence`
                (:`then_1`
                  (if (`self.bStepFin1`)
                    (if (> (`self.CamPushDuration`) 0.0)
                      (`self.K2_SetActorLocation` _returnvalue_8) ; カメラ更新
                      (`self.K2_SetActorRotation` (`KismetMathLibrary.FindLookAtRotation` _returnvalue_8 (+ (* (`self.GetActorUpVector` _returnvalue_2) 30.0) (`self.K2_GetActorLocation` _returnvalue_2))))
                      (`/Engine/EditorBlueprintResources/StandardMacros.DecrementFloat` (`self.CamPushDuration`)))))))))))))

(fn `UserConstructionScript`)