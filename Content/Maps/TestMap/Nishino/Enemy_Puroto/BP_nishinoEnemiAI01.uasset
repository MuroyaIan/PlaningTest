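; Prototype AI controller for BP_nishinoEnemy01 enemies in a test map, sending the pawn toward a charger location.
; Each tick it caches the controlled enemy, then issues AIMoveTo to that enemy's ChargerLocation while its ChargerFlg is set.
; SeePlayer, PopPontData and Vector_XY are unfinished: the line-trace sight check is disconnected and none of these functions is called.
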(event `self.ReceiveTick`
  (params (DeltaSeconds :type "Float (single-precision)"))
  (`self.TickCastData`) ; 情報の獲得
  (`self.EnemyMove`))

(event `EnemyMove`
  (bind _controlled_bp_nishinoenemy (`self.Controlled_BP_NishinoEnemy`))
  (if (`/Game/Maps/TestMap/Nishino/Enemy_Puroto/BP_nishinoEnemy01.ChargerFlg` _controlled_bp_nishinoenemy)
    (`|AIMoveTo` (`self.ControlledPawn`) (`/Game/Maps/TestMap/Nishino/Enemy_Puroto/BP_nishinoEnemy01.ChargerLocation` _controlled_bp_nishinoenemy) null 0.0)))

(fn `PopPontData`)

(fn `SeePlayer`
  (returns (Watch :type Boolean))
  (bind _asbp_nishino_enemy_01 (cast `/Game/Maps/TestMap/Nishino/Enemy_Puroto/BP_nishinoEnemy01` (`self.K2_GetPawn`))))

(fn `TickCastData`
  (bind _output_get (set `self.ControlledPawn` (`self.K2_GetPawn`)))
  (bind _asbp_nishino_enemy_01 (cast `/Game/Maps/TestMap/Nishino/Enemy_Puroto/BP_nishinoEnemy01` _output_get))
  (set `self.Controlled_BP_NishinoEnemy` _asbp_nishino_enemy_01))

(fn `UserConstructionScript`)