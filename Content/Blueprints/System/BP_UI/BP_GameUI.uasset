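; BP_GameUI is an in-stage UI manager that creates the main HUD widget and controls its reticle, quest guides and stage-intro skip prompt.
; On BeginPlay it hides the flask gauge, reticle and guides, then, unless the stage is a restart, shows the skip widget after a delay.
; Holding UI_Confirm fills the skip gauge, and Tick flags success when full and animates the reticle on aim-mode changes.
; StartQuestGuide shows the guide matching the selected stage.
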(event `self.ReceiveBeginPlay`
  (bind _asbp_player_controller (cast `/Game/Blueprints/Player/BP_PlayerController` (`GameplayStatics.GetPlayerController` 0)))
  (bind _output_get (set `self.Player Controller` _asbp_player_controller))
  (`self.EnableInput` _output_get) ; 入力有効化
  (set `self.AinModePrev` (`/Game/Blueprints/Player/BP_PlayerController.AimMode` _output_get))
  (bind _returnvalue (`|CreateWidget` "/Game/Maps/TestMap/Kitayama/UI_Kitayama/Widget_UI/GameWidget/UMG_GameUI.UMG_GameUI_C"))
  (bind _output_get_2 (set `self.Widget_GameUI` _returnvalue))
  (`UserWidget.AddToViewport` _output_get_2 0)
  (`Widget.RemoveFromParent` (`/Game/Maps/TestMap/Kitayama/UI_Kitayama/Widget_UI/GameWidget/UMG_GameUI.UMG_Flask` _output_get_2)) ; 初期状態はフラスコゲージが消えているように
  (`/Game/Maps/TestMap/Kitayama/UI_Kitayama/Widget_UI/GameWidget/UMG_GameUI.DispReticle` _output_get_2 false)
  (`Widget.RemoveFromParent` (`/Game/Maps/TestMap/Kitayama/UI_Kitayama/Widget_UI/GameWidget/UMG_GameUI.UMG_QG2_Stage1` _output_get_2))
  (`Widget.RemoveFromParent` (`/Game/Maps/TestMap/Kitayama/UI_Kitayama/Widget_UI/GameWidget/UMG_GameUI.UMG_QG2_Stage2` _output_get_2))
  (bind _asbp_global_data (cast `/Game/Blueprints/System/BP_GlobalData` (`GameplayStatics.GetGameInstance`)))
  (if (not (`/Game/Blueprints/System/BP_GlobalData.bStageRestart` _asbp_global_data))
    (bind _returnvalue_2 (`|CreateWidget` "/Game/Maps/TestMap/Kitayama/UI_Kitayama/Widget_UI/ButtonWidget/UMG_Skip.UMG_Skip_C"))
    (bind _output_get_3 (set `self.Widget_SkipUI` _returnvalue_2))
    (`KismetSystemLibrary.Delay` 1.5)
    (`UserWidget.AddToViewport` _output_get_3 4)
    (set `self.bCanSkip` true)))

(event `self.ReceiveTick`
  (params (DeltaSeconds :type "Float (single-precision)"))
  (bind _widget_skipui (`self.Widget_SkipUI`))
  (bind _aimmode (`/Game/Blueprints/Player/BP_PlayerController.AimMode` (`self.Player Controller`)))
  (bind _umg_reticle (`/Game/Maps/TestMap/Kitayama/UI_Kitayama/Widget_UI/GameWidget/UMG_GameUI.UMG_Reticle` (`self.Widget_GameUI`)))
  (`|ExecutionSequence`
    (:`then_0`
      (if (!= (`self.AinModePrev`) _aimmode)
        (if _aimmode
          (`/Game/Maps/TestMap/Kitayama/UI_Kitayama/Widget_UI/GameWidget/UMG_Reticle.PlayAimAnim` _umg_reticle)
          (set `self.AinModePrev` true)
          (else
            (`/Game/Maps/TestMap/Kitayama/UI_Kitayama/Widget_UI/GameWidget/UMG_Reticle.PlayNotAimAnim` _umg_reticle)
            (set `self.AinModePrev` false)))))
    (:`then_1`
      (if (`KismetSystemLibrary.IsValid` _widget_skipui)
        (if (`/Game/Maps/TestMap/Kitayama/UI_Kitayama/Widget_UI/ButtonWidget/UMG_Skip.GaugeMax` _widget_skipui)
          (`/Engine/EditorBlueprintResources/StandardMacros.DoOnce` false
            (:`Completed`
              (set `self.bSkipSuccess` true))))))))

(event `DispReticle`
  (params (Disp :type Boolean))
  (`/Game/Maps/TestMap/Kitayama/UI_Kitayama/Widget_UI/GameWidget/UMG_GameUI.DispReticle` (`self.Widget_GameUI`) Disp))

(event `InputAction|UI_Confirm` :consume false
  (params (Key :type "Key Structure"))
  (bind _widget_skipui (`self.Widget_SkipUI`))
  (:`Pressed`
    (if (`self.bCanSkip`)
      (if (`Widget.IsVisible` _widget_skipui)
        (set `self.bWillSkip` true)
        (`/Game/Maps/TestMap/Kitayama/UI_Kitayama/Widget_UI/ButtonWidget/UMG_Skip.Press` _widget_skipui 2.0))))
  (:`Released`
    (if (`self.bCanSkip`)
      (if (`Widget.IsVisible` _widget_skipui)
        (if (`self.bWillSkip`)
          (set `self.bWillSkip` false)
          (`/Game/Maps/TestMap/Kitayama/UI_Kitayama/Widget_UI/ButtonWidget/UMG_Skip.Release` _widget_skipui))))))

(fn `StartQuestGuide`
  (bind _asbp_global_data (cast `/Game/Blueprints/System/BP_GlobalData` (`GameplayStatics.GetGameInstance`)))
  (switch `int` (`/Game/Blueprints/System/BP_GlobalData.StageSelect` _asbp_global_data)
    (:`0`
      (`UserWidget.AddToViewport` (`/Game/Maps/TestMap/Kitayama/UI_Kitayama/Widget_UI/GameWidget/UMG_GameUI.UMG_QG2_Stage1` (`self.Widget_GameUI`)) 0))
    (:`1`
      (`UserWidget.AddToViewport` (`/Game/Maps/TestMap/Kitayama/UI_Kitayama/Widget_UI/GameWidget/UMG_GameUI.UMG_QG2_Stage2` (`self.Widget_GameUI`)) 0))))

(fn `UserConstructionScript`)