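; BP_Camera_Landscape is a scripted landscape camera sequence that moves a camera along a spline while the player moves forward.
; On BeginPlay it turns the player controller's rotation toward the PlayerDirection actor on the XY plane.
; Once Start is set, Tick advances the camera along SplineCameraRoute at MoveSpeed and feeds slight forward movement input to the pawn.
; A Delay in Tick sets Fin after three seconds, ending the sequence.
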(event `self.ReceiveBeginPlay`
  (bind _returnvalue (`GameplayStatics.GetPlayerPawn` 0))
  (bind _asbp_player (cast `/Game/Blueprints/Player/BP_Player` _returnvalue))
  (bind _playercontroller (`/Game/Blueprints/Player/BP_Player.GetUserController` _asbp_player))
  (bind _output_get (set `/Game/Blueprints/Player/BP_PlayerController.TargetRotation` (`KismetMathLibrary.FindLookAtRotation` (`/Game/Blueprints/BP_FuncLibrary.Vector to 2D(XY)` (`self.K2_GetActorLocation` _returnvalue)) (`/Game/Blueprints/BP_FuncLibrary.Vector to 2D(XY)` (`self.K2_GetActorLocation` (`self.PlayerDirection`)))) _playercontroller)) ; プレイヤー向き更新
  (set `/Game/Blueprints/Player/BP_PlayerController.Rotation` _output_get _playercontroller))

(event `self.ReceiveTick`
  (params (DeltaSeconds :type "Float (single-precision)"))
  (bind _returnvalue (`GameplayStatics.GetPlayerPawn` 0))
  (if (and (`self.bStart`) (not (`self.bFin`)))
    (set `self.CurrentDistance` (+ (`self.CurrentDistance`) (* (`self.MoveSpeed`) DeltaSeconds)))
    (`SceneComponent.K2_SetWorldLocation` (`self.CameraComponent`) (`SplineComponent.GetLocationAtDistanceAlongSpline` (`self.Spline_CameraRoute`) (`self.CurrentDistance`) "World") false false) ; カメラ位置更新
    (`Pawn.AddMovementInput` _returnvalue (`self.GetActorForwardVector` _returnvalue) 0.001 false) ; プレイヤー走行
    (`KismetSystemLibrary.Delay` 3.0)
    (set `self.bFin` true) ; カメラワーク終了
  ))

(fn `UserConstructionScript`)