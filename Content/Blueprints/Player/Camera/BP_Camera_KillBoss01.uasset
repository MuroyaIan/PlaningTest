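; Cinematic camera for the first shot of the boss kill, triggered while the player's weapon has SuckBoss set.
; A DoOnce on Tick places it front-left of the player with a level look-at, takes the view, then blends to NextCamera after a delay and starts that BP_Camera_SuckBoss02.
; Each tick it narrows the FOV, easing the interp speed down for a fast, decelerating zoom-in.
; The DoOnce resets when SuckBoss is off.
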(event `self.ReceiveBeginPlay`)

(event `self.ReceiveTick`
  (params (DeltaSeconds :type "Float (single-precision)"))
  (bind _nextcamera (`self.NextCamera`))
  (set `self.DeltaSec` DeltaSeconds)
  (bind _asbp_player (cast `/Game/Blueprints/Player/BP_Player` (`GameplayStatics.GetPlayerPawn` 0)))
  (if (`/Game/Blueprints/Weapon/BP_Weapon.bSuckBoss` (`/Game/Blueprints/Player/BP_Player.GetWeapon` _asbp_player))
    (`|ExecutionSequence`
      (:`then_0`
        (`/Engine/EditorBlueprintResources/StandardMacros.DoOnce` false :!label _label
          (:`Completed`
            (bind _returnvalue (`self.K2_GetActorLocation` _asbp_player))
            (bind _returnvalue_2 (+ (* (`self.GetActorForwardVector` _asbp_player) 150.0) (* (`self.GetActorRightVector` _asbp_player) -150.0) (* (`self.GetActorUpVector` _asbp_player) 30.0) _returnvalue))
            (`self.K2_SetActorLocation` _returnvalue_2) ; カメラ更新
            (`self.K2_SetActorRotation` (`KismetMathLibrary.FindLookAtRotation` _returnvalue_2 (`KismetMathLibrary.MakeVector` (.x _returnvalue) (.y _returnvalue) (.z _returnvalue_2))))
            (`PlayerController.SetViewTargetWithBlend` (`GameplayStatics.GetPlayerController` 0) self 0.0 "VTBlend_Linear" 0.0 false) ; 演出カメラ切替
            (set `self.FOV` 90.0)
            (set `self.SpeedFOV` 200.0)
            (set `self.AlphaFOV` 0.0)
            (`KismetSystemLibrary.Delay` 0.8) ; カメラ切替
            (`PlayerController.SetViewTargetWithBlend` (`GameplayStatics.GetPlayerController` 0) _nextcamera 0.5 "VTBlend_Linear" 0.0 false)
            (bind _asbp_camera_suck_boss_02 (cast `/Game/Blueprints/Player/Camera/BP_Camera_SuckBoss02` _nextcamera))
            (set `/Game/Blueprints/Player/Camera/BP_Camera_SuckBoss02.bStart` true _asbp_camera_suck_boss_02))))
      (:`then_1`
        (bind _output_get (set `self.FOV` (`KismetMathLibrary.FInterpTo_Constant` (`self.FOV`) 60.0 (`self.DeltaSec`) (`self.SpeedFOV`))))
        (`CameraComponent.SetFieldOfView` (`self.CameraComponent`) _output_get) ; ズームイン
        (bind _output_get_2 (set `self.AlphaFOV` (`KismetMathLibrary.FInterpTo_Constant` (`self.AlphaFOV`) 1.0 (`self.DeltaSec`) 0.5)))
        (set `self.SpeedFOV` (`|EaseFunction` "EaseOut" _output_get_2 (`self.SpeedFOV`) 5.0 4.0))))
    (else
      (goto _label :!via `Reset`))))

(fn `UserConstructionScript`)